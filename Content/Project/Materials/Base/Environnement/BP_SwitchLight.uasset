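; BP_SwitchLight is a world actor that turns day toward night when the player enters a trigger.
; Overlapping component 1 with BP_PlayerCharacter calls DaytimeToNightTime, which plays the GoDown timeline to pitch the DayLight actor at fixed yaw.
; Triggers 2 and 3 do nothing.
; The GoUp NightLight rotation and staged playback-position checks are disconnected, so only the sun moves.
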(event OnComponentBeginOverlap(1)
  (params (OverlappedComponent :type Primitive%20Component%20Object%20Reference) (OtherActor :type Actor%20Object%20Reference) (OtherComp :type Primitive%20Component%20Object%20Reference) (OtherBodyIndex :type Integer) (bFromSweep :type Boolean) (SweepResult :type Hit%20Result%20Structure%20%28by%20ref%29))
  (Utilities|Casting|CastToBP_PlayerCharacter OtherActor)
  (CallFunction|DaytimetoNightTime))

(event OnComponentBeginOverlap(2)
  (params (OverlappedComponent :type Primitive%20Component%20Object%20Reference) (OtherActor :type Actor%20Object%20Reference) (OtherComp :type Primitive%20Component%20Object%20Reference) (OtherBodyIndex :type Integer) (bFromSweep :type Boolean) (SweepResult :type Hit%20Result%20Structure%20%28by%20ref%29)))

(event OnComponentBeginOverlap(3)
  (params (OverlappedComponent :type Primitive%20Component%20Object%20Reference) (OtherActor :type Actor%20Object%20Reference) (OtherComp :type Primitive%20Component%20Object%20Reference) (OtherBodyIndex :type Integer) (bFromSweep :type Boolean) (SweepResult :type Hit%20Result%20Structure%20%28by%20ref%29)))

(event Custom|DaytimeToNightTime
  (bind _y_axis_rotation (Timeline|GoDown Play)
    (:Update
      (Transformation|SetActorRotation (Variables|Default|GetDayLight) (Math|Rotator|MakeRotator 0.0 _y_axis_rotation 92.0)))
    (:Finished
      (Development|PrintString "End sun move"))))

(event EventBeginPlay)

(event Collision|EventActorBeginOverlap
  (params (OtherActor :type Actor%20Object%20Reference)))

(event EventTick
  (params (DeltaSeconds :type Float%20%28single-precision%29)))

(fn ConstructionScript)