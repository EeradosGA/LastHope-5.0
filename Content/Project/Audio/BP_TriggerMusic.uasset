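; Music trigger actor that changes or stops the music when the player crosses its boxes.
; BoxEnter fades in MusicOnTrigger or fades out the current track through MusicPlayer, per its flags.
; BoxExit fades to MusicExitTrigger, with latches making each track switch one-shot.
; DeactiveAtKill suppresses the exit switch, but the logic meant to switch once Enemy is invalid is disconnected and never runs.
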(event OnComponentBeginOverlap(BoxEnter)
  (params (OverlappedComponent :type Primitive%20Component%20Object%20Reference) (OtherActor :type Actor%20Object%20Reference) (OtherComp :type Primitive%20Component%20Object%20Reference) (OtherBodyIndex :type Integer) (bFromSweep :type Boolean) (SweepResult :type Hit%20Result%20Structure%20%28by%20ref%29))
  (Utilities|Casting|CastToBP_PlayerCharacter OtherActor)
  (if (not (Variables|Default|GetActiveOneTime))
    (Utilities|FlowControl|Sequence
      (:then_0
        (if (Variables|Default|GetPlayNewMusic)
          (Default|PlayMusicFade (Variables|Default|GetMusicPlayer) (Variables|Default|GetMusicOnTrigger) 3.0 3.0 0.0)
          (Variables|Default|SetActiveOneTime true)))
      (:then_1
        (if (Variables|Default|GetStopMusic)
          (Default|StopActualMusic (Variables|Default|GetMusicPlayer) true 4.0 0.0 "Linear"))))))

(event OnComponentEndOverlap(BoxExit)
  (params (OverlappedComponent :type Primitive%20Component%20Object%20Reference) (OtherActor :type Actor%20Object%20Reference) (OtherComp :type Primitive%20Component%20Object%20Reference) (OtherBodyIndex :type Integer))
  (Utilities|Casting|CastToBP_PlayerCharacter OtherActor)
  (if (not (Variables|Default|GetDeactiveAtKill))
    (if (Variables|Default|GetActiveOneTime)
      (if (not (Variables|Default|GetEndTrigger))
        (if (Variables|Default|GetPlayNewMusic)
          (Default|PlayMusicFade (Variables|Default|GetMusicPlayer) (Variables|Default|GetMusicExitTrigger) 3.0 3.0 0.0)
          (Variables|Default|SetEndTrigger true))))))

(event EventBeginPlay)

(event Collision|EventActorBeginOverlap
  (params (OtherActor :type Actor%20Object%20Reference)))

(event EventTick
  (params (DeltaSeconds :type Float%20%28single-precision%29)))

(fn ConstructionScript)