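; Music player Blueprint that plays one 2D track at a time, chosen by a music state enum for menu, areas, fights and ambience.
; PlayMusicFade stores the state, fade times and start time, then sets a flag that Tick consumes to fade out, wait, and fade in the new track.
; LaunchMusic starts a track immediately without stopping the current one, or fades out on STOP; StopActualMusic fades or cuts playback.
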(event EventTick
  (params (DeltaSeconds :type Float%20%28single-precision%29))
  (if (Variables|Default|GetPerformStateChangement)
    (Variables|Default|SetPerformStateChangement false)
    (if (Utilities|IsValid (Variables|Default|GetMusicSource_Actual))
      (Audio|Components|Audio|FadeOut (Variables|Default|GetMusicSource_Actual) (Variables|Default|GetDelayFadeOut) 0.0 "Linear" :!class /Script/Engine.AudioComponent)
      (Utilities|FlowControl|Delay (Variables|Default|GetDelayFadeOut)))
    (switch Utilities|FlowControl|Switch|SwitchonEnum_Musics (Variables|Default|GetEMusicsState)
      (:NewEnumerator0
        (bind _returnvalue (Audio|SpawnSound2D "/Game/Project/Audio/Music/SC_M_Menu.SC_M_Menu" 1.0 1.0 0.0 0))
        (Variables|Default|SetMusicSource_Actual _returnvalue))
      (:NewEnumerator1
        (bind _returnvalue_2 (Audio|SpawnSound2D "/Game/Project/Audio/Music/SC_M_Canyon_loop.SC_M_Canyon_Loop" 1.0 1.0 0.0 0))
        (Variables|Default|SetMusicSource_Actual _returnvalue_2))
      (:NewEnumerator2
        (bind _returnvalue_3 (Audio|SpawnSound2D "/Game/Project/Audio/Music/SC_M_Fight_Simple.SC_M_Fight_Simple" 1.0 1.0 0.0 0))
        (Variables|Default|SetMusicSource_Actual _returnvalue_3))
      (:NewEnumerator3
        (bind _returnvalue_4 (Audio|SpawnSound2D "/Game/Project/Audio/Music/SC_M_Horde_Loop.SC_M_Horde_Loop" 1.0 1.0 0.0 0))
        (Variables|Default|SetMusicSource_Actual _returnvalue_4))
      (:NewEnumerator6
        (bind _returnvalue_5 (Audio|SpawnSound2D "/Game/Project/Audio/Music/SC_M_Temple_Loop.SC_M_Temple_Loop" 1.0 1.0 0.0 0))
        (Variables|Default|SetMusicSource_Actual _returnvalue_5))
      (:NewEnumerator4
        (bind _returnvalue_6 (Audio|SpawnSound2D "/Game/Project/Audio/Music/SC_M_Boss.SC_M_Boss" 1.0 1.0 0.0 0))
        (Variables|Default|SetMusicSource_Actual _returnvalue_6))
      (:NewEnumerator7
        (bind _returnvalue_7 (Audio|SpawnSound2D "/Game/Project/Audio/Music/Ambience/SC_M_DesertAmbience.SC_M_DesertAmbience" 1.0 1.0 0.0 0))
        (Variables|Default|SetMusicSource_Actual _returnvalue_7))
      (:NewEnumerator8
        (bind _returnvalue_8 (Audio|SpawnSound2D "/Game/Project/Audio/Music/Ambience/SC_M_Rumble.SC_M_Rumble" 1.0 1.0 0.0 0))
        (Variables|Default|SetMusicSource_Actual _returnvalue_8))
      (:NewEnumerator9
        (bind _returnvalue_9 (Audio|SpawnSound2D "/Game/Project/Audio/Music/SC_M_EntryTemple.SC_M_EntryTemple" 1.0 1.0 0.0 0))
        (Variables|Default|SetMusicSource_Actual _returnvalue_9)))
    (Audio|Components|Audio|FadeIn (Variables|Default|GetMusicSource_Actual) (Variables|Default|GetDelayFadeIn) 1.0 (Variables|Default|GetStartTime) "Linear" :!class /Script/Engine.AudioComponent)))

(fn ConstructionScript)

(fn PlayMusicFade
  (params (Music :type Enum_Musics%20Enum :default "NewEnumerator0") (DelayFadeOut :type Float%20%28single-precision%29) (DelayFadeIn :type Float%20%28single-precision%29) (StartTime :type Float%20%28single-precision%29))
  (Variables|Default|SetDelayFadeOut DelayFadeOut)
  (Variables|Default|SetDelayFadeIn DelayFadeIn)
  (Variables|Default|SetStartTime StartTime)
  (Variables|Default|SetEMusicsState Music)
  (Variables|Default|SetPerformStateChangement true))

(fn StopActualMusic
  (params (WithFade :type Boolean) (FadeOutDuration :type Float%20%28single-precision%29) (FadeVolumeLevel :type Float%20%28single-precision%29) (FadeCurve :type EAudioFaderCurve%20Enum :default "Linear"))
  (if (Utilities|IsValid (Variables|Default|GetMusicSource_Actual))
    (if WithFade
      (Audio|Components|Audio|FadeOut (Variables|Default|GetMusicSource_Actual) FadeOutDuration FadeVolumeLevel FadeCurve :!class /Script/Engine.AudioComponent)
      (else
        (Audio|Components|Audio|Stop (Variables|Default|GetMusicSource_Actual))))))

(fn LaunchMusic
  (params (Music :type Enum_Musics%20Enum :default "NewEnumerator0") (FadeInDuration :type Float%20%28single-precision%29) (FadeVolumeLevel :type Float%20%28single-precision%29) (StartTime :type Float%20%28single-precision%29))
  (switch Utilities|FlowControl|Switch|SwitchonEnum_Musics Music
    (:NewEnumerator0
      (bind _returnvalue (Audio|SpawnSound2D "/Game/Project/Audio/Music/SC_M_Menu.SC_M_Menu" 1.0 1.0 0.0 0))
      (Variables|Default|SetMusicSource_Actual _returnvalue)
      (Audio|Components|Audio|FadeIn (Variables|Default|GetMusicSource_Actual) FadeInDuration FadeVolumeLevel StartTime "Linear" :!class /Script/Engine.AudioComponent :!label _label))
    (:NewEnumerator1
      (bind _returnvalue_2 (Audio|SpawnSound2D "/Game/Project/Audio/Music/SC_M_Canyon_loop.SC_M_Canyon_Loop" 1.0 1.0 0.0 0))
      (Variables|Default|SetMusicSource_Actual _returnvalue_2)
      (goto _label))
    (:NewEnumerator2
      (bind _returnvalue_3 (Audio|SpawnSound2D "/Game/Project/Audio/Music/SC_M_Fight_Simple.SC_M_Fight_Simple" 1.0 1.0 0.0 0))
      (Variables|Default|SetMusicSource_Actual _returnvalue_3)
      (goto _label))
    (:NewEnumerator3
      (bind _returnvalue_4 (Audio|SpawnSound2D "/Game/Project/Audio/Music/SC_M_Horde_Loop.SC_M_Horde_Loop" 1.0 1.0 0.0 0))
      (Variables|Default|SetMusicSource_Actual _returnvalue_4)
      (goto _label))
    (:NewEnumerator6
      (bind _returnvalue_5 (Audio|SpawnSound2D "/Game/Project/Audio/Music/SC_M_Temple_Loop.SC_M_Temple_Loop" 1.0 1.0 0.0 0))
      (Variables|Default|SetMusicSource_Actual _returnvalue_5)
      (goto _label))
    (:NewEnumerator4
      (bind _returnvalue_6 (Audio|SpawnSound2D "/Game/Project/Audio/Music/SC_M_Boss.SC_M_Boss" 1.0 1.0 0.0 0))
      (Variables|Default|SetMusicSource_Actual _returnvalue_6)
      (goto _label))
    (:NewEnumerator5
      (CallFunction|StopActualMusic true 3.0 0.0 "Linear"))
    (:NewEnumerator7
      (bind _returnvalue_7 (Audio|SpawnSound2D "/Game/Project/Audio/Music/Ambience/SC_M_DesertAmbience.SC_M_DesertAmbience" 1.0 1.0 0.0 0))
      (Variables|Default|SetMusicSource_Actual _returnvalue_7)
      (goto _label))
    (:NewEnumerator8
      (bind _returnvalue_8 (Audio|SpawnSound2D "/Game/Project/Audio/Music/Ambience/SC_M_Rumble.SC_M_Rumble" 1.0 1.0 0.0 0))
      (Variables|Default|SetMusicSource_Actual _returnvalue_8)
      (goto _label))
    (:NewEnumerator9
      (bind _returnvalue_9 (Audio|SpawnSound2D "/Game/Project/Audio/Music/SC_M_EntryTemple.SC_M_EntryTemple" 1.0 1.0 0.0 0))
      (Variables|Default|SetMusicSource_Actual _returnvalue_9)
      (goto _label))))

(fn PlayMusicTransition)