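; Save manager actor that starts, saves and continues a game through a BP_SaveGameLastHope object in a single named slot.
; Saving maps level item picked and object used flags by object name, plus player health, inventory classes, backpack and spawn position.
; Continuing destroys picked items, replays UseObject on used objects and restores the player, rebuilding inventory from briefly spawned actors.
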(event Custom|NewGame
  (bind _returnvalue (SaveGame|CreateSaveGameObject "/Game/Project/Blueprints/System/BP_SaveGameLastHope.BP_SaveGameLastHope_C"))
  (Variables|Default|SetRefSaveGameLastHope _returnvalue)
  ;[1 1 1] Register Data from BP_Spawn
  (CallFunction|RegisterLevel)
  (bind _asbp_player_character (Utilities|Casting|CastToBP_PlayerCharacter (Game|Player|GetPlayerPawn 0))
    (:then
      (CallFunction|RegisterPlayer _asbp_player_character))
    (:CastFailed
      (Development|PrintString "ERROR  BP_Spawn, cant register player data because player is null" true true "(R=1.000000,G=0.000000,B=0.008760,A=1.000000)"))))

(event Custom|ContinueGame
  (bind _asbp_save_game_last_hope (CallFunction|LoadGame))
  (bind _output_get (Variables|Default|SetRefSaveGameLastHope _asbp_save_game_last_hope))
  (Utilities|IsValid _output_get
    (:Is%20Valid
      (Development|PrintString "Hugo : BP_Spawn Successfully Loaded Save !" true true "(R=0.000000,G=1.000000,B=0.100456,A=1.000000)" 0.5)
      (CallFunction|SpawnItems)
      (bind _asbp_player_character (Utilities|Casting|CastToBP_PlayerCharacter (Game|Player|GetPlayerPawn 0))
        (:then
          (CallFunction|SetPlayerDatafromSave _asbp_player_character))
        (:CastFailed
          (Development|PrintString "ERROR  BP_Spawn, cant set player data because player is null" true true "(R=1.000000,G=0.000000,B=0.008760,A=1.000000)"))))
    (:Is%20Not%20Valid
      (Development|PrintString "Hugo : BP_Spawn ERROR  Laoding save !" true true "(R=1.000000,G=0.000000,B=0.000000,A=1.000000)" 5.0))))

(event EventBeginPlay
  (bind _returnvalue (SaveGame|CreateSaveGameObject "/Game/Project/Blueprints/System/BP_SaveGameLastHope.BP_SaveGameLastHope_C"))
  (Variables|Default|SetRefSaveGameLastHope _returnvalue))

(event Collision|EventActorBeginOverlap
  (params (OtherActor :type Actor%20Object%20Reference)))

(event EventTick
  (params (DeltaSeconds :type Float%20%28single-precision%29)))

(fn ConstructionScript)

(fn RegisterLevel
  (for _array_element (Variables|Default|GetitemList)
    (Utilities|IsValid _array_element
      (:Is%20Valid
        (Utilities|Map|Add (Variables|/Game/Project/Blueprints/System/BP_SaveGameLastHope.BP_SaveGameLastHope_C|GetboolWithID (Variables|Default|GetRefSaveGameLastHope)) (Utilities|GetObjectName _array_element) (Variables|/Game/Project/Blueprints/Items/BP_Item.BP_Item_C|GetisPick? _array_element)))))
  (for _array_element_2 (Variables|Default|GetobjectList)
    (Utilities|Map|Add (Variables|/Game/Project/Blueprints/System/BP_SaveGameLastHope.BP_SaveGameLastHope_C|GetboolWithID (Variables|Default|GetRefSaveGameLastHope)) (Utilities|GetObjectName _array_element_2) (.hasBeenUsed? (Utilities|Struct|BreakStruct_InfoObject (Variables|/Game/Project/Blueprints/Objects/BP_Object.BP_Object_C|GetStruct_InfoObject _array_element_2))))
    (Development|PrintString (Utilities|String|Append "Qdding object :" (Utilities|GetObjectName _array_element_2) "zith bool :" (Utilities|String|ToString(Boolean) (.hasBeenUsed? (Utilities|Struct|BreakStruct_InfoObject (Variables|/Game/Project/Blueprints/Objects/BP_Object.BP_Object_C|GetStruct_InfoObject _array_element_2))))) true true "(R=0.740537,G=0.361517,B=1.000000,A=1.000000)" 2e+01)))

(fn SaveGame
  (CallFunction|RegisterLevel)
  (CallFunction|RegisterPlayer (.AsBP%20Player%20Character (Utilities|Casting|CastToBP_PlayerCharacter (Game|Player|GetPlayerPawn 0))))
  (bind _returnvalue (SaveGame|SaveGametoSlot (Variables|Default|GetRefSaveGameLastHope) (Variables|Default|GetGameSaveName)))
  (if _returnvalue
    (Development|PrintString "Hugo : BP_Spawn Created Save !" true true "(R=0.000000,G=1.000000,B=0.100456,A=1.000000)" 0.5)
    (else
      (Development|PrintString "Hugo : BP_Spawn ERROR  creating save !" true true "(R=1.000000,G=0.000000,B=0.000000,A=1.000000)" 5.0))))

(fn LoadGame
  (bind _returnvalue (SaveGame|LoadGamefromSlot (Variables|Default|GetGameSaveName)))
  (bind _asbp_save_game_last_hope (Utilities|Casting|CastToBP_SaveGameLastHope _returnvalue)
    (:then
      (return _asbp_save_game_last_hope))
    (:CastFailed
      (Development|PrintString "failed to cast to BP_SaveGame"))))

(fn SpawnItems
  (for _array_element (Variables|Default|GetitemList)
    (if (.ReturnValue (Utilities|Map|Find (Variables|/Game/Project/Blueprints/System/BP_SaveGameLastHope.BP_SaveGameLastHope_C|GetboolWithID (Variables|Default|GetRefSaveGameLastHope)) (Utilities|GetObjectName _array_element)))
      (if (.Value (Utilities|Map|Find (Variables|/Game/Project/Blueprints/System/BP_SaveGameLastHope.BP_SaveGameLastHope_C|GetboolWithID (Variables|Default|GetRefSaveGameLastHope)) (Utilities|GetObjectName _array_element)))
        (Utilities|Array|RemoveItem (Variables|Default|GetitemList) _array_element)
        (Utilities|Array|Add (LocalVariables|GetDeleteItems) _array_element)
        (Development|PrintString (Utilities|String|Append "removing element bcs it is picked" (Utilities|GetDisplayName _array_element)) true true "(R=0.090802,G=1.000000,B=0.002553,A=1.000000)"))
      (else
        (Development|PrintString (Utilities|String|Append "Hugo BP_Spawn : Loading ERROR could not find  " (Utilities|GetObjectName _array_element)) true true "(R=1.000000,G=0.046545,B=0.000000,A=1.000000)"))))
  (for _array_element_2 (Variables|Default|GetobjectList)
    (if (.ReturnValue (Utilities|Map|Find (Variables|/Game/Project/Blueprints/System/BP_SaveGameLastHope.BP_SaveGameLastHope_C|GetboolWithID (Variables|Default|GetRefSaveGameLastHope)) (Utilities|GetObjectName _array_element_2)))
      (if (.Value (Utilities|Map|Find (Variables|/Game/Project/Blueprints/System/BP_SaveGameLastHope.BP_SaveGameLastHope_C|GetboolWithID (Variables|Default|GetRefSaveGameLastHope)) (Utilities|GetObjectName _array_element_2)))
        (Default|UseObject _array_element_2))))
  (for _array_element_3 (LocalVariables|GetDeleteItems)
    (Actor|DestroyActor _array_element_3)))

(fn RegisterPlayer
  (params (refPlayer :type BP%20Player%20Character%20Object%20Reference))
  (bind _acp_inventory (Variables|/Game/Project/Blueprints/BP_PlayerCharacter.BP_PlayerCharacter_C|GetACP_Inventory refPlayer))
  (bind _refsavegamelasthope (Variables|Default|GetRefSaveGameLastHope))
  (Variables|/Game/Project/Blueprints/System/BP_SaveGameLastHope.BP_SaveGameLastHope_C|SetplayerLifeAmount _refsavegamelasthope (Variables|/Game/Project/Blueprints/BP_PlayerCharacter.BP_PlayerCharacter_C|GetCurrentHP refPlayer))
  (Variables|/Game/Project/Blueprints/System/BP_SaveGameLastHope.BP_SaveGameLastHope_C|SetInventoryItemList _refsavegamelasthope (Variables|/Game/Project/Blueprints/Items/ACP_Inventory.ACP_Inventory_C|GetlistItemClass _acp_inventory))
  (Variables|/Game/Project/Blueprints/System/BP_SaveGameLastHope.BP_SaveGameLastHope_C|SethasBackPack _refsavegamelasthope (Variables|/Game/Project/Blueprints/Items/ACP_Inventory.ACP_Inventory_C|GethaveBackpack? _acp_inventory))
  (Variables|/Game/Project/Blueprints/System/BP_SaveGameLastHope.BP_SaveGameLastHope_C|SetspawnPosition _refsavegamelasthope (Variables|Default|GetspawnPosition)))

(fn SetPlayerDatafromSave
  (params (refPlayer :type BP%20Player%20Character%20Object%20Reference))
  (bind _acp_inventory (Variables|/Game/Project/Blueprints/BP_PlayerCharacter.BP_PlayerCharacter_C|GetACP_Inventory refPlayer))
  (Variables|/Game/Project/Blueprints/BP_PlayerCharacter.BP_PlayerCharacter_C|SetCurrentHP refPlayer (Variables|/Game/Project/Blueprints/System/BP_SaveGameLastHope.BP_SaveGameLastHope_C|GetplayerLifeAmount (Variables|Default|GetRefSaveGameLastHope)))
  (for _array_element (Variables|/Game/Project/Blueprints/System/BP_SaveGameLastHope.BP_SaveGameLastHope_C|GetInventoryItemList (Variables|Default|GetRefSaveGameLastHope))
    (bind _returnvalue (Game|SpawnActorfromClass _array_element (Math|Transform|MakeTransform "0, 0, 0" "0, 0, 0" "1,1,1") "Undefined" 0 0))
    (Default|AddItem _acp_inventory _returnvalue _array_element)
    (Actor|DestroyActor _returnvalue))
  (Variables|/Game/Project/Blueprints/Items/ACP_Inventory.ACP_Inventory_C|SethaveBackpack? _acp_inventory (Variables|/Game/Project/Blueprints/System/BP_SaveGameLastHope.BP_SaveGameLastHope_C|GethasBackPack (Variables|Default|GetRefSaveGameLastHope)))
  (Transformation|SetActorLocation refPlayer (Variables|/Game/Project/Blueprints/System/BP_SaveGameLastHope.BP_SaveGameLastHope_C|GetspawnPosition (Variables|Default|GetRefSaveGameLastHope)) false false)
  (Development|PrintString "Set player data from save"))