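; BP_SoundVoiceRing is an environment sound actor that plays its audio until the player has a ring in their inventory.
; BeginPlay starts the Audio component from the beginning.
; Every Tick, it loops through the player character's inventory item list and stops the audio when an entry casts to BP_Ring.
; The check polls each frame and keeps running after the sound stops.
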(event EventBeginPlay
  (Audio|Components|Audio|Play (Variables|Default|GetAudio) 0.0))

(event Collision|EventActorBeginOverlap
  (params (OtherActor :type Actor%20Object%20Reference)))

(event EventTick
  (params (DeltaSeconds :type Float%20%28single-precision%29))
  (bind _asbp_player_character (Utilities|Casting|CastToBP_PlayerCharacter (Game|GetPlayerCharacter 0)))
  (for _array_element (Variables|/Game/Project/Blueprints/Items/ACP_Inventory.ACP_Inventory_C|GetlistItemClass (Variables|/Game/Project/Blueprints/BP_PlayerCharacter.BP_PlayerCharacter_C|GetACP_Inventory _asbp_player_character))
    (Utilities|Casting|CastToBP_RingClass _array_element)
    (Audio|Components|Audio|Stop (Variables|Default|GetAudio))))

(fn ConstructionScript)