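; Directional light actor that rotates the sun and updates the sky sphere as horde completion advances.
; Each horde update from the game instance, re-bound every Tick, maps progress to a target roll between the initial and maximum angles.
; Tick rotates toward that target at a speed tiered by current roll, then stops.
; The first tier compares roll against SpeedMedium, a speed value, and the stored initial intensity is unused.
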(event Custom|UpdateHorde
  (params (Percentage%280%20to%201%29 :type Float%20%28single-precision%29) (IsFinished? :type Boolean))
  (bind _output_get (Variables|Enemy|SetCurrentEnemiesKilled Percentage%280%20to%201%29))
  (Variables|Enemy|SetRotationXToAttempt (+ (* _output_get (/ (- (Variables|Enemy|GetMaxRotationX) (Variables|Enemy|GetInitialRotationX)) (Variables|Enemy|GetMaxNumberEnemies))) (Variables|Enemy|GetInitialRotationX)))
  (Variables|Default|SetLaunchDynamic true)
  (Development|PrintString "Update Horde"))

(event EventBeginPlay
  (Variables|Default|SetInitialIntensity (Variables|/Script/Engine.LightComponentBase|GetIntensity (Variables|DayNightCycle|GetDirectionalLightComponent)))
  (Variables|Enemy|SetInitialRotationX (.roll (Transformation|GetActorRotation)))
  (bind _asbp_last_hope_game_instance (Utilities|Casting|CastToBP_LastHopeGameInstance (Game|GetGameInstance)))
  (Variables|Default|SetGameInstance _asbp_last_hope_game_instance))

(event EventTick
  (params (DeltaSeconds :type Float%20%28single-precision%29))
  (Utilities|FlowControl|Sequence
    (:then_0
      (EventDispatchers|BindEventtoUpdateHordeCompletion (Variables|Default|GetGameInstance) (delegate Custom|UpdateHorde)))
    (:then_1
      (if (< (.roll (Transformation|GetActorRotation)) (Variables|Speed|GetSpeedMedium))
        (Variables|Speed|SetActualSpeed (Variables|Speed|GetSpeedHigh))
        (elif (and (>= (.roll (Transformation|GetActorRotation)) (Variables|Speed|GetPercentSpeedMedium)) (< (.roll (Transformation|GetActorRotation)) (Variables|Speed|GetPercentSpeedHigh)))
          (Variables|Speed|SetActualSpeed (Variables|Speed|GetSpeedMedium))
          (elif (>= (.roll (Transformation|GetActorRotation)) (Variables|Speed|GetPercentSpeedHigh))
            (Variables|Speed|SetActualSpeed (Variables|Speed|GetSpeedLow))
            (else
              (Variables|Speed|SetActualSpeed 2.0))))))
    (:then_2
      (if (Variables|Default|GetLaunchDynamic)
        (Class|Actor|AddActorWorldRotation (Math|Rotator|MakeRotator (* DeltaSeconds (Variables|Speed|GetActualSpeed)) 0.0 0.0))
        (Default|UpdateSunDirection (Variables|Default|GetSkySphere))
        (if (>= (.roll (Transformation|GetActorRotation)) (Variables|Enemy|GetRotationXToAttempt))
          (Variables|Default|SetLaunchDynamic false))))))

(fn ConstructionScript)