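; BP_BraseiroFire_2 is a brazier fire actor with particles, a flickering point light and audio, started on BeginPlay if StartWithoutTrigger is set, otherwise through its Initialization event.
; Initialization activates the fire, starts the flicker timeline and plays light-up and thrower sounds once.
; The flicker lerps light intensity toward a target that is re-randomized after short random delays.
; IsFireOn mirrors the particle's active state, refreshed on Tick while Initialized is true.
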(event Custom|Initialization
  (CallFunction|DevPrint "NewEnumerator6" 0 "BP_BraseiroFire_2 Initialization" true true "(R=0.000000,G=0.658824,B=1.000000,A=1.000000)" 2.0)
  (Utilities|FlowControl|Sequence
    (:then_0
      (Components|Activation|Activate (Variables|Default|GetP_Fire) false)
      (Rendering|SetVisibility (Variables|Default|GetPointLight) true false)
      (CallFunction|ManageActivationFire))
    (:then_1
      (Timeline|FlickeringTimeline Play
        (:Update
          (Utilities|FlowControl|Sequence
            (:then_0
              (Rendering|Components|Light|SetIntensity (Variables|Default|GetPointLight) (Math|Float|Lerp (Variables|/Script/Engine.LightComponentBase|GetIntensity (Variables|Default|GetPointLight)) (Variables|Default|GetTargetIntensity) 0.5)))
            (:then_1
              (Utilities|FlowControl|Delay (Math|Random|RandomFloatinRange 0.05 0.1))
              (Variables|Default|SetTargetIntensity (Math|Random|RandomFloatinRange 2e+03 1.5e+04)))))))
    (:then_2
      (if (and (Variables|Default|GetisFireOn) (not (Variables|Default|GethasBeenInitialized)))
        (CallFunction|PlayThrowerAudio)))))

(event EventBeginPlay
  (if (Variables|Default|GetstartWithoutTrigger)
    (CallFunction|Initialization)))

(event EventTick
  (params (DeltaSeconds :type Float%20%28single-precision%29))
  (if (Variables|Default|Getinitialized?)
    (CallFunction|ManageActivationFire)))

(fn ConstructionScript)

(fn ManageActivationFire
  (if (Components|Activation|IsActive (Variables|Default|GetP_Fire))
    (Variables|Default|SetisFireOn true)
    (else
      (Variables|Default|SetisFireOn false))))

(fn ActivateFire
  (params (Activate :type Boolean))
  (Variables|Default|SetisFireOn Activate))

(fn PlayThrowerAudio
  (Audio|Components|Audio|Play (Variables|Default|GetAudio_LightUp) 0.0)
  (Audio|Components|Audio|Play (Variables|Default|GetAudio_Thrower) 0.0)
  (Variables|Default|SethasBeenInitialized true))