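; BP_BraseiroFire is a brazier fire actor with a flickering point light and ignition audio.
; A timeline eases light intensity halfway toward a target on each update, re-randomizing that target after short random delays.
; Tick mirrors the PFire particle's active state into IsFireOn and plays the light-up and thrower sounds once when first lit.
; ActivateFire only sets IsFireOn, which the next particle check overwrites.
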(event EventBeginPlay
  (Utilities|FlowControl|Sequence
    (:then_0
      (CallFunction|ManageActivationFire))
    (:then_1
      (Timeline|FlickeringTimeline Play
        (:Update
          (Utilities|FlowControl|Sequence
            (:then_0
              (Rendering|Components|Light|SetIntensity (Variables|Default|GetPointLight) (Math|Float|Lerp (Variables|/Script/Engine.LightComponentBase|GetIntensity (Variables|Default|GetPointLight)) (Variables|Default|GetTargetIntensity) 0.5)))
            (:then_1
              (Utilities|FlowControl|Delay (Math|Random|RandomFloatinRange 0.05 0.1))
              (Variables|Default|SetTargetIntensity (Math|Random|RandomFloatinRange 5e+01 3e+02)))))))))

(event EventTick
  (params (DeltaSeconds :type Float%20%28single-precision%29))
  (CallFunction|ManageActivationFire)
  (if (and (Variables|Default|GetisFireOn) (not (Variables|Default|GethasBeenInitialized)))
    (CallFunction|PlayThrowerAudio)))

(fn ConstructionScript)

(fn ManageActivationFire
  (if (Components|Activation|IsActive (Variables|Default|GetP_Fire))
    (Variables|Default|SetisFireOn true)
    (else
      (Variables|Default|SetisFireOn false))))

(fn ActivateFire
  (params (Activate :type Boolean))
  (Variables|Default|SetisFireOn Activate))

(fn PlayThrowerAudio
  (Audio|Components|Audio|Play (Variables|Default|GetAudio_LightUp) 0.0)
  (Audio|Components|Audio|Play (Variables|Default|GetAudio_Thrower) 0.0)
  (Variables|Default|SethasBeenInitialized true))