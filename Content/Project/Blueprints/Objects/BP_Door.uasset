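; BP_Door is a usable object that opens an entry door once when used.
; It overrides UseObject, calls the parent logic, then checks a HasBeenOpen flag.
; On first use it plays a button sound at its location and runs the Sequencer_EntryDoor level sequence through a newly created player.
; It then marks its object info struct as used and sets the flag to block replays.
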(fn ConstructionScript
  (|CallParentFunction))

(fn UseObject
  (|CallParentFunction)
  (if (not (Variables|Default|GethasBeenOpen))
    (Audio|PlaySoundatLocation "/Game/Project/Audio/SFX/Environment/Door/SoundCue/SC_ButtonDoor.SC_ButtonDoor" (Transformation|GetActorLocation) "0, 0, 0" 1.0 1.0 0.0 0 0 0)
    (bind _returnvalue (Sequencer|Player|CreateLevelSequencePlayer "/Game/Project/Environement/Sequencer/Sequencer_EntryDoor.Sequencer_EntryDoor"))
    (Sequencer|Player|Play _returnvalue :!class /Script/MovieScene.MovieSceneSequencePlayer)
    (Variables|Default|SetStruct_InfoObject (Utilities|Struct|MakeStruct_InfoObject true "NewEnumerator0"))
    (Variables|Default|SethasBeenOpen true)))