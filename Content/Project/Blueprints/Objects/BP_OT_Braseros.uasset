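; BP_OT_Braseros is a triggered set piece that lights paired left and right braziers in sequence once the player enters its box.
; Tick accumulates a timer and initializes the next pair from the two brazier arrays at each interval, stopping after the last.
; The final pair waits over twice as long, then also spawns two horde enemies at fixed distances along the actor's right vector.
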(event OnComponentBeginOverlap(Box)
  (params (OverlappedComponent :type Primitive%20Component%20Object%20Reference) (OtherActor :type Actor%20Object%20Reference) (OtherComp :type Primitive%20Component%20Object%20Reference) (OtherBodyIndex :type Integer) (bFromSweep :type Boolean) (SweepResult :type Hit%20Result%20Structure%20%28by%20ref%29))
  (Utilities|Casting|CastToBP_PlayerCharacter OtherActor)
  (Variables|Default|SetstartFireAll true))

(event Custom|StartNewLine
  (Default|Initialization (Utilities|Array|Get(acopy) (Variables|Default|GettabBraseroLeft) (Variables|Default|GetNbLineToStart)))
  (Variables|Default|SetcurrentTimerBetweenStart 0.0))

(event EventBeginPlay
  (|CallParentFunction) ; This node is disabled and will not be called.\nDrag off pins to build functionality.
)

(event Collision|EventActorBeginOverlap
  (params (OtherActor :type Actor%20Object%20Reference))
  (|CallParentFunction OtherActor) ; This node is disabled and will not be called.\nDrag off pins to build functionality.
)

(event EventTick
  (params (DeltaSeconds :type Float%20%28single-precision%29))
  (|CallParentFunction DeltaSeconds)
  (if (Variables|Default|GetstartFireAll)
    (if (not (Variables|Default|Getfinished?))
      (if (< (Variables|Default|GetNbLineToStart) (Utilities|Array|Length (Variables|Default|GettabBraseroLeft)))
        (if (== (Variables|Default|GetNbLineToStart) (- (Utilities|Array|Length (Variables|Default|GettabBraseroLeft)) 1))
          (if (< (Variables|Default|GetcurrentTimerBetweenStart) (* (Variables|Default|GettimerBetweenStart) 2.3))
            (Variables|Default|SetcurrentTimerBetweenStart (+ (Variables|Default|GetcurrentTimerBetweenStart) (Utilities|Time|GetWorldDeltaSeconds)))
            (else
              (CallFunction|StartNewLine)
              (Math|Integer|IncrementInt (Variables|Default|GetNbLineToStart)
                (:%20%20
                  (Game|SpawnActorfromClass "/Game/Project/Blueprints/AI/Characters/BP_EnemiBase_Horde.BP_EnemiBase_Horde_C" (Math|Transform|MakeTransform (+ (Transformation|GetActorLocation) (* (Transformation|GetActorRightVector) 5e+03)) "0,-90.000000, 0" "1,1,1") "Undefined" 0 false "NewEnumerator5" 0 1e+02 false false 0)
                  (Game|SpawnActorfromClass "/Game/Project/Blueprints/AI/Characters/BP_EnemiBase_Horde.BP_EnemiBase_Horde_C" (Math|Transform|MakeTransform (+ (Transformation|GetActorLocation) (* (Transformation|GetActorRightVector) 8e+03)) "0,-90.000000, 0" "1,1,1") "Undefined" 0 false "NewEnumerator5" 0 1e+02 false false 0)))))
          (elif (< (Variables|Default|GetcurrentTimerBetweenStart) (Variables|Default|GettimerBetweenStart))
            (Variables|Default|SetcurrentTimerBetweenStart (+ (Variables|Default|GetcurrentTimerBetweenStart) (Utilities|Time|GetWorldDeltaSeconds)))
            (else
              (CallFunction|StartNewLine)
              (Math|Integer|IncrementInt (Variables|Default|GetNbLineToStart)))))
        (else
          (Variables|Default|Setfinished? true))))))

(fn ConstructionScript
  (|CallParentFunction))