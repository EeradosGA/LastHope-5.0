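; Pressure plate object that opens a linked door when the player character steps on it.
; A Box begin-overlap passes the actor to CheckPlayerOnPlate, which filters for BP_PlayerCharacter and checks Activable.
; If the plate is activable and DoorToOpen is valid, it sets the door's NeedOpen flag and calls UseObject, with debug prints reporting the activation state.
; Nothing handles stepping off, so the plate itself never closes the door.
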(event OnComponentBeginOverlap(Box)
  (params (OverlappedComponent :type Primitive%20Component%20Object%20Reference) (OtherActor :type Actor%20Object%20Reference) (OtherComp :type Primitive%20Component%20Object%20Reference) (OtherBodyIndex :type Integer) (bFromSweep :type Boolean) (SweepResult :type Hit%20Result%20Structure%20%28by%20ref%29))
  (CallFunction|CheckPlayeronPlate OtherActor))

(fn ConstructionScript
  (|CallParentFunction))

(fn CheckPlayeronPlate
  (params (Object :type Object%20Object%20Reference))
  (bind _doortoopen (Variables|Default|GetdoorToOpen))
  (Utilities|Casting|CastToBP_PlayerCharacter Object)
  (if (Variables|Default|Getactivable)
    (Development|PrintString "activating trigger")
    (Utilities|IsValid _doortoopen
      (:Is%20Valid
        (Variables|/Game/Project/Blueprints/Objects/BP_Door.BP_Door_C|SetneedOpen _doortoopen true)
        (Default|UseObject _doortoopen)))
    (else
      (Development|PrintString "not activable"))))