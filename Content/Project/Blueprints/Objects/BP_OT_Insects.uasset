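; Scarab swarm hazard that damages the player inside its box unless the player's equipped ring is active.
; Each tick it feeds the active ring's position and controller forward vector to the beetle Niagara system, driving swarm avoidance.
; Overlapping players without an active ring lose health on a cooldown, with camera shake and an on-face insect sound.
; That sound stops on ring activation, on leaving the box, or shortly after death.
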(event OnComponentEndOverlap(Box)
  (params (OverlappedComponent :type Primitive%20Component%20Object%20Reference) (OtherActor :type Actor%20Object%20Reference) (OtherComp :type Primitive%20Component%20Object%20Reference) (OtherBodyIndex :type Integer))
  (Utilities|Casting|CastToBP_PlayerCharacter OtherActor)
  (Variables|Default|SetsoundPlayedAway false)
  (Audio|Components|Audio|Stop (Variables|Default|GetS_InsectsOnFace)))

(event EventBeginPlay
  (|CallParentFunction)
  (Audio|Components|Audio|Play (Variables|Default|GetS_InsectsIdle) 0.0))

(event Collision|EventActorBeginOverlap
  (params (OtherActor :type Actor%20Object%20Reference))
  (|CallParentFunction OtherActor) ; This node is disabled and will not be called.\nDrag off pins to build functionality.
)

(event EventTick
  (params (DeltaSeconds :type Float%20%28single-precision%29))
  (|CallParentFunction DeltaSeconds)
  (CallFunction|CheckOverlapInsects)
  (CallFunction|UpdateCooldownDamage))

(fn ConstructionScript
  (|CallParentFunction))

(fn CheckOverlapInsects
  (bind _returnvalue (Game|GetPlayerController 0))
  (bind _fx_beetleswarm (Variables|Default|GetFX_BeetleSwarm))
  (bind _box (Variables|Default|GetBox))
  (bind _returnvalue_2 (Transformation|GetActorForwardVector _returnvalue))
  (bind _overlappingactors (Collision|GetOverlappingActors _box "/Game/Project/Blueprints/BP_PlayerCharacter.BP_PlayerCharacter_C" :!class /Script/Engine.PrimitiveComponent))
  (bind _output (Utilities|Array|Get(acopy) _overlappingactors))
  (bind _asbp_player_character (Utilities|Casting|CastToBP_PlayerCharacter _output))
  (bind _acp_weapon (Variables|/Game/Project/Blueprints/BP_PlayerCharacter.BP_PlayerCharacter_C|GetACP_Weapon _asbp_player_character))
  (bind _currentring (Variables|/Game/Project/Blueprints/Items/ACP_Weapon.ACP_Weapon_C|GetCurrentRing _acp_weapon))
  (Utilities|FlowControl|Sequence
    (:then_0
      (bind _asbp_player_character_2 (Utilities|Casting|CastToBP_PlayerCharacter (Pawn|GetControlledPawn _returnvalue)))
      (if (Utilities|IsValid (.AsBP%20Ring (Utilities|Casting|CastToBP_Ring (Variables|/Game/Project/Blueprints/Items/ACP_Weapon.ACP_Weapon_C|GetCurrentRing (Variables|/Game/Project/Blueprints/BP_PlayerCharacter.BP_PlayerCharacter_C|GetACP_Weapon _asbp_player_character_2)))))
        (if (Variables|/Game/Project/Blueprints/Items/ItemEquip/BP_Ring.BP_Ring_C|GetisActivate (.AsBP%20Ring (Utilities|Casting|CastToBP_Ring (Variables|/Game/Project/Blueprints/Items/ACP_Weapon.ACP_Weapon_C|GetCurrentRing (Variables|/Game/Project/Blueprints/BP_PlayerCharacter.BP_PlayerCharacter_C|GetACP_Weapon _asbp_player_character_2)))))
          (Niagara|SetNiagaraVariable(Float) _fx_beetleswarm "User_AvoidIntensity" 1e+01)
          (Class|NiagaraComponent|SetNiagaraVariableVec3 _fx_beetleswarm "User_LightStartPos" (Transformation|GetActorLocation (Variables|/Game/Project/Blueprints/Items/ACP_Weapon.ACP_Weapon_C|GetCurrentRing (Variables|/Game/Project/Blueprints/BP_PlayerCharacter.BP_PlayerCharacter_C|GetACP_Weapon _asbp_player_character_2))))
          (Niagara|SetNiagaraVariable(Vector3) _fx_beetleswarm "User_LightEndPos" (+ (Transformation|GetActorLocation (Variables|/Game/Project/Blueprints/Items/ACP_Weapon.ACP_Weapon_C|GetCurrentRing (Variables|/Game/Project/Blueprints/BP_PlayerCharacter.BP_PlayerCharacter_C|GetACP_Weapon _asbp_player_character_2))) (* _returnvalue_2 1e+03)))
          (Class|NiagaraComponent|SetNiagaraVariableVec3 _fx_beetleswarm "User_LightAxis" (Math|Vector|VectorGetAbs _returnvalue_2))
          (else
            (Niagara|SetNiagaraVariable(Float) _fx_beetleswarm "User_AvoidIntensity" 0.0)))))
    (:then_1
      (if (> (Utilities|Array|Length _overlappingactors) 0)
        (if (not (Variables|Default|GethaveDamagePlayer))
          (Utilities|IsValid _currentring
            (:Is%20Valid
              (Utilities|FlowControl|Sequence
                (:then_0
                  (if (Variables|/Game/Project/Blueprints/Items/ItemEquip/BP_Ring.BP_Ring_C|GetisActivate (.AsBP%20Ring (Utilities|Casting|CastToBP_Ring _currentring)))
                    (Development|PrintString "scarab runaway" true true "(R=0.000000,G=0.660000,B=1.000000,A=1.000000)" 0.001)
                    (Audio|Components|Audio|Stop (Variables|Default|GetS_InsectsOnFace))
                    (if (not (Variables|Default|GetsoundPlayedAway))
                      (Variables|Default|SetsoundPlayedAway true))
                    (else
                      (Variables|/Game/Project/Blueprints/BP_PlayerCharacter.BP_PlayerCharacter_C|SetCurrentHp _asbp_player_character (- (Variables|/Game/Project/Blueprints/BP_PlayerCharacter.BP_PlayerCharacter_C|GetCurrentHp _asbp_player_character) (Variables|Default|Getdamage)) :!label _label)
                      (Development|PrintString "scarab damage player" true true "(R=0.000000,G=0.660000,B=1.000000,A=1.000000)" 1.0)
                      (Variables|Default|SethaveDamagePlayer true)
                      (Variables|Default|SetsoundPlayedAway false)
                      (Default|CameraShakeHitScarab (.AsBP%20Player%20Character (Utilities|Casting|CastToBP_PlayerCharacter (Game|GetPlayerCharacter 0))))
                      (if (> (Variables|/Game/Project/Blueprints/BP_PlayerCharacter.BP_PlayerCharacter_C|GetCurrentHP _asbp_player_character) 0.0)
                        (if (not (Audio|Components|Audio|IsPlaying (Variables|Default|GetS_InsectsOnFace)))
                          (Audio|Components|Audio|Play (Variables|Default|GetS_InsectsOnFace) 0.0))))))
                (:then_1
                  (if (<= (Variables|/Game/Project/Blueprints/BP_PlayerCharacter.BP_PlayerCharacter_C|GetCurrentHP _asbp_player_character) 0.0)
                    (Audio|Components|Audio|StopDelayed (Variables|Default|GetS_InsectsOnFace) 1.5)))))
            (:Is%20Not%20Valid
              (goto _label))))
        (elif (Variables|Default|GethaveDamagePlayer)
          (Variables|Default|SethaveDamagePlayer false))))))

(fn UpdateCooldownDamage
  (if (Variables|Default|GethaveDamagePlayer)
    (bind _output_get (Variables|Default|SetcooldownDamage (- (Variables|Default|GetcooldownDamage) (Utilities|Time|GetWorldDeltaSeconds))))
    (if (<= _output_get 0.0)
      (Variables|Default|SethaveDamagePlayer false)
      (Variables|Default|SetcooldownDamage 0.1))))