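; Actor component on BP_PlayerCharacter that manages the player's weapon, ring and bracelet.
; Equipping swaps the class on child actor components passed in by InitWeapon, then sets owner and current references; rings and bracelets equip only into empty slots and activate energy bars.
; Attacks and item use forward to the equipped actors and set use flags.
; Heavy and slight attacks block each other; nothing here clears those flags.
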(event EventBeginPlay
  (bind _asbp_player_character (Utilities|Casting|CastToBP_PlayerCharacter (Components|GetOwner)))
  (Variables|Default|SetRefPlayer _asbp_player_character))

(fn InitWeapon
  (params (RefPlayer :type BP%20Player%20Character%20Object%20Reference) (ChildWeapon :type Child%20Actor%20Component%20Object%20Reference) (ChildRing :type Child%20Actor%20Component%20Object%20Reference) (ChildBracelet :type Child%20Actor%20Component%20Object%20Reference))
  (Variables|Default|SetRefPlayer RefPlayer)
  (Variables|Default|SetChildWeapon ChildWeapon)
  (Variables|Default|SetChildRing ChildRing)
  (Variables|Default|SetChildBracelet ChildBracelet))

(fn EquipWeapon
  (params (ItemWeapon :type BP%20Item%20Object%20Reference) (ItemWeaponClass :type BP%20Item%20Class%20Reference))
  (bind _childweapon (Variables|Default|GetChildWeapon))
  (ChildActorComponent|SetChildActorClass _childweapon ItemWeaponClass)
  (bind _asbp_weapon (Utilities|Casting|CastToBP_Weapon (Variables|/Script/Engine.ChildActorComponent|GetChildActor _childweapon)))
  (Variables|/Game/Project/Blueprints/Items/BP_Item.BP_Item_C|SetOwnerRef _asbp_weapon (Variables|Default|GetRefPlayer))
  (Variables|/Game/Project/Blueprints/Items/BP_Item.BP_Item_C|SetisPick? _asbp_weapon true)
  (Variables|Weapon|SetCurrentWeapon _asbp_weapon)
  (Variables|Weapon|SetWeaponEquip? true)
  (bind _asbp_sword (Utilities|Casting|CastToBP_Sword _asbp_weapon))
  (Default|PickedUp _asbp_sword)
  (Default|UpdateSurbrillance _asbp_weapon))

(fn EquipItemEquip
  (params (ItemEquipClass :type Actor%20Class%20Reference) (TypeItemEquip :type Enum_TypeItemEquip%20Enum :default "NewEnumerator0"))
  (switch Utilities|FlowControl|Switch|SwitchonEnum_TypeItemEquip TypeItemEquip
    (:NewEnumerator0
      (if (not (Variables|ItemEquip|Ring|GetRingEquip?))
        (Audio|PlaySound2D "/Game/Project/Audio/SFX/Environment/GettingRing/SC_GettingRingEvent.SC_GettingRingEvent" 1.0 1.0 0.0 0 0)
        (Variables|ItemEquip|Ring|SetRingEquip? true)
        (LocalVariables|SetChildNeed (Variables|Default|GetChildRing))
        (ChildActorComponent|SetChildActorClass (LocalVariables|GetChildNeed) ItemEquipClass)
        (bind _asbp_item_equip (Utilities|Casting|CastToBP_ItemEquip (Variables|/Script/Engine.ChildActorComponent|GetChildActor (LocalVariables|GetChildNeed))))
        (Utilities|IsValid (Variables|/Game/Project/Blueprints/Items/BP_Item.BP_Item_C|GetRotatingMovement _asbp_item_equip)
          (:Is%20Valid
            (Components|DestroyComponent (Variables|/Game/Project/Blueprints/Items/BP_Item.BP_Item_C|GetRotatingMovement _asbp_item_equip)))
          (:Is%20Not%20Valid
            _))
        (Variables|/Game/Project/Blueprints/Items/BP_Item.BP_Item_C|SetOwnerRef _asbp_item_equip (Variables|Default|GetRefPlayer))
        (Variables|ItemEquip|Ring|SetCurrentRing _asbp_item_equip)
        (CallFunction|ActivateRingBarEnergy)
        (Default|UpdateSurbrillance _asbp_item_equip)))
    (:NewEnumerator1
      (if (not (Variables|ItemEquip|Bracelet|GetBraceletEquip?))
        (Variables|ItemEquip|Bracelet|SetBraceletEquip? true)
        (LocalVariables|SetChildNeed (Variables|Default|GetChildBracelet))
        (ChildActorComponent|SetChildActorClass (LocalVariables|GetChildNeed) ItemEquipClass)
        (bind _asbp_item_equip_2 (Utilities|Casting|CastToBP_ItemEquip (Variables|/Script/Engine.ChildActorComponent|GetChildActor (LocalVariables|GetChildNeed))))
        (Utilities|IsValid (Variables|/Game/Project/Blueprints/Items/BP_Item.BP_Item_C|GetRotatingMovement _asbp_item_equip_2)
          (:Is%20Valid
            (Components|DestroyComponent (Variables|/Game/Project/Blueprints/Items/BP_Item.BP_Item_C|GetRotatingMovement _asbp_item_equip_2)))
          (:Is%20Not%20Valid
            _))
        (Variables|/Game/Project/Blueprints/Items/BP_Item.BP_Item_C|SetOwnerRef _asbp_item_equip_2 (Variables|Default|GetRefPlayer))
        (Variables|ItemEquip|Bracelet|SetCurrentBracelet _asbp_item_equip_2)
        (CallFunction|ActivateBraceletBarEnergy)
        (Default|UpdateSurbrillance _asbp_item_equip_2)))))

(fn AttackHeavy
  (bind _currentweapon (Variables|Weapon|GetCurrentWeapon))
  (if (not (or (Variables|Weapon|GetUseHeavyAttack?) (Variables|Weapon|GetUseSlightAttack?)))
    (Utilities|IsValid _currentweapon
      (:Is%20Valid
        (Default|AttackHeavy _currentweapon)
        (Variables|Weapon|SetUseHeavyAttack? true)
        (Variables|Weapon|SetUseSlightAttack? false)))))

(fn AttackSlight
  (bind _currentweapon (Variables|Weapon|GetCurrentWeapon))
  (if (not (or (Variables|Weapon|GetUseHeavyAttack?) (Variables|Weapon|GetUseSlightAttack?)))
    (Utilities|IsValid _currentweapon
      (:Is%20Valid
        (Default|AttackSlight _currentweapon)
        (Variables|Weapon|SetUseSlightAttack? true)
        (Variables|Weapon|SetUseHeavyAttack? false)))))

(fn UseItemEquip
  (params (TypeItemEquip :type Enum_TypeItemEquip%20Enum :default "NewEnumerator0"))
  (switch Utilities|FlowControl|Switch|SwitchonEnum_TypeItemEquip TypeItemEquip
    (:NewEnumerator0
      (LocalVariables|SetChildNeed (Variables|Default|GetChildRing))
      (Variables|ItemEquip|Ring|SetUseRing? true))
    (:NewEnumerator1
      (LocalVariables|SetChildNeed (Variables|Default|GetChildBracelet))
      (Variables|ItemEquip|Bracelet|SetUseBracelet? true)))
  (bind _asbp_item_equip (Utilities|Casting|CastToBP_ItemEquip (Variables|/Script/Engine.ChildActorComponent|GetChildActor (LocalVariables|GetChildNeed))))
  (Class|InterfaceUseItem|UseItemEquip(Message) _asbp_item_equip))