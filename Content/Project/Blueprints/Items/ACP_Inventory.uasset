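; Player inventory component that records picked-up item classes and reacts to each pickup by item type.
; AddItem stores the class, then switches on the type: weapons and equippable items go to the weapon component supplied through InitInventory, while treasure only plays a sound.
; Weapon pickups also notify the game instance, and backpacks set an ownership flag and switch off the player mesh's material glow.
; Most pickups play a 2D sound.
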(event EventBeginPlay)

(event EventTick
  (params (DeltaSeconds :type Float%20%28single-precision%29)))

(fn InitInventory
  (params (ACP%20Weapon :type ACP%20Weapon%20Object%20Reference))
  (Variables|Default|SetACP%20Weapon ACP%20Weapon))

(fn AddItem
  (params (ItemAdd :type BP%20Item%20Object%20Reference) (ItemClass :type BP%20Item%20Class%20Reference))
  (bind _acp_weapon (Variables|Default|GetACP%20Weapon))
  (Utilities|Array|Add (Variables|Default|GetlistItemClass) ItemClass)
  (Development|PrintString "add item")
  (switch Utilities|FlowControl|Switch|SwitchonEnum_TypeItem (.typeitem (Variables|/Game/Project/Blueprints/Items/BP_Item.BP_Item_C|GetStruct%20InfoItem ItemAdd))
    (:NewEnumerator0
      (Default|EquipWeapon _acp_weapon 0 ItemClass)
      (Audio|PlaySound2D "/Game/Project/Audio/SFX/Environment/GettingWeapon/SC_GetSword.SC_GetSword" 1.0 1.0 0.0 0 0)
      (Development|PrintString "equip zeqpon")
      (bind _asbp_last_hope_game_instance (Utilities|Casting|CastToBP_LastHopeGameInstance (Game|GetGameInstance)))
      (Default|CallTriggerWeaponPickup _asbp_last_hope_game_instance))
    (:NewEnumerator1
      (bind _asbp_item_equip (Utilities|Casting|CastToBP_ItemEquip ItemAdd))
      (Default|EquipItemEquip _acp_weapon ItemClass (Variables|/Game/Project/Blueprints/Items/BP_ItemEquip.BP_ItemEquip_C|GetTypeItemEquip _asbp_item_equip))
      (if (Utilities|Enum|Equal(Enum) (Variables|/Game/Project/Blueprints/Items/BP_ItemEquip.BP_ItemEquip_C|GetTypeItemEquip _asbp_item_equip) "NewEnumerator1")
        (Audio|PlaySound2D "/Game/Project/Audio/SFX/Environment/GettingBracelet/SC_GettingBracelet.SC_GettingBracelet" 1.0 1.0 0.0 0 0)))
    (:NewEnumerator2
      (Audio|PlaySound2D "/Game/Project/Audio/SFX/Entity/Player/Foley/SoundCue/SC_PlayerFoleyMovement.SC_PlayerFoleyMovement" 1.0 1.0 0.0 0 0))
    (:NewEnumerator3
      (Variables|Default|SethaveBackpack? true)
      (Audio|PlaySound2D "/Game/Project/Audio/SFX/Entity/Player/Foley/SoundCue/SC_CarryBag.SC_CarryBag" 1.0 1.0 0.0 0 0)
      (Rendering|Material|SetScalarParameterValueonMaterials (Variables|/Game/Project/Blueprints/BP_PlayerCharacter.BP_PlayerCharacter_C|GetSM_ThirdPerson (.AsBP%20Player%20Character (Utilities|Casting|CastToBP_PlayerCharacter (Game|GetPlayerCharacter 0)))) "Glow Strength" 0.0))))