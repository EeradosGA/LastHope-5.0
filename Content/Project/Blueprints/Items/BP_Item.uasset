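; BP_Item is an item actor, apparently for pickup, with optional spinning set up in its construction script.
; That script either applies a configured rotation rate to RotatingMovement or destroys the component.
; The event graph is inert: its events do nothing.
; Unconnected chains hold the former pickup detection, which used Box overlaps to set the player's ItemOverlaped and Collided and toggle a W_PopUpTuto prompt.
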(event OnComponentBeginOverlap(Box)
  (params (OverlappedComponent :type Primitive%20Component%20Object%20Reference) (OtherActor :type Actor%20Object%20Reference) (OtherComp :type Primitive%20Component%20Object%20Reference) (OtherBodyIndex :type Integer) (bFromSweep :type Boolean) (SweepResult :type Hit%20Result%20Structure%20%28by%20ref%29))
  ;[1 1 1] Collider for PICKUP
)

(event OnComponentEndOverlap(Box)
  (params (OverlappedComponent :type Primitive%20Component%20Object%20Reference) (OtherActor :type Actor%20Object%20Reference) (OtherComp :type Primitive%20Component%20Object%20Reference) (OtherBodyIndex :type Integer))
  ;[1 1 1] Collider for PICKUP
)

(event Custom|UpdateSurbrillance)

(event EventBeginPlay)

(event EventTick
  (params (DeltaSeconds :type Float%20%28single-precision%29))
  (if (Variables|Default|GetisPick?)
    _))

(fn ConstructionScript
  (if (Variables|Default|GetIsRotate?)
    (Variables|/Script/Engine.RotatingMovementComponent|SetRotationRate (Variables|Default|GetRotatingMovement) (Variables|Default|GetVectorRotation))
    (else
      (Components|DestroyComponent (Variables|Default|GetRotatingMovement)))))