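; BP_Weapon is a weapon item Blueprint, largely a skeleton, with a Box collision component and placeholder attack functions.
; AttackHeavy and AttackSlight only print debug strings, and the box's overlap event has no logic.
; Two helper functions check whether a given enemy is in ListEnnemiHit or a given arm is in ListArm, though nothing here fills those lists or calls the helpers.
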(event OnComponentBeginOverlap(Box)
  (params (OverlappedComponent :type Primitive%20Component%20Object%20Reference) (OtherActor :type Actor%20Object%20Reference) (OtherComp :type Primitive%20Component%20Object%20Reference) (OtherBodyIndex :type Integer) (bFromSweep :type Boolean) (SweepResult :type Hit%20Result%20Structure%20%28by%20ref%29)))

(event EventBeginPlay)

(event Collision|EventActorBeginOverlap
  (params (OtherActor :type Actor%20Object%20Reference)))

(event EventTick
  (params (DeltaSeconds :type Float%20%28single-precision%29))
  (|CallParentFunction DeltaSeconds))

(fn ConstructionScript
  (|CallParentFunction))

(fn AttackHeavy
  (Development|PrintString "Attack Heavy!"))

(fn AttackSlight
  (Development|PrintString "Attack Slight!"))

(fn ContainsEnnemi?
  (params (EnemiToFind :type BP%20Enemi%20Base%20Object%20Reference%20%28by%20ref%29))
  (return (Utilities|Array|ContainsItem (Variables|Default|GetListEnnemiHit) EnemiToFind)))

(fn ContainsArm?
  (params (Arm :type Bp%20Boss%20Arm%20Template%20Object%20Reference))
  (return (Utilities|Array|ContainsItem (Variables|Default|GetListArm) Arm)))