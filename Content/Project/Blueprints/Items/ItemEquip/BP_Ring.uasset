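; BP_Ring is an equippable ring item that powers a scarab light from a limited, rechargeable energy pool.
; Using it requires enough Power and plays a sound; releasing it or running out makes the child BP_ScarabLight disappear.
; Tick drains Power in timed steps while active, refills it when released, and feeds the ratio to the scarab's emissive.
; SetIntensityFromPower converts Power into normal and spot light target intensities.
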(event EventBeginPlay)

(event Collision|EventActorBeginOverlap
  (params (OtherActor :type Actor%20Object%20Reference)))

(event EventTick
  (params (DeltaSeconds :type Float%20%28single-precision%29))
  (|CallParentFunction DeltaSeconds)
  (if (Variables|Default|GetisPick?)
    (bind _asbp_scarab_light (Utilities|Casting|CastToBP_ScarabLight (Variables|/Script/Engine.ChildActorComponent|GetChildActor (Variables|Default|GetChildActor))))
    (Default|UpdateEmissive _asbp_scarab_light (/ (Variables|Stats|GetPower) (Variables|Stats|GetMaxPower)))
    (if (and (Variables|Default|GetisActivate) (Variables|Default|GetAnimOk?))
      ;[1 1 1] Healing
      (if (> (Variables|Stats|GetPower) 0.0)
        (bind _output_get (Variables|Stats|SetCurrentTimeLosePower (+ (Variables|Stats|GetCurrentTimeLosePower) (Utilities|Time|GetWorldDeltaSeconds))))
        (if (> _output_get (Variables|Stats|GetTimeToLosePower))
          (Variables|Stats|SetPower (- (Variables|Stats|GetPower) (Variables|Stats|GetNbPowerUpdate)))
          (Variables|Stats|SetCurrentTimeLosePower 0.0)
          (CallFunction|SetIntensityfromPower))
        (else
          (Variables|Default|SetisActivate false)
          (Variables|Stats|SetCurrentTimeLosePower 0.0)
          (bind _asbp_scarab_light_2 (Utilities|Casting|CastToBP_ScarabLight (Variables|/Script/Engine.ChildActorComponent|GetChildActor (Variables|Default|GetChildActor))))
          (Default|Disappear _asbp_scarab_light_2)))
      (else
        ;[1 1 1] UnActivate
        (if (not (Variables|Default|GetIsPress?))
          (bind _output_get_2 (Variables|Stats|SetCurrentTimeLosePower (+ (Variables|Stats|GetCurrentTimeLosePower) (Utilities|Time|GetWorldDeltaSeconds))))
          (if (> _output_get_2 (Variables|Stats|GetTimeToUpPower))
            (Variables|Stats|SetCurrentTimeLosePower 0.0)
            (if (< (Variables|Stats|GetPower) 1e+02)
              (Variables|Stats|SetPower (+ (Variables|Stats|GetPower) (Variables|Stats|GetNbPowerUpdate)))
              (CallFunction|SetIntensityfromPower))))))))

(event EventUpdateSurbrillance
  (Rendering|Material|SetScalarParameterValueonMaterials (Variables|Default|GetStaticMesh) "Glow Strength" 0.0))

(event EventUseItemEquip
  (if (not (< (Variables|Stats|GetPower) (* 2 (Variables|Stats|GetNbPowerUpdate))))
    (Variables|Default|SetisActivate true)
    (Variables|Default|SetIsPress? true)
    (Audio|PlaySound2D "/Game/Project/Audio/SFX/Entity/Player/Ring/ActiveRing_/SC_ActiveRing_Insects.SC_ActiveRing_Insects" 1.0 1.0 0.0 0 0)))

(event EventStopUseItemEquip
  (Variables|Default|SetisActivate false)
  (Variables|Default|SetIsPress? false)
  (Audio|PlaySound2D "/Game/Project/Audio/SFX/Entity/Player/Ring/SC_DeactiveRing.SC_DeactiveRing" 1.0 1.0 0.0 0 0)
  (bind _asbp_scarab_light (Utilities|Casting|CastToBP_ScarabLight (Variables|/Script/Engine.ChildActorComponent|GetChildActor (Variables|Default|GetChildActor))))
  (Default|Disappear _asbp_scarab_light))

(fn ConstructionScript
  (bind _staticmesh (Variables|Default|GetStaticMesh))
  (|CallParentFunction)
  (Variables|Stats|SetPower (Variables|Stats|GetMaxPower))
  (CallFunction|SetIntensityfromPower)
  (if (Variables|Default|GetisPick?)
    (Transformation|SetWorldScale3D _staticmesh "1.000000,1.000000,1.000000")
    (else
      (Transformation|SetWorldScale3D _staticmesh "2.900000,2.900000,2.900000"))))

(fn SetIntensityfromPower
  (bind _maxintensity (Variables|Stats|GetMaxIntensity))
  (bind _maxpower (Variables|Stats|GetMaxPower))
  (bind _power (Variables|Stats|GetPower))
  (bind _returnvalue (/ _power _maxpower))
  (bind _returnvalue_2 (* _maxintensity _returnvalue))
  (if (!= _returnvalue_2 (Variables|Stats|GetTargetIntensityNormal))
    (if (>= _returnvalue_2 (Variables|Stats|GetMinIntensity))
      (bind _output_get (Variables|Stats|SetTargetIntensityNormal _returnvalue_2))
      (if (!= (Variables|Stats|GetPower) 0.0)
        (Variables|Stats|SetTargetIntensitySpot (* (Variables|Stats|GetIntensitySpotMultipleFromNormal) _output_get))
        (else
          (Variables|Stats|SetTargetIntensitySpot 0.0))))))