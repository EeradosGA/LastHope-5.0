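; BP_Bracelet is an equippable item that heals its owner in pulses while in use, drawing on a limited reserve.
; Use and stop events toggle healing; Tick timers, gated by AnimOk, move reserve points into owner HP with a Niagara burst.
; The reserve recharges over time whenever healing is inactive.
; The construction script enlarges the mesh when not picked, and UpdateSurbrillance zeroes its glow.
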(event EventBeginPlay)

(event Collision|EventActorBeginOverlap
  (params (OtherActor :type Actor%20Object%20Reference)))

(event EventTick
  (params (DeltaSeconds :type Float%20%28single-precision%29))
  (bind _ownerref (Variables|Default|GetOwnerRef))
  (bind _ownerref_2 (Variables|Default|GetOwnerRef))
  (|CallParentFunction DeltaSeconds)
  (if (and (Variables|General|GetisHealing?) (Variables|Default|GetAnimOk?))
    ;[1 1 1] Healing
    (if (and (!= (Variables|/Game/Project/Blueprints/BP_PlayerCharacter.BP_PlayerCharacter_C|GetCurrentHP _ownerref_2) (Variables|/Game/Project/Blueprints/BP_PlayerCharacter.BP_PlayerCharacter_C|GetMaxHp _ownerref_2)) (> (Variables|General|GetHealLeft) 0.0))
      (bind _output_get (Variables|Healing|SetCurrentTimeHeal (+ (Variables|Healing|GetCurrentTimeHeal) (Utilities|Time|GetWorldDeltaSeconds))))
      (if (> _output_get (Variables|Healing|GetTimeToHeal))
        (Variables|General|SetHealLeft (- (Variables|General|GetHealLeft) 1e+01))
        (Variables|Healing|SetCurrentTimeHeal 0.0)
        (Variables|/Game/Project/Blueprints/BP_PlayerCharacter.BP_PlayerCharacter_C|SetCurrentHP _ownerref (+ (Variables|/Game/Project/Blueprints/BP_PlayerCharacter.BP_PlayerCharacter_C|GetCurrentHP _ownerref) 1e+01))
        (Components|Activation|Activate (Variables|Default|GetNiagara) true)))
    (else
      (bind _output_get_2 (Variables|RegeneHeal|SetCurrentTimeUpHeal (+ (Variables|RegeneHeal|GetCurrentTimeUpHeal) (Utilities|Time|GetWorldDeltaSeconds))))
      (if (> _output_get_2 (Variables|RegeneHeal|GetTimeToUpHeal))
        (Variables|RegeneHeal|SetCurrentTimeUpHeal 0.0)
        (if (< (Variables|General|GetHealLeft) 1e+02)
          (Variables|General|SetHealLeft (+ (Variables|General|GetHealLeft) 1e+01)))))))

(event EventUpdateSurbrillance
  (Rendering|Material|SetScalarParameterValueonMaterials (Variables|Default|GetStaticMesh) "Glow Strength" 0.0))

(event EventStopUseItemEquip
  (Variables|General|SetisHealing? false)
  (Development|PrintString "Stop Heal"))

(event EventUseItemEquip
  (Variables|General|SetisHealing? true)
  (Variables|Healing|SetCurrentTimeHeal 0.0)
  (Development|PrintString "Heal"))

(fn ConstructionScript
  (bind _staticmesh (Variables|Default|GetStaticMesh))
  (|CallParentFunction)
  (if (Variables|Default|GetisPick?)
    (Transformation|SetWorldScale3D _staticmesh "1.000000,1.000000,1.000000")
    (else
      (Transformation|SetWorldScale3D _staticmesh "2.200000,2.200000,2.200000"))))