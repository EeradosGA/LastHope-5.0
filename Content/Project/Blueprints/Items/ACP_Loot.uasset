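; ACP_Loot is an actor component that drops loot items at its owner's location.
; SpawnLoot spawns every class in ListItemOfLoot slightly below the valid owner's position and clears IsPick on each spawned item.
; Each spawn prints a debug message with its index.
; A random drop-chance check is left disconnected, so every listed item spawns whenever SpawnLoot runs.
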(event EventBeginPlay)

(event EventTick
  (params (DeltaSeconds :type Float%20%28single-precision%29)))

(fn SpawnLoot
  (bind _returnvalue (Components|GetOwner))
  (bind _listitemofloot (Variables|Default|GetlistItemOfLoot))
  (if (> (Utilities|Array|Length _listitemofloot) 0)
    (for (_array_element _array_index) _listitemofloot
      (Utilities|IsValid _returnvalue
        (:Is%20Valid
          (bind _returnvalue_2 (Game|SpawnActorfromClass _array_element (Math|Transform|MakeTransform (- (Transformation|GetActorLocation _returnvalue) "0, 0,15.000000") "0, 0, 0" "1,1,1") "Undefined" 0 0))
          (Variables|/Game/Project/Blueprints/Items/BP_Item.BP_Item_C|SetisPick? _returnvalue_2 false)
          (Development|PrintString (Utilities|String|Append "spawn loot " (Utilities|String|ToString(Integer) _array_index))))))))