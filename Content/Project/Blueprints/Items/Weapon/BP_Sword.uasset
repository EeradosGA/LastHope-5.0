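; Sword weapon Blueprint with a blade and bracelet that damages enemies and boss arms, using separate light and heavy attack damage.
; Tick dissolves the blade away after an idle delay and back in when needed.
; While a hit is active, it polls hitbox overlaps, tracking targets to avoid repeat damage, with sounds per hit type.
; Sand-wound impact FX spawn for horde enemies and for sword enemies not blocking.
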(event Custom|PickedUp
  (Collision|SetCollisionEnabled (Variables|Default|GetLame) "NoCollision"))

(event EventBeginPlay)

(event Collision|EventActorBeginOverlap
  (params (OtherActor :type Actor%20Object%20Reference)))

(event EventTick
  (params (DeltaSeconds :type Float%20%28single-precision%29))
  (bind _ownerref (Variables|Default|GetOwnerRef))
  (bind _acp_weapon (Variables|/Game/Project/Blueprints/BP_PlayerCharacter.BP_PlayerCharacter_C|GetACP_Weapon _ownerref))
  (|CallParentFunction DeltaSeconds)
  (if (and (Variables|Default|GetNeedShow?) (Variables|Default|GetIsHide?))
    (bind _output_get (Variables|Default|SetCurrentTimeHide (+ (Variables|Default|GetCurrentTimeHide) (/ (Utilities|Time|GetWorldDeltaSeconds) (Variables|Default|GetTimeHide)))))
    (Rendering|Material|SetScalarParameterValueonMaterials (Variables|Default|GetLame) "Dissolve Amount" (Math|Float|Lerp 1.0 -1.0 _output_get))
    (if (> (Variables|Default|GetCurrentTimeHide) 1.0)
      (Variables|Default|SetCurrentTimeToHide 0.0)
      (Variables|Default|SetCurrentTimeHide 0.0)
      (Variables|Default|SetNeedShow? false)
      (Variables|Default|SetIsHide? false))
    (else
      ;[1 1 1] System Hide Blade
      (bind _output_get_2 (Variables|Default|SetCurrentTimeToHide (+ (Utilities|Time|GetWorldDeltaSeconds) (Variables|Default|GetCurrentTimeToHide))))
      (if (> _output_get_2 (Variables|Default|GetTimeToHide))
        (if (Variables|Default|GetIsHide?)
          _
          (else
            (bind _output_get_3 (Variables|Default|SetCurrentTimeHide (+ (Variables|Default|GetCurrentTimeHide) (/ (Utilities|Time|GetWorldDeltaSeconds) (Variables|Default|GetTimeHide)))))
            (Rendering|Material|SetScalarParameterValueonMaterials (Variables|Default|GetLame) "Dissolve Amount" (Math|Float|Lerp -1.0 1.0 _output_get_3))
            (if (> (Variables|Default|GetCurrentTimeHide) 1.0)
              (Variables|Default|SetCurrentTimeToHide 0.0)
              (Variables|Default|SetCurrentTimeHide 0.0)
              (Variables|Default|SetIsHide? true)
              (Variables|Default|SetNeedShow? false)))))))
  ;[1 1 1] Chich Hit
  (if (Variables|Default|GetisHit?)
    (Utilities|FlowControl|Sequence
      (:then_0
        (for _array_element (Collision|GetOverlappingActors (Variables|Default|GetBoxHit) "/Game/Project/Blueprints/AI/Characters/BP_EnemiBase.BP_EnemiBase_C" :!class /Script/Engine.PrimitiveComponent)
          (bind _asbp_enemi_base (Utilities|Casting|CastToBP_EnemiBase _array_element))
          (bind _returnvalue (CallFunction|ContainsEnnemi? _asbp_enemi_base))
          (if (not _returnvalue)
            (CallFunction|GetImpact _asbp_enemi_base)
            (Utilities|Array|Add (Variables|Default|GetListEnnemiHit) _asbp_enemi_base)
            (if (Variables|/Game/Project/Blueprints/Items/ACP_Weapon.ACP_Weapon_C|GetUseHeavyAttack? _acp_weapon)
              (Audio|PlaySound2D "/Game/Project/Audio/SFX/Entity/Commun/Attack/SoundCue/SC_SwordAttackImpactBody_High.SC_SwordAttackImpactBody_High" 1.0 1.0 0.0 0 0)
              (Class|ICombat|TakeDamage(Message) _asbp_enemi_base (.damage (Variables|Default|GetStruct%20Weapon)) "NewEnumerator2")
              (CallFunction|Print "NewEnumerator2" 0 "Hit" true true "(R=0.000000,G=0.658824,B=1.000000,A=1.000000)" 2.0 :!label _label)
              (elif (Variables|/Game/Project/Blueprints/Items/ACP_Weapon.ACP_Weapon_C|GetUseSlightAttack? _acp_weapon)
                (Audio|PlaySound2D "/Game/Project/Audio/SFX/Entity/Commun/Attack/SoundCue/SC_SwordAttackImpactBody_Low.SC_SwordAttackImpactBody_Low" 1.0 1.0 0.0 0 0)
                (Class|ICombat|TakeDamage(Message) _asbp_enemi_base (.damage (Variables|Default|GetStruct%20Weapon)) "NewEnumerator1")
                (goto _label))))))
      (:then_1
        (for _array_element_2 (Collision|GetOverlappingActors (Variables|Default|GetBoxHit) "/Game/Project/Blueprints/AI/Boss/Bp_BossArm_Template.Bp_BossArm_Template_C" :!class /Script/Engine.PrimitiveComponent)
          (bind _asbp_boss_arm_template (Utilities|Casting|CastToBp_BossArm_Template _array_element_2))
          (bind _returnvalue_2 (CallFunction|ContainsArm? _asbp_boss_arm_template))
          (if (not _returnvalue_2)
            (Utilities|Array|Add (Variables|Default|GetListArm) _asbp_boss_arm_template)
            (Default|TakeDamageArm _asbp_boss_arm_template (.damage (Variables|Default|GetStruct%20Weapon)))
            (Audio|PlaySound2D "/Game/Project/Audio/SFX/Entity/Enemy/Armed/SC_SwordLightHitShield.SC_SwordLightHitShield" 1.0 (Math|Random|RandomFloatinRange 0.65 0.9) 0.0 0 0)))))))

(event EventUpdateSurbrillance
  (Rendering|Material|SetScalarParameterValueonMaterials (Variables|Default|GetLame) "Glow Strength" 0.0))

(fn ConstructionScript
  (bind _bracelet (Variables|Default|GetBracelet))
  (|CallParentFunction)
  (if (Variables|Default|GetisPick?)
    (Transformation|SetWorldScale3D _bracelet "1.000000,1.000000,1.000000")
    (else
      (Transformation|SetWorldScale3D _bracelet "1.750000,1.750000,1.750000"))))

(fn AttackHeavy
  (|CallParentFunction)
  (Variables|Default|SetStruct%20Weapon (Utilities|Struct|MakeStruct_Weapon 65.0 "(listAnimCombo_3_D8BE2E424C85829BC0A3C2AD1843B799=)")))

(fn AttackSlight
  (|CallParentFunction)
  (Variables|Default|SetStruct%20Weapon (Utilities|Struct|MakeStruct_Weapon 35.0 "(listAnimCombo_3_D8BE2E424C85829BC0A3C2AD1843B799=)")))

(fn GetImpact
  (params (Enemi :type BP%20Enemi%20Base%20Object%20Reference))
  (bind _returnvalue (Transformation|GetActorLocation Enemi))
  (switch Utilities|FlowControl|Switch|SwitchonE_NPCBehavoir (Variables|/Game/Project/Blueprints/AI/Characters/BP_EnemiBase.BP_EnemiBase_C|GetBehavior Enemi)
    (:NewEnumerator5
      (Niagara|SpawnSystematLocation "/Game/Project/FX/Systems/Validé/FX_EnemySandWound.FX_EnemySandWound" (- _returnvalue (* (- _returnvalue (Transformation|GetWorldLocation (Variables|Default|GetLame))) 0.5)) :!label _label))
    (:NewEnumerator6
      (bind _asbp_ennemi_weapon (Utilities|Casting|CastToBP_EnnemiWeapon Enemi))
      (if (not (Variables|/Game/Project/Blueprints/AI/Characters/BP_EnnemiWeapon.BP_EnnemiWeapon_C|GetIsProtecting? _asbp_ennemi_weapon))
        (goto _label)))))