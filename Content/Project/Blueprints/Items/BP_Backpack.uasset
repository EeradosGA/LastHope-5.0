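; BP_Backpack is a backpack item actor whose mesh can be highlighted with a glow.
; It toggles the "Glow Strength" material parameter on its StaticMesh, starting with the glow off at BeginPlay.
; ActivateSurbrillance turns the glow on, while UpdateSurbrillance switches it back off rather than refreshing it.
; Nothing in this Blueprint calls either event, and its construction script only runs the parent's.
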(event Custom|ActivateSurbrillance
  (Rendering|Material|SetScalarParameterValueonMaterials (Variables|Default|GetStaticMesh) "Glow Strength" 1.0))

(event EventBeginPlay
  (|CallParentFunction)
  (Rendering|Material|SetScalarParameterValueonMaterials (Variables|Default|GetStaticMesh) "Glow Strength" 0.0))

(event Collision|EventActorBeginOverlap
  (params (OtherActor :type Actor%20Object%20Reference))
  (|CallParentFunction OtherActor) ; This node is disabled and will not be called.\nDrag off pins to build functionality.
)

(event EventTick
  (params (DeltaSeconds :type Float%20%28single-precision%29))
  (|CallParentFunction DeltaSeconds) ; This node is disabled and will not be called.\nDrag off pins to build functionality.
)

(event EventUpdateSurbrillance
  (Rendering|Material|SetScalarParameterValueonMaterials (Variables|Default|GetStaticMesh) "Glow Strength" 0.0))

(fn ConstructionScript
  (|CallParentFunction))