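; Global is a function library of debug print helpers that show messages only for the developer currently selected in the game.
; Dev Print, its Print wrapper and the append variant compare a Developper enum against CurrentDevelopper on BP_LastHopeGameInstance, fetched by GetInstance, before calling PrintString.
; Calls left on the unselected enum value print an orange warning instead.
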(fn DevPrint
  (params (Developper :type Enum_Developper%20Enum :default "NewEnumerator9") (World%20Context%20Object :type Object%20Object%20Reference) (In%20String :type String) (Print%20To%20Screen :type Boolean) (Print%20To%20Log :type Boolean) (Text%20Color :type Linear%20Color%20Structure :default "(R=0.000000,G=0.658824,B=1.000000,A=1.000000)") (Duration :type Float%20%28single-precision%29))
  (if (Utilities|Enum|Equal(Enum) Developper "NewEnumerator9")
    (Development|PrintString 0 "Global / Dev Print --> No Developper selected for this print" true true "(R=1.000000,G=0.500000,B=0.000000,A=1.000000)" 4.0)
    (elif (Utilities|Enum|Equal(Enum) (Variables|/Game/Project/Blueprints/BP_LastHopeGameInstance.BP_LastHopeGameInstance_C|GetCurrentDevelopper (CallFunction|GetInstance)) Developper)
      (Development|PrintString World%20Context%20Object In%20String Print%20To%20Screen Print%20To%20Log Text%20Color Duration))))

(fn GetInstance
  (return (.AsBP%20Last%20Hope%20Game%20Instance (Utilities|Casting|CastToBP_LastHopeGameInstance (Game|GetGameInstance)))))

(fn Print
  (params (Developper :type Enum_Developper%20Enum :default "NewEnumerator9") (World%20Context%20Object :type Object%20Object%20Reference) (In%20String :type String) (Print%20To%20Screen :type Boolean) (Print%20To%20Log :type Boolean) (Text%20Color :type Linear%20Color%20Structure :default "(R=0.000000,G=0.658824,B=1.000000,A=1.000000)") (Duration :type Float%20%28single-precision%29))
  (CallFunction|DevPrint Developper World%20Context%20Object In%20String Print%20To%20Screen Print%20To%20Log Text%20Color Duration))

(fn DevPrintwithAppend
  (params (Developper :type Enum_Developper%20Enum :default "NewEnumerator9") (World%20Context%20Object :type Object%20Object%20Reference) (String%20: :type String) (Value :type String) (Print%20To%20Screen :type Boolean) (Print%20To%20Log :type Boolean) (Text%20Color :type Linear%20Color%20Structure :default "(R=0.000000,G=0.658824,B=1.000000,A=1.000000)") (Duration :type Float%20%28single-precision%29))
  (if (Utilities|Enum|Equal(Enum) Developper "NewEnumerator9")
    (Development|PrintString 0 "Global / Dev Print --> No Developper selected for this print" true true "(R=1.000000,G=0.500000,B=0.000000,A=1.000000)" 4.0)
    (elif (Utilities|Enum|Equal(Enum) (Variables|/Game/Project/Blueprints/BP_LastHopeGameInstance.BP_LastHopeGameInstance_C|GetCurrentDevelopper (CallFunction|GetInstance)) Developper)
      (Development|PrintString World%20Context%20Object (Utilities|String|Append String%20: Value) Print%20To%20Screen Print%20To%20Log Text%20Color Duration))))