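; Room encounter trigger that spawns a hard-coded enemy group when the player first enters its active box, or when TriggerSpawn is called.
; It creates a BP_CombatDirector, spawns one of two groups (chosen by IsFirst) at tagged spawn points matched by Index, then starts combat.
; The first group also starts a music fade, and a temporary Tick poll switches music once those enemies are gone; the second group's music check is unconnected.
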(event OnComponentBeginOverlap(Box)
  (params (OverlappedComponent :type Primitive%20Component%20Object%20Reference) (OtherActor :type Actor%20Object%20Reference) (OtherComp :type Primitive%20Component%20Object%20Reference) (OtherBodyIndex :type Integer) (bFromSweep :type Boolean) (SweepResult :type Hit%20Result%20Structure%20%28by%20ref%29))
  (if (Variables|Default|GetisActive?)
    (if (and (== (Utilities|GetClass OtherActor) "/Game/Project/Blueprints/BP_PlayerCharacter.BP_PlayerCharacter_C") (not (Variables|Default|GethasBeenTriggered?)))
      (Variables|Default|SethasBeenTriggered? true)
      (bind _returnvalue (Game|SpawnActorfromClass "/Game/Project/Blueprints/AI/Behavior/BP_CombatDirector.BP_CombatDirector_C" (Transformation|GetActorTransform self) "AlwaysSpawn" 0 0))
      (Variables|Default|SetCombatDirector _returnvalue)
      (if (Variables|Default|GetisFirst?)
        (bind _array_element (Utilities|Array|ForEachLoopwithBreak (Variables|Default|GetSpawnPoints) :!label _label)
          (:LoopBody
            (if (== (Variables|/Game/Project/Blueprints/AI/BP_SpawnPoint.BP_SpawnPoint_C|GetIndex _array_element) 1)
              (bind _returnvalue_2 (Game|SpawnActorfromClass "/Game/Project/Blueprints/AI/Characters/BP_EnnemiWeapon.BP_EnnemiWeapon_C" (Transformation|GetActorTransform _array_element) "Undefined" 0 "NewEnumerator6" 0 1e+02 false true 0))
              (Utilities|Array|Add (Variables|Default|GetEnemyArrayFirst) _returnvalue_2)
              (goto _label Break)))
          (:Completed
            (bind _array_element_2 (Utilities|Array|ForEachLoopwithBreak (Variables|Default|GetSpawnPoints) :!label _label_2)
              (:LoopBody
                (if (== (Variables|/Game/Project/Blueprints/AI/BP_SpawnPoint.BP_SpawnPoint_C|GetIndex _array_element_2) 2)
                  (bind _returnvalue_3 (Game|SpawnActorfromClass "/Game/Project/Blueprints/AI/Characters/BP_EnemiBase_Horde.BP_EnemiBase_Horde_C" (Transformation|GetActorTransform _array_element_2) "Undefined" 0 false "NewEnumerator5" 0 1e+02 false false 0))
                  (Utilities|Array|Add (Variables|Default|GetEnemyArrayFirst) _returnvalue_3)
                  (Utilities|Array|Add (Variables|/Game/Project/Blueprints/AI/Behavior/BP_CombatDirector.BP_CombatDirector_C|GetEnemyList (Variables|Default|GetCombatDirector)) 0)
                  (goto _label_2 Break)))
              (:Completed
                (bind _array_element_3 (Utilities|Array|ForEachLoopwithBreak (Variables|Default|GetSpawnPoints) :!label _label_3)
                  (:LoopBody
                    (if (== (Variables|/Game/Project/Blueprints/AI/BP_SpawnPoint.BP_SpawnPoint_C|GetIndex _array_element_3) 3)
                      (bind _returnvalue_4 (Game|SpawnActorfromClass "/Game/Project/Blueprints/AI/Characters/BP_EnemiBase_Horde.BP_EnemiBase_Horde_C" (Transformation|GetActorTransform _array_element_3) "Undefined" 0 false "NewEnumerator5" 0 1e+02 false false 0))
                      (Utilities|Array|Add (Variables|Default|GetEnemyArrayFirst) _returnvalue_4)
                      (Utilities|Array|Add (Variables|/Game/Project/Blueprints/AI/Behavior/BP_CombatDirector.BP_CombatDirector_C|GetEnemyList (Variables|Default|GetCombatDirector)) 0)
                      (goto _label_3 Break)))
                  (:Completed
                    (Default|InitCombat (Variables|Default|GetCombatDirector))
                    (Development|PrintString "Init firrst combat !!!!!!!!!!!!!!")
                    (Variables|Default|SetHasSpawn1 true)
                    (bind _returnvalue_5 (Actor|GetActorOfClass "/Game/Project/Audio/BP_MusicPlayer.BP_MusicPlayer_C"))
                    (Default|PlayMusicFade _returnvalue_5 "NewEnumerator2" 2.0 2.0 0.0)))))))
        (else
          (bind _array_element_4 (Utilities|Array|ForEachLoopwithBreak (Variables|Default|GetSpawnPoints) :!label _label_4)
            (:LoopBody
              (if (== (Variables|/Game/Project/Blueprints/AI/BP_SpawnPoint.BP_SpawnPoint_C|GetIndex _array_element_4) 2)
                (bind _returnvalue_6 (Game|SpawnActorfromClass "/Game/Project/Blueprints/AI/Characters/BP_EnnemiWeapon.BP_EnnemiWeapon_C" (Transformation|GetActorTransform _array_element_4) "Undefined" 0 "NewEnumerator6" 0 1e+02 false false 0))
                (Utilities|Array|Add (Variables|Default|GetEnemyArraySecond) _returnvalue_6)
                (Utilities|Array|Add (Variables|/Game/Project/Blueprints/AI/Behavior/BP_CombatDirector.BP_CombatDirector_C|GetEnemyList (Variables|Default|GetCombatDirector)) _returnvalue_6)
                (goto _label_4 Break)))
            (:Completed
              (bind _array_element_5 (Utilities|Array|ForEachLoopwithBreak (Variables|Default|GetSpawnPoints) :!label _label_5)
                (:LoopBody
                  (if (== (Variables|/Game/Project/Blueprints/AI/BP_SpawnPoint.BP_SpawnPoint_C|GetIndex _array_element_5) 3)
                    (bind _returnvalue_7 (Game|SpawnActorfromClass "/Game/Project/Blueprints/AI/Characters/BP_EnnemiWeapon.BP_EnnemiWeapon_C" (Transformation|GetActorTransform _array_element_5) "Undefined" 0 "NewEnumerator6" 0 1e+02 false false 0))
                    (Utilities|Array|Add (Variables|Default|GetEnemyArraySecond) _returnvalue_7)
                    (Utilities|Array|Add (Variables|/Game/Project/Blueprints/AI/Behavior/BP_CombatDirector.BP_CombatDirector_C|GetEnemyList (Variables|Default|GetCombatDirector)) _returnvalue_7)
                    (goto _label_5 Break)))
                (:Completed
                  (Default|InitCombat (Variables|Default|GetCombatDirector))
                  (Variables|Default|SetHasSpawn2 true))))))))))

(event Custom|TriggerSpawn
  (Variables|Default|SethasBeenTriggered? true)
  (bind _returnvalue (Game|SpawnActorfromClass "/Game/Project/Blueprints/AI/Behavior/BP_CombatDirector.BP_CombatDirector_C" (Transformation|GetActorTransform self) "AlwaysSpawn" 0 0))
  (Variables|Default|SetCombatDirector _returnvalue)
  (if (Variables|Default|GetisFirst?)
    (bind _array_element (Utilities|Array|ForEachLoopwithBreak (Variables|Default|GetSpawnPoints) :!label _label)
      (:LoopBody
        (if (== (Variables|/Game/Project/Blueprints/AI/BP_SpawnPoint.BP_SpawnPoint_C|GetIndex _array_element) 1)
          (bind _returnvalue_2 (Game|SpawnActorfromClass "/Game/Project/Blueprints/AI/Characters/BP_EnnemiWeapon.BP_EnnemiWeapon_C" (Transformation|GetActorTransform _array_element) "Undefined" 0 "NewEnumerator6" 0 1e+02 false true 0))
          (Utilities|Array|Add (Variables|Default|GetEnemyArrayFirst) _returnvalue_2)
          (goto _label Break)))
      (:Completed
        (bind _array_element_2 (Utilities|Array|ForEachLoopwithBreak (Variables|Default|GetSpawnPoints) :!label _label_2)
          (:LoopBody
            (if (== (Variables|/Game/Project/Blueprints/AI/BP_SpawnPoint.BP_SpawnPoint_C|GetIndex _array_element_2) 2)
              (bind _returnvalue_3 (Game|SpawnActorfromClass "/Game/Project/Blueprints/AI/Characters/BP_EnemiBase_Horde.BP_EnemiBase_Horde_C" (Transformation|GetActorTransform _array_element_2) "Undefined" 0 false "NewEnumerator5" 0 1e+02 false false 0))
              (Utilities|Array|Add (Variables|Default|GetEnemyArrayFirst) _returnvalue_3)
              (Utilities|Array|Add (Variables|/Game/Project/Blueprints/AI/Behavior/BP_CombatDirector.BP_CombatDirector_C|GetEnemyList (Variables|Default|GetCombatDirector)) 0)
              (goto _label_2 Break)))
          (:Completed
            (bind _array_element_3 (Utilities|Array|ForEachLoopwithBreak (Variables|Default|GetSpawnPoints) :!label _label_3)
              (:LoopBody
                (if (== (Variables|/Game/Project/Blueprints/AI/BP_SpawnPoint.BP_SpawnPoint_C|GetIndex _array_element_3) 3)
                  (bind _returnvalue_4 (Game|SpawnActorfromClass "/Game/Project/Blueprints/AI/Characters/BP_EnemiBase_Horde.BP_EnemiBase_Horde_C" (Transformation|GetActorTransform _array_element_3) "Undefined" 0 false "NewEnumerator5" 0 1e+02 false false 0))
                  (Utilities|Array|Add (Variables|Default|GetEnemyArrayFirst) _returnvalue_4)
                  (Utilities|Array|Add (Variables|/Game/Project/Blueprints/AI/Behavior/BP_CombatDirector.BP_CombatDirector_C|GetEnemyList (Variables|Default|GetCombatDirector)) 0)
                  (goto _label_3 Break)))
              (:Completed
                (Default|InitCombat (Variables|Default|GetCombatDirector))
                (Development|PrintString "Init firrst combat !!!!!!!!!!!!!!")
                (Variables|Default|SetHasSpawn1 true)
                (bind _returnvalue_5 (Actor|GetActorOfClass "/Game/Project/Audio/BP_MusicPlayer.BP_MusicPlayer_C"))
                (Default|PlayMusicFade _returnvalue_5 "NewEnumerator2" 2.0 2.0 0.0)))))))
    (else
      (bind _array_element_4 (Utilities|Array|ForEachLoopwithBreak (Variables|Default|GetSpawnPoints) :!label _label_4)
        (:LoopBody
          (if (== (Variables|/Game/Project/Blueprints/AI/BP_SpawnPoint.BP_SpawnPoint_C|GetIndex _array_element_4) 2)
            (bind _returnvalue_6 (Game|SpawnActorfromClass "/Game/Project/Blueprints/AI/Characters/BP_EnnemiWeapon.BP_EnnemiWeapon_C" (Transformation|GetActorTransform _array_element_4) "Undefined" 0 "NewEnumerator6" 0 1e+02 false false 0))
            (Utilities|Array|Add (Variables|Default|GetEnemyArraySecond) _returnvalue_6)
            (Utilities|Array|Add (Variables|/Game/Project/Blueprints/AI/Behavior/BP_CombatDirector.BP_CombatDirector_C|GetEnemyList (Variables|Default|GetCombatDirector)) _returnvalue_6)
            (goto _label_4 Break)))
        (:Completed
          (bind _array_element_5 (Utilities|Array|ForEachLoopwithBreak (Variables|Default|GetSpawnPoints) :!label _label_5)
            (:LoopBody
              (if (== (Variables|/Game/Project/Blueprints/AI/BP_SpawnPoint.BP_SpawnPoint_C|GetIndex _array_element_5) 3)
                (bind _returnvalue_7 (Game|SpawnActorfromClass "/Game/Project/Blueprints/AI/Characters/BP_EnnemiWeapon.BP_EnnemiWeapon_C" (Transformation|GetActorTransform _array_element_5) "Undefined" 0 "NewEnumerator6" 0 1e+02 false false 0))
                (Utilities|Array|Add (Variables|Default|GetEnemyArraySecond) _returnvalue_7)
                (Utilities|Array|Add (Variables|/Game/Project/Blueprints/AI/Behavior/BP_CombatDirector.BP_CombatDirector_C|GetEnemyList (Variables|Default|GetCombatDirector)) _returnvalue_7)
                (goto _label_5 Break)))
            (:Completed
              (Default|InitCombat (Variables|Default|GetCombatDirector))
              (Variables|Default|SetHasSpawn2 true))))))))

(event EventBeginPlay
  (bind _outactors (Actor|GetAllActorsOfClasswithTag "/Game/Project/Blueprints/AI/BP_SpawnPoint.BP_SpawnPoint_C" (Variables|Default|GetSpawnTag)))
  (bind _output_get (Variables|Default|SetSpawnPoints _outactors))
  (CallFunction|DevPrintwithAppend "NewEnumerator1" 0 "foundPoints :" (Utilities|String|ToString(Integer) (Utilities|Array|Length _output_get)) true true "(R=0.000000,G=0.658824,B=1.000000,A=1.000000)" 2.0))

(event Collision|EventActorBeginOverlap
  (params (OtherActor :type Actor%20Object%20Reference)))

(event EventTick
  (params (DeltaSeconds :type Float%20%28single-precision%29))
  (CallFunction|ManageMusic(TMP)))

(fn ConstructionScript)

(fn ManageMusic(TMP)
  (Utilities|FlowControl|Sequence
    (:then_0
      (if (and (Variables|Default|GetHasSpawn1) (not (Variables|Default|GetMusicFight1Played)))
        (LocalVariables|SetStopMusic false)
        (for _array_element (Variables|Default|GetEnemyArrayFirst)
          (if (Utilities|IsValid _array_element)
            (LocalVariables|SetStopMusic true)))
        (if (not (LocalVariables|GetStopMusic))
          (bind _returnvalue (Actor|GetActorOfClass "/Game/Project/Audio/BP_MusicPlayer.BP_MusicPlayer_C"))
          (Default|PlayMusicFade _returnvalue "NewEnumerator6" 2.0 2.0 0.0)
          (Variables|Default|SetMusicFight1Played true))))))