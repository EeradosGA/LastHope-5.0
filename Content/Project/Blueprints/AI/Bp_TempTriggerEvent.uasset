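; Temporary trigger actor that signals a weapon pickup to the game instance when a player with a weapon is inside its sphere.
; Sphere overlap begin and end toggle HasBeenTriggered for BP_PlayerCharacter.
; While the flag is set, Tick polls overlapping players for a valid current weapon, calls CallTriggerWeaponPickup on BP_LastHopeGameInstance, then clears the flag.
; Despite the flag's name, re-entering the sphere re-arms the trigger.
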(event OnComponentBeginOverlap(Sphere)
  (params (OverlappedComponent :type Primitive%20Component%20Object%20Reference) (OtherActor :type Actor%20Object%20Reference) (OtherComp :type Primitive%20Component%20Object%20Reference) (OtherBodyIndex :type Integer) (bFromSweep :type Boolean) (SweepResult :type Hit%20Result%20Structure%20%28by%20ref%29))
  (if (not (Variables|Default|GetHasBeenTriggered?))
    (if (== (Utilities|GetClass OtherActor) "/Game/Project/Blueprints/BP_PlayerCharacter.BP_PlayerCharacter_C")
      (Variables|Default|SetHasBeenTriggered? true))))

(event OnComponentEndOverlap(Sphere)
  (params (OverlappedComponent :type Primitive%20Component%20Object%20Reference) (OtherActor :type Actor%20Object%20Reference) (OtherComp :type Primitive%20Component%20Object%20Reference) (OtherBodyIndex :type Integer))
  (Utilities|Casting|CastToBP_PlayerCharacter OtherActor)
  (Variables|Default|SetHasBeenTriggered? false))

(event EventBeginPlay)

(event Collision|EventActorBeginOverlap
  (params (OtherActor :type Actor%20Object%20Reference)))

(event EventTick
  (params (DeltaSeconds :type Float%20%28single-precision%29))
  (if (Variables|Default|GetHasBeenTriggered?)
    (for _array_element (Collision|GetOverlappingActors (Variables|Default|GetSphere) "/Game/Project/Blueprints/BP_PlayerCharacter.BP_PlayerCharacter_C" :!class /Script/Engine.PrimitiveComponent)
      (bind _asbp_player_character (Utilities|Casting|CastToBP_PlayerCharacter _array_element))
      (Utilities|IsValid (Variables|/Game/Project/Blueprints/Items/ACP_Weapon.ACP_Weapon_C|GetCurrentWeapon (Variables|/Game/Project/Blueprints/BP_PlayerCharacter.BP_PlayerCharacter_C|GetACP_Weapon _asbp_player_character))
        (:Is%20Valid
          (bind _asbp_last_hope_game_instance (Utilities|Casting|CastToBP_LastHopeGameInstance (Game|GetGameInstance)))
          (Default|CallTriggerWeaponPickup _asbp_last_hope_game_instance)
          (Variables|Default|SetHasBeenTriggered? false))))))

(fn ConstructionScript)