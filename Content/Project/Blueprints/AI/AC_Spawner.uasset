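; AC_Spawner is an actor component that spawns horde enemies for a combat zone and tracks how many remain.
; SpawnActors places a static leader BP_EnemiBase_Horde slightly above every BP_SpawnPoint with the given tag, counting each one.
; KillEvent decrements that count and tells the owning BP_ZoneCombat to remove its HUD at zero; its game instance binding is disconnected.
; It also stores and exposes whether the player is in the zone.
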(event Custom|SetPlayerInZone
  (params (IsInZone? :type Boolean))
  (Variables|Default|SetPlayerInZone? IsInZone?))

(event Custom|SpawnActors
  (params (Tag :type Name))
  (bind _outactors (Actor|GetAllActorsOfClasswithTag "/Game/Project/Blueprints/AI/BP_SpawnPoint.BP_SpawnPoint_C" Tag))
  (for _array_element _outactors
    (Game|SpawnActorfromClass "/Game/Project/Blueprints/AI/Characters/BP_EnemiBase_Horde.BP_EnemiBase_Horde_C" (Math|Transform|MakeTransform (Math|Vector|MakeVector (.X (Math|Vector|BreakVector (.location (Transformation|GetActorTransform _array_element)))) (.Y (Math|Vector|BreakVector (.location (Transformation|GetActorTransform _array_element)))) (+ (.Z (Math|Vector|BreakVector (.location (Transformation|GetActorTransform _array_element)))) 88.0)) (.rotation (Transformation|GetActorTransform _array_element)) (.scale (Transformation|GetActorTransform _array_element))) "AlwaysSpawn" 0 true "NewEnumerator5" 0 1e+02 true 0)
    (Math|Integer|IncrementInt (Variables|Default|GetEnemyCount))))

(event Custom|KillEvent
  (bind _enemycount (Variables|Default|GetEnemyCount))
  (Math|Integer|DecrementInt _enemycount
    (:%20%20
      (if (== _enemycount 0)
        (bind _asbp_zone_combat (Utilities|Casting|CastToBP_ZoneCombat (Components|GetOwner)))
        (Default|RemoveHud _asbp_zone_combat)))))

(event EventBeginPlay)

(event EventTick
  (params (DeltaSeconds :type Float%20%28single-precision%29)))

(fn GetIsPlayerinZone?
  (return (Variables|Default|GetPlayerInZone?)))