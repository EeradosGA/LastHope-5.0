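; Horde enemy character with glowing eyes and melee attacks against the player.
; On introduction the leader sets its anim blueprint to shout, while the others start their behavior.
; Light attacks play random montages whose notify sphere-traces from the right hand, applying damage through I_Combat with camera shake; DrawHitBox repeats this with caller-supplied damage.
; Hits interrupt montages with random reactions, eyes receive player position each tick, and death turns them off.
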(event EventBeginPlay
  (|CallParentFunction)
  (Utilities|FlowControl|Delay 2.0)
  (Components|Activation|Activate (Variables|Default|GetLeftEye) true)
  (Components|Activation|Activate (Variables|Default|GetRightEye) true))

(event Collision|EventActorBeginOverlap
  (params (OtherActor :type Actor%20Object%20Reference))
  (|CallParentFunction OtherActor) ; This node is disabled and will not be called.\nDrag off pins to build functionality.
)

(event EventTick
  (params (DeltaSeconds :type Float%20%28single-precision%29))
  (|CallParentFunction DeltaSeconds)
  (if (and (not (Variables|Default|GetIsBeeingDestroyed?)) (Variables|Default|GetIsSpawned?))
    (CallFunction|SendPlayerPositiontoGlowEyes (Variables|Default|GetLeftEye) (Variables|Default|GetRightEye))))

(event EventLightAttack
  (bind _mesh (Variables|Character|GetMesh))
  (bind _returnvalue (Transformation|GetSocketLocation _mesh "hand_rSocket"))
  ;[1 1 1] Melee LightAttack
  (if (not (Variables|Default|GetIsBeeingDestroyed?))
    (bind _output_get (Variables|Default|SetCurrentMontage (select (Math|Random|RandomBool) "/Game/Mannequin/Animations/With_Weapon/AM_NPCLightAttack2.AM_NPCLightAttack2" "/Game/Mannequin/Animations/With_Weapon/AM_NPCLightAttack1.AM_NPCLightAttack1")))
    (Animation|Montage|PlayMontage (Variables|Character|GetMesh) _output_get
      (:OnNotifyBegin
        (bind _outactors (Actor|GetAllActorsOfClass "/Game/Project/Blueprints/AI/Characters/BP_EnemiBase.BP_EnemiBase_C"))
        (bind (_outhit _returnvalue_2) (Collision|SphereTraceByChannel _returnvalue (+ _returnvalue (* (Math|Vector|GetForwardVector (Transformation|GetActorRotation)) 2e+01)) 2e+01 "TraceTypeQuery2" false _outactors "None"))
        (if (and _returnvalue_2 (== (Utilities|GetClass (.HitActor (Collision|BreakHitResult _outhit))) "/Game/Project/Blueprints/BP_PlayerCharacter.BP_PlayerCharacter_C"))
          (if (Utilities|DoesObjectImplementInterface (.HitActor (Collision|BreakHitResult _outhit)) "/Game/Project/Interface/I_Combat.I_Combat_C")
            (Class|ICombat|TakeDamage(Message) (.HitActor (Collision|BreakHitResult _outhit)) 1e+01 "NewEnumerator1")
            (bind _asbp_player_character (Utilities|Casting|CastToBP_PlayerCharacter (.HitActor (Collision|BreakHitResult _outhit))))
            (Default|CameraShakeHitEnemyLight _asbp_player_character)))))))

(event EventDrawHitBox
  (params (DammageValue :type Float%20%28single-precision%29) (AttackType :type E_AttackType%20Enum :default "NewEnumerator0"))
  (bind _mesh (Variables|Character|GetMesh))
  (bind _returnvalue (Transformation|GetSocketLocation _mesh "hand_rSocket"))
  (bind _outactors (Actor|GetAllActorsOfClass "/Game/Project/Blueprints/AI/Characters/BP_EnemiBase.BP_EnemiBase_C"))
  (bind (_outhit _returnvalue_2) (Collision|SphereTraceByChannel _returnvalue (+ _returnvalue (* (Math|Vector|GetForwardVector (Transformation|GetActorRotation)) 2e+01)) 2e+01 "TraceTypeQuery2" false _outactors "None"))
  (if (and _returnvalue_2 (== (Utilities|GetClass (.HitActor (Collision|BreakHitResult _outhit))) "/Game/Project/Blueprints/BP_PlayerCharacter.BP_PlayerCharacter_C"))
    (if (Utilities|DoesObjectImplementInterface (.HitActor (Collision|BreakHitResult _outhit)) "/Game/Project/Interface/I_Combat.I_Combat_C")
      (Class|ICombat|TakeDamage(Message) (.HitActor (Collision|BreakHitResult _outhit)) DammageValue AttackType)
      (bind _asbp_player_character (Utilities|Casting|CastToBP_PlayerCharacter (.HitActor (Collision|BreakHitResult _outhit))))
      (Default|CameraShakeHitEnemiHeavy _asbp_player_character))))

(event EventKillEnemy
  (bind _righteye (Variables|Default|GetRightEye))
  (bind _lefteye (Variables|Default|GetLeftEye))
  (|CallParentFunction)
  (Rendering|SetVisibility _lefteye false false)
  (Components|Activation|Deactivate _lefteye)
  (Rendering|SetVisibility _righteye false false)
  (Components|Activation|Deactivate _righteye))

(event EventIntroduce
  (|CallParentFunction)
  (if (Variables|Default|GetIsLeader?)
    (bind _asabp_enemy (Utilities|Casting|CastToABP_Enemy (Components|SkeletalMesh|GetAnimInstance (Variables|Character|GetMesh))))
    (Variables|/Game/Project/Animations/ABP_Enemy.ABP_Enemy_C|SetisShouting? _asabp_enemy true)
    (else
      (CallFunction|StartBehavior))))

(event EventHandleHitReaction
  (params (AttackType :type E_AttackType%20Enum :default "NewEnumerator0") (Value :type Float%20%28single-precision%29))
  (Animation|StopAnimMontage (Animation|GetCurrentMontage :!class /Script/Engine.Character))
  (Animation|Montage|PlayMontage (Variables|Character|GetMesh) (select (Math|Random|RandomBool) "/Game/Mannequin/Animations/With_Weapon/AM_NPCGetHit1.AM_NPCGetHit1" "/Game/Mannequin/Animations/With_Weapon/AM_NPCGetHit2.AM_NPCGetHit2")
    (:then
      (CallFunction|MakeDammages Value))))

(fn ConstructionScript
  (|CallParentFunction))