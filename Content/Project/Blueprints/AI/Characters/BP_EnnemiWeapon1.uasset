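; Sword-and-shield enemy character that starts its AI controller's behavior when introduced.
; Its light attack drops the shield, then a montage notify fires a sword-socket box trace that damages the player and shakes their camera.
; While shielded, one attack type triggers a block and another gets through; unshielded hits play a random reaction and deal damage.
; The heavy attack only plays a counter montage.
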(event Custom|DrawBox
  (params (Value :type Float%20%28single-precision%29) (AttackType :type E_AttackType%20Enum :default "NewEnumerator0"))
  (bind _mesh (Variables|Character|GetMesh))
  (bind _returnvalue (Transformation|GetSocketLocation _mesh "swordSocket"))
  (bind _outactors (Actor|GetAllActorsOfClass "/Game/Project/Blueprints/AI/Characters/BP_EnemiBase.BP_EnemiBase_C"))
  (bind (_outhit _returnvalue_2) (Collision|BoxTraceByChannel _returnvalue (+ _returnvalue (* (Math|Vector|GetForwardVector (Transformation|GetActorRotation)) 5e+01)) "15.000000,15.000000,15.000000" (Transformation|GetSocketRotation (Variables|Character|GetMesh) "swordSocket") "TraceTypeQuery2" false _outactors "None" true "(R=0.000000,G=0.214648,B=1.000000,A=1.000000)"))
  (if (not (Variables|Default|GetIsBeeingDestroyed?))
    (if (and _returnvalue_2 (== (Utilities|GetClass (.HitActor (Collision|BreakHitResult _outhit))) "/Game/Project/Blueprints/BP_PlayerCharacter.BP_PlayerCharacter_C"))
      (if (Utilities|DoesObjectImplementInterface (.HitActor (Collision|BreakHitResult _outhit)) "/Game/Project/Interface/I_Combat.I_Combat_C")
        (Class|ICombat|TakeDamage(Message) (.HitActor (Collision|BreakHitResult _outhit)) Value AttackType)
        (bind _asbp_player_character (Utilities|Casting|CastToBP_PlayerCharacter (.HitActor (Collision|BreakHitResult _outhit))))
        (Default|CameraShakeHitEnemiHeavy _asbp_player_character)))))

(event Custom|ToogleShieldFx
  (params (isVisible? :type Boolean))
  (Rendering|SetVisibility (Variables|Default|GetCylinder) isVisible? false)
  (Variables|Default|SetIsProtecting? isVisible?)
  (if isVisible?
    _))

(event EventBeginPlay
  (|CallParentFunction)
  (Variables|Default|SetBehavior "NewEnumerator6"))

(event Collision|EventActorBeginOverlap
  (params (OtherActor :type Actor%20Object%20Reference))
  (|CallParentFunction OtherActor) ; This node is disabled and will not be called.\nDrag off pins to build functionality.
)

(event EventTick
  (params (DeltaSeconds :type Float%20%28single-precision%29))
  (|CallParentFunction DeltaSeconds) ; This node is disabled and will not be called.\nDrag off pins to build functionality.
)

(event EventLightAttack
  (CallFunction|ToogleShieldFx false)
  (Animation|Montage|PlayMontage (Variables|Character|GetMesh) "/Game/Project/Animations/AM_SwordAttack.AM_SwordAttack"
    (:OnNotifyBegin
      (CallFunction|DrawBox 3e+01 "NewEnumerator1"))))

(event EventDrawHitBox
  (params (DammageValue :type Float%20%28single-precision%29) (AttackType :type E_AttackType%20Enum :default "NewEnumerator0")))

(event EventIntroduce
  (|CallParentFunction)
  (bind _asbp_aicontroller (Utilities|Casting|CastToBP_AIController (AI|GetAIController self)))
  (Default|BehaviorStart _asbp_aicontroller false))

(event EventHeavyAttack
  (Animation|Montage|PlayMontage 0 "/Game/Project/Animations/AM_CounterAttack.AM_CounterAttack"))

(event EventHandleHitReaction
  (params (AttackType :type E_AttackType%20Enum :default "NewEnumerator0") (Value :type Float%20%28single-precision%29))
  (if (Variables|Default|GetIsProtecting?)
    (if (Utilities|Enum|Equal(Enum) AttackType "NewEnumerator1")
      (Animation|StopAnimMontage (Animation|GetCurrentMontage :!class /Script/Engine.Character))
      (Animation|Montage|PlayMontage (Variables|Character|GetMesh) "/Game/Project/Animations/AM_BlockShield.AM_BlockShield")
      (elif (Utilities|Enum|Equal(Enum) AttackType "NewEnumerator2")
        (Animation|StopAnimMontage (Animation|GetCurrentMontage :!class /Script/Engine.Character))
        (Animation|Montage|PlayMontage (Variables|Character|GetMesh) (select (Math|Random|RandomBool) "/Game/Project/Animations/AM_SwordGetHit2.AM_SwordGetHit2" "/Game/Project/Animations/AM_SwordGetHit1.AM_SwordGetHit1")
          (:then
            (CallFunction|MakeDammages Value)))))
    (else
      (Animation|Montage|PlayMontage (Variables|Character|GetMesh) (select (Math|Random|RandomBool) "/Game/Project/Animations/AM_SwordGetHit2.AM_SwordGetHit2" "/Game/Project/Animations/AM_SwordGetHit1.AM_SwordGetHit1")
        (:then
          (CallFunction|MakeDammages Value))))))

(fn ConstructionScript
  (|CallParentFunction))