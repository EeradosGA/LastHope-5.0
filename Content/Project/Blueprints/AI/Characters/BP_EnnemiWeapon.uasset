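; Sword-and-shield enemy character that starts its AI behavior and eye effects when introduced and switches the eyes off on death.
; Light and heavy attacks box-trace from the sword socket, damaging the player through I_Combat and shaking the camera.
; A protecting flag drives the shield's dynamic material color and strength.
; While protecting, light hits trigger a block montage; heavy hits, or hits when unprotected, play random hit reactions and deal damage.
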(event Custom|DrawBox
  (params (Value :type Float%20%28single-precision%29) (AttackType :type E_AttackType%20Enum :default "NewEnumerator0"))
  (bind _mesh (Variables|Character|GetMesh))
  (bind _returnvalue (Transformation|GetSocketLocation _mesh "swordSocket"))
  (bind _outactors (Actor|GetAllActorsOfClass "/Game/Project/Blueprints/AI/Characters/BP_EnemiBase.BP_EnemiBase_C"))
  (bind (_outhit _returnvalue_2) (Collision|BoxTraceByChannel _returnvalue (+ _returnvalue (* (Math|Vector|GetForwardVector (Transformation|GetActorRotation)) 5e+01)) "15.000000,15.000000,15.000000" (Transformation|GetSocketRotation (Variables|Character|GetMesh) "swordSocket") "TraceTypeQuery2" false _outactors "Persistent" true "(R=0.000000,G=0.214648,B=1.000000,A=1.000000)"))
  (if (and _returnvalue_2 (== (Utilities|GetClass (.HitActor (Collision|BreakHitResult _outhit))) "/Game/Project/Blueprints/BP_PlayerCharacter.BP_PlayerCharacter_C"))
    (if (Utilities|DoesObjectImplementInterface (.HitActor (Collision|BreakHitResult _outhit)) "/Game/Project/Interface/I_Combat.I_Combat_C")
      (Class|ICombat|TakeDamage(Message) (.HitActor (Collision|BreakHitResult _outhit)) Value AttackType)
      (bind _asbp_player_character (Utilities|Casting|CastToBP_PlayerCharacter (.HitActor (Collision|BreakHitResult _outhit))))
      (Default|CameraShakeHitEnemiHeavy _asbp_player_character))))

(event Custom|ToogleShieldFx
  (params (isVisible? :type Boolean))
  (bind _m_equipement (Variables|Default|GetM_Equipement))
  (bind _m_equipement_2 (Variables|Default|GetM_Equipement))
  (Variables|Default|SetIsProtecting? isVisible?)
  (if isVisible?
    (Rendering|Material|SetScalarParameterValue _m_equipement "ShieldStrenght" 0.5 :!class /Script/Engine.MaterialInstanceDynamic)
    (Rendering|Material|SetVectorParameterValue _m_equipement "ShieldColor" "(R=1.000000,G=0.000000,B=0.000000,A=1.000000)" :!class /Script/Engine.MaterialInstanceDynamic)
    (else
      (Rendering|Material|SetScalarParameterValue _m_equipement_2 "ShieldStrenght" 1.0 :!class /Script/Engine.MaterialInstanceDynamic)
      (Rendering|Material|SetVectorParameterValue _m_equipement_2 "ShieldColor" "(R=0.000000,G=1.000000,B=0.000000,A=1.000000)" :!class /Script/Engine.MaterialInstanceDynamic))))

(event EventBeginPlay
  (|CallParentFunction)
  (Variables|Default|SetBehavior "NewEnumerator6")
  (bind _returnvalue (Rendering|Material|CreateDynamicMaterialInstance (Variables|Character|GetMesh) 1 "/Game/Project/Materials/EnemySwordTexturesMaterials/M_Enemyarme.M_Enemyarme" "None" :!class /Script/Engine.PrimitiveComponent))
  (Variables|Default|SetM_Equipement _returnvalue))

(event Collision|EventActorBeginOverlap
  (params (OtherActor :type Actor%20Object%20Reference))
  (|CallParentFunction OtherActor) ; This node is disabled and will not be called.\nDrag off pins to build functionality.
)

(event EventTick
  (params (DeltaSeconds :type Float%20%28single-precision%29))
  (|CallParentFunction DeltaSeconds) ; This node is disabled and will not be called.\nDrag off pins to build functionality.
)

(event EventLightAttack
  (CallFunction|ToogleShieldFx false)
  (Animation|Montage|PlayMontage (Variables|Character|GetMesh) "/Game/Project/Animations/AM_SwordAttack.AM_SwordAttack"
    (:OnNotifyBegin
      (CallFunction|DrawBox 2e+01 "NewEnumerator1"))))

(event EventDrawHitBox
  (params (DammageValue :type Float%20%28single-precision%29) (AttackType :type E_AttackType%20Enum :default "NewEnumerator0")))

(event EventKillEnemy
  (bind _righteye (Variables|Default|GetRightEye))
  (bind _lefteye (Variables|Default|GetLeftEye))
  (|CallParentFunction)
  (Rendering|SetVisibility _lefteye false false)
  (Components|Activation|Deactivate _lefteye)
  (Rendering|SetVisibility _righteye false false)
  (Components|Activation|Deactivate _righteye))

(event EventHeavyAttack
  (CallFunction|DrawBox 4e+01 "NewEnumerator2")
  (bind _asabp_enemy_weapon (Utilities|Casting|CastToABP_EnemyWeapon (Components|SkeletalMesh|GetAnimInstance (Variables|Character|GetMesh))))
  (Variables|/Game/Project/Animations/ABP_EnemyWeapon.ABP_EnemyWeapon_C|SetcounterAttack? _asabp_enemy_weapon false))

(event EventHandleHitReaction
  (params (AttackType :type E_AttackType%20Enum :default "NewEnumerator0") (Value :type Float%20%28single-precision%29))
  (if (Variables|Default|GetIsProtecting?)
    (if (Utilities|Enum|Equal(Enum) AttackType "NewEnumerator1")
      (Animation|StopAnimMontage (Animation|GetCurrentMontage :!class /Script/Engine.Character))
      (Animation|Montage|PlayMontage (Variables|Character|GetMesh) "/Game/Project/Animations/AM_BlockShield.AM_BlockShield"
        (:then
          (Audio|PlaySoundatLocation "/Game/Project/Audio/SFX/Entity/Enemy/Armed/SC_SwordHighHitShield.SC_SwordHighHitShield" (Transformation|GetActorLocation) "0, 0, 0" 1.0 1.0 0.0 0 0 0)))
      (elif (Utilities|Enum|Equal(Enum) AttackType "NewEnumerator2")
        (Animation|StopAnimMontage (Animation|GetCurrentMontage :!class /Script/Engine.Character))
        (Animation|Montage|PlayMontage (Variables|Character|GetMesh) (select (Math|Random|RandomBool) "/Game/Project/Animations/AM_SwordGetHit2.AM_SwordGetHit2" "/Game/Project/Animations/AM_SwordGetHit1.AM_SwordGetHit1")
          (:then
            (CallFunction|MakeDammages Value)
            (Audio|PlaySoundatLocation "/Game/Project/Audio/SFX/Entity/Enemy/Armed/SC_SwordLightHitShield.SC_SwordLightHitShield" (Transformation|GetActorLocation) "0, 0, 0" 1.0 1.0 0.0 0 0 0)))))
    (else
      (Animation|Montage|PlayMontage (Variables|Character|GetMesh) (select (Math|Random|RandomBool) "/Game/Project/Animations/AM_SwordGetHit2.AM_SwordGetHit2" "/Game/Project/Animations/AM_SwordGetHit1.AM_SwordGetHit1")
        (:then
          (CallFunction|MakeDammages Value)
          (Audio|PlaySoundatLocation "/Game/Project/Audio/SFX/Entity/Enemy/Armed/SC_SwordHighHitShield.SC_SwordHighHitShield" (Transformation|GetActorLocation) "0, 0, 0" 1.0 1.0 0.0 0 0 0))))))

(event EventIntroduce
  (|CallParentFunction)
  (bind _asbp_aicontroller (Utilities|Casting|CastToBP_AIController (AI|GetAIController self)))
  (Default|BehaviorStart _asbp_aicontroller false)
  (Components|Activation|SetActive (Variables|Default|GetLeftEye) true false)
  (Components|Activation|SetActive (Variables|Default|GetRightEye) true false))

(fn ConstructionScript
  (|CallParentFunction))