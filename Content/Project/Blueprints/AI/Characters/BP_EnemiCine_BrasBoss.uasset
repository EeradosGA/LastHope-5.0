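; BP_EnemiCine_BrasBoss is an enemy character, apparently for cinematics, that spawns and dies through visual effects.
; It tags itself "E" plus its Index and stays hidden unless IsAlreadySpawned.
; StartSpawn plays SpawnFX, then reveals the mesh after a delay and makes it destroyable.
; If destroyable, Startdestroy plays DeathFX, hides the mesh and disables capsule collision, then the actor destroys itself when that effect finishes.
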(event OnSystemFinished(DeathFX)
  (params (PSystem :type Niagara%20Component%20Object%20Reference))
  (Actor|DestroyActor))

(event Custom|Start%20destroy
  (if (Variables|Default|GetcanBeDestroyed?)
    (Components|Activation|Activate (Variables|Default|GetDeathFX) false)
    (Rendering|SetVisibility (Variables|Character|GetMesh) false false)
    (Collision|SetCollisionEnabled (Variables|Default|GetCapsuleComponent) "NoCollision")))

(event Custom|StartSpawn
  (Rendering|SetVisibility (Variables|Default|GetSpawnFX) true false)
  (Components|Activation|Activate (Variables|Default|GetSpawnFX) true)
  (Utilities|FlowControl|Delay 2.0)
  (Rendering|SetVisibility (Variables|Character|GetMesh) true false)
  (Variables|Default|SetcanBeDestroyed? true))

(event EventBeginPlay
  (Variables|Default|SetTags self (Utilities|Array|MakeArray (Utilities|String|StringToName (Utilities|String|Append "E" (Utilities|String|ToString(Integer) (Variables|Default|GetIndex))))))
  (if (not (Variables|Default|GetisAlreadySpawned?))
    (Rendering|SetVisibility (Variables|Character|GetMesh) false false)))

(event Collision|EventActorBeginOverlap
  (params (OtherActor :type Actor%20Object%20Reference)))

(event EventTick
  (params (DeltaSeconds :type Float%20%28single-precision%29)))

(fn ConstructionScript
  (bind _isalreadyspawned_ (Variables|Default|GetisAlreadySpawned?))
  (|CallParentFunction)
  (Rendering|SetVisibility (Variables|Character|GetMesh) _isalreadyspawned_ false)
  (Variables|Default|SetcanBeDestroyed? _isalreadyspawned_))