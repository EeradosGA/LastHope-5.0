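; AI controller for BP_EnemiBase pawns that runs patrol behavior and reacts to seeing the player.
; Shortly after BeginPlay it starts BT_NPCPatrol for NONE or PATROL behaviors and seeds BB_EnemyPawn with direction and the pawn's path looping flag.
; AI Perception target updates write player visibility and last stimulus location to the blackboard, with debug prints.
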(event OnTargetPerceptionUpdated(AIPerception)
  (params (Actor :type Actor%20Object%20Reference) (Stimulus :type AI%20Stimulus%20Structure))
  (bind (_age _expirationage _strength _stimuluslocation _receiverlocation _tag _bsuccessfullysensed) (Utilities|Struct|BreakAIStimulus Stimulus))
  (if (and (== (Utilities|GetClass Actor) "/Game/Project/Blueprints/BP_PlayerCharacter.BP_PlayerCharacter_C") _bsuccessfullysensed)
    (Development|PrintString "Can see player" true true "(R=0.000000,G=1.000000,B=0.000000,A=1.000000)")
    (AI|Components|Blackboard|SetValueasBool (AI|GetBlackboard 0) (Utilities|Name|MakeLiteralName "IsSeeingPlayer?") true)
    (AI|Components|Blackboard|SetValueasVector (AI|GetBlackboard 0) (Utilities|Name|MakeLiteralName "Destination") _stimuluslocation)
    (else
      (Development|PrintString "Cant see player" true true "(R=1.000000,G=0.000000,B=0.000000,A=1.000000)")
      (AI|Components|Blackboard|SetValueasBool (AI|GetBlackboard 0) (Utilities|Name|MakeLiteralName "IsSeeingPlayer?") false))))

(event OnPerceptionUpdated(AIPerception)
  (params (UpdatedActors :type Array%20of%20Actor%20Object%20References)))

(event EventBeginPlay
  (bind _returnvalue (Pawn|GetControlledPawn))
  (Utilities|FlowControl|Delay 0.2)
  (Utilities|IsValid _returnvalue
    (:Is%20Valid
      (bind _output_get (Variables|Default|SetControlledPawn (.AsBP%20Enemi%20Base (Utilities|Casting|CastToBP_EnemiBase _returnvalue))))
      (switch Utilities|FlowControl|Switch|SwitchonE_NPCBehavoir (Variables|/Game/Project/Blueprints/AI/Characters/BP_EnemiBase.BP_EnemiBase_C|GetBehavior _output_get)
        (:NewEnumerator3
          _)
        (:NewEnumerator1
          _))
      (AI|RunBehaviorTree "/Game/Project/Blueprints/AI/Behavior/BT_NPCPatrol.BT_NPCPatrol")
      (bind _blackboardcomponent (Class|AIController|UseBlackboard "/Game/Project/Blueprints/AI/Behavior/BB_EnemyPawn.BB_EnemyPawn"))
      (Class|BlackboardComponent|SetValueasInt _blackboardcomponent (Utilities|Name|MakeLiteralName "Direction") 1)
      (AI|Components|Blackboard|SetValueasBool _blackboardcomponent (Utilities|Name|MakeLiteralName "IsPathLooping?") (Variables|/Game/Project/Blueprints/AI/Behavior/BP_PatrolPath.BP_PatrolPath_C|GetIsLooping? (Variables|/Game/Project/Blueprints/AI/Characters/BP_EnemiBase.BP_EnemiBase_C|GetPatrolPath (Variables|Default|GetControlledPawn)))))
    (:Is%20Not%20Valid
      (Development|PrintString "Could not get controlled pawn"))))

(fn ConstructionScript)