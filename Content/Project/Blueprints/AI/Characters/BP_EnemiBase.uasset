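; Base enemy character providing spawn, damage, death and foot IK, with empty hooks for introduction, hit reaction, hitbox and kill.
; Spawning plays sound and reveals the mesh, after a delay unless already spawned; StartBehavior triggers the AI controller.
; Lethal damage notifies the game instance's wave count, flags the blackboard and destroys the actor when death FX finishes.
; Tick traces under both feet, interpolating foot offsets, slope rotations and hip offset.
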(event OnSystemFinished(SpawnFX)
  (params (PSystem :type Niagara%20Component%20Object%20Reference)))

(event OnSystemFinished(DeathFX)
  (params (PSystem :type Niagara%20Component%20Object%20Reference))
  (Actor|DestroyActor))

(event Custom|DrawHitBox
  (params (DammageValue :type Float%20%28single-precision%29) (AttackType :type E_AttackType%20Enum :default "NewEnumerator0")))

(event Custom|KillEnemy)

(event Custom|StartBehavior
  (bind _asbp_aicontroller (Utilities|Casting|CastToBP_AIController (AI|GetAIController self)))
  (Default|BehaviorStart _asbp_aicontroller (Variables|Default|GetIsStatic?)))

(event Custom|Introduce)

(event Custom|HandleHitReaction
  (params (AttackType :type E_AttackType%20Enum :default "NewEnumerator0") (Value :type Float%20%28single-precision%29)))

(event Custom|MakeDammages
  (params (Value :type Float%20%28single-precision%29))
  (bind _returnvalue (AI|GetBlackboard 0))
  (bind _output_get (Variables|Stats|SetLife (- (Variables|Stats|GetLife) Value)))
  (if (<= _output_get 0.0)
    (Default|CallEnemyWaveKilled (Variables|References|GetGameInstance))
    (CallFunction|KillEnemy)
    (Components|Activation|Activate (Variables|Default|GetDeathFX) false)
    (Rendering|SetVisibility (Variables|Character|GetMesh) false false)
    (Collision|SetCollisionEnabled (Variables|Collision|GetCapsuleComponent) "NoCollision")
    (bind _output_get_2 (Variables|states|SetIsBeeingDestroyed? true))
    (Utilities|IsValid _returnvalue
      (:Is%20Valid
        (AI|Components|Blackboard|SetValueasBool _returnvalue (Utilities|Name|MakeLiteralName "IsDestroyed?") _output_get_2)
        (Audio|PlaySoundatLocation "/Game/Project/Audio/SFX/Entity/Enemy/Death/SC_DeathEnemy.SC_DeathEnemy" (Transformation|GetWorldLocation (Variables|Character|GetMesh)) "0, 0, 0" 1.0 1.0 0.0 0 0 0)))))

(event EventBeginPlay
  (bind _spawnfx (Variables|Default|GetSpawnFX))
  (bind _spawnfx_2 (Variables|Default|GetSpawnFX))
  (bind _asbp_last_hope_game_instance (Utilities|Casting|CastToBP_LastHopeGameInstance (Game|GetGameInstance)))
  (Variables|References|SetGameInstance _asbp_last_hope_game_instance)
  (if (Variables|Default|GetAlreadySpawned?)
    (Audio|PlaySoundatLocation "/Game/Project/Audio/SFX/Entity/Enemy/Spawn/SC_SpawnEnemySand.SC_SpawnEnemySand" (Transformation|GetWorldLocation (Variables|Character|GetMesh)) "0, 0, 0" 1.0 1.0 0.0 0 0 0)
    (Variables|states|SetIsSpawned? true)
    (Rendering|SetVisibility (Variables|Character|GetMesh) true false)
    (Rendering|SetVisibility _spawnfx_2 false false)
    (Components|Activation|Deactivate _spawnfx_2)
    (CallFunction|Introduce)
    (else
      (Audio|PlaySoundatLocation "/Game/Project/Audio/SFX/Entity/Enemy/Spawn/SC_SpawnEnemySand.SC_SpawnEnemySand" (Transformation|GetWorldLocation (Variables|Character|GetMesh)) "0, 0, 0" 1.0 1.0 0.0 0 0 0)
      (Utilities|FlowControl|Delay 2.0)
      (Variables|states|SetIsSpawned? true)
      (Rendering|SetVisibility (Variables|Character|GetMesh) true false)
      (Rendering|SetVisibility _spawnfx false false)
      (Components|Activation|Deactivate _spawnfx)
      (CallFunction|Introduce))))

(event Collision|EventActorBeginOverlap
  (params (OtherActor :type Actor%20Object%20Reference)))

(event EventTick
  (params (DeltaSeconds :type Float%20%28single-precision%29))
  (bind (_out_hit_location _foottraceoffset _out_hit_impact_normal) (CallFunction|IKFootTrace "foot_lSocket" (Variables|/Script/Engine.CapsuleComponent|GetCapsuleHalfHeight (Variables|Collision|GetCapsuleComponent))))
  (Variables|Default|SetOut%20Hit%20Impact%20Normal%20Left _out_hit_impact_normal)
  (Variables|Default|SetIKLeftOffset (Math|Interpolation|FInterpTo (Variables|Default|GetIKLeftOffset) _foottraceoffset (Utilities|Time|GetWorldDeltaSeconds) 2e+01))
  (bind (_out_hit_location_2 _foottraceoffset_2 _out_hit_impact_normal_2) (CallFunction|IKFootTrace "foot_rSocket" (Variables|/Script/Engine.CapsuleComponent|GetCapsuleHalfHeight (Variables|Collision|GetCapsuleComponent))))
  (Variables|Default|SetOut%20Hit%20Impact%20Normal%20Right _out_hit_impact_normal_2)
  (Variables|Default|SetIKRightOffset (Math|Interpolation|FInterpTo (Variables|Default|GetIKRightOffset) _foottraceoffset_2 (Utilities|Time|GetWorldDeltaSeconds) 2e+01))
  (Variables|Default|SetIKHipOffset (Math|Interpolation|FInterpTo (Variables|Default|GetIKHipOffset) (Math|Float|SelectFloat (* (Math|Float|Absolute(Float) (.z (- _out_hit_location_2 _out_hit_location))) -0.5) 0.0 (< (Math|Float|Absolute(Float) (.z (- _out_hit_location_2 _out_hit_location))) 1e+02)) (Utilities|Time|GetWorldDeltaSeconds) 2e+01))
  (bind _rotationoffset (CallFunction|CalculateFootRotation (Variables|Default|GetLeftRotation) (Variables|Default|GetOut%20Hit%20Impact%20Normal%20Left)))
  (Variables|Default|SetLeftRotation _rotationoffset)
  (bind _rotationoffset_2 (CallFunction|CalculateFootRotation (Variables|Default|GetRightRotation) (Variables|Default|GetOut%20Hit%20Impact%20Normal%20Right)))
  (Variables|Default|SetRightRotation _rotationoffset_2))

(event EventTakeDamage
  (params (Value :type Float%20%28single-precision%29) (AttackType :type E_AttackType%20Enum :default "NewEnumerator0"))
  (CallFunction|HandleHitReaction AttackType Value))

(fn ConstructionScript)

(fn IKFootTrace
  (params (SocketName :type Name) (Distance :type Float%20%28single-precision%29))
  (bind _mesh (Variables|Character|GetMesh))
  (bind _returnvalue (Transformation|GetSocketLocation _mesh SocketName))
  (bind (_outhit _returnvalue_2) (Collision|LineTraceByChannel (Math|Vector|MakeVector (.x _returnvalue) (.y _returnvalue) (.z (Transformation|GetActorLocation))) (Math|Vector|MakeVector (.x _returnvalue) (.y _returnvalue) (- (.z _returnvalue) Distance)) "TraceTypeQuery1" false 0 "None"))
  (if _returnvalue_2
    (return (.location _outhit) (- (.z (- (.location _outhit) (Transformation|GetWorldLocation (Variables|Character|GetMesh)))) (Variables|Default|GetIKHipOffset)) (.impactnormal _outhit))
    (else
      (return "0, 0, 0" 0.0 "0, 0, 0"))))

(fn CalculateFootRotation
  (params (CurrentRotation :type Rotator) (FloorNormal :type Vector))
  (bind _self self)
  (bind _returnvalue (Transformation|GetActorUpVector _self))
  (return (Math|Interpolation|RInterpTo CurrentRotation (Math|Vector|RotatorfromAxisandAngle (Math|Vector|CrossProduct _returnvalue FloorNormal) (Class|KismetMathLibrary|DegAcos (Math|Vector|DotProduct _returnvalue FloorNormal))) (Utilities|Time|GetWorldDeltaSeconds) 2e+01)))