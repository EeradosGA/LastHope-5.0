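; Combat director that paces enemy attacks by choosing one enemy to attack on a looping timer.
; InitCombat gives each enemy in EnemyList a random starting rank, then starts the timer.
; Each tick of that timer scales ranks by how opposed enemy and player forward vectors are, orders the top enemy's BP_AIController to attack, then re-randomizes that rank.
; Debug rank widget code is disconnected.
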(event Custom|TriggerAttack
  (CallFunction|RecalculateRanks)
  (bind _gratestrankai1 (CallFunction|FindHighestRank))
  (bind _asbp_aicontroller (Utilities|Casting|CastToBP_AIController (AI|GetAIController _gratestrankai1)))
  (Default|AIAttack _asbp_aicontroller)
  (Utilities|Map|Add (Variables|Default|GetEnemyRanking) _gratestrankai1 (Math|Random|RandomFloatinRange 1.0 5.0)))

(event Custom|InitCombat
  (for _array_element (Variables|Default|GetEnemyList)
    (CallFunction|AddDebugWidgets _array_element))
  (Utilities|Time|SetTimerbyEvent (delegate Custom|TriggerAttack) 2.0 true))

(event EventBeginPlay)

(event Collision|EventActorBeginOverlap
  (params (OtherActor :type Actor%20Object%20Reference)))

(event EventTick
  (params (DeltaSeconds :type Float%20%28single-precision%29)))

(fn ConstructionScript)

(fn FindHighestRank
  (bind _keys (Utilities|Map|Keys (Variables|Default|GetEnemyRanking)))
  (for _array_element _keys
    (Utilities|IsValid _array_element
      (:Is%20Valid
        (if (> (.Value (Utilities|Map|Find (Variables|Default|GetEnemyRanking) _array_element)) (LocalVariables|GetHighestValue))
          (LocalVariables|SetHighestValue (.Value (Utilities|Map|Find (Variables|Default|GetEnemyRanking) _array_element)))
          (LocalVariables|SetGratestRankAI _array_element)))))
  (return (LocalVariables|GetHighestValue) (LocalVariables|GetGratestRankAI)))

(fn AddDebugWidgets
  (params (EnemyInstance :type BP%20Ennemi%20Weapon%20Object%20Reference%20%28by%20ref%29))
  (Utilities|Map|Add (Variables|Default|GetEnemyRanking) EnemyInstance (Math|Random|RandomFloatinRange 1.0 5.0)))

(fn UpdateWidgets
  (params (EnemyInstance :type BP%20Ennemi%20Weapon%20Object%20Reference))
  (Variables|/Game/Project/Blueprints/AI/Behavior/UW_DebugAI.UW_DebugAI_C|SetRank (.Value (Utilities|Map|Find (Variables|Default|GetEnemyWidgets) EnemyInstance)) (.Value (Utilities|Map|Find (Variables|Default|GetEnemyRanking) EnemyInstance))))

(fn RecalculateRanks
  (CallFunction|RankbyPosition))

(fn RankbyPosition
  (bind _enemyranking (Variables|Default|GetEnemyRanking))
  (for _array_element (Variables|Default|GetEnemyList)
    (Utilities|IsValid _array_element
      (:Is%20Valid
        (Utilities|Map|Add _enemyranking _array_element (* (.Value (Utilities|Map|Find _enemyranking _array_element)) (+ (Math|Float|NormalizetoRange (* (Math|Vector|DotProduct (Transformation|GetActorForwardVector _array_element) (Transformation|GetActorForwardVector (Game|GetPlayerCharacter 0))) -1.0) -1.0 1.0) 0.5)))))))