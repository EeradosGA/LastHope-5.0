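; Trigger actor that runs an enemy horde encounter when the player enters, with music and an optional sandstorm.
; It spawns a leader-led first wave at local points, then refills when few enemies remain, using tagged spawn points either farthest from the player or one per enemy.
; Kills update horde completion through the GameInstance.
; Completion spawns indexed cinematic enemies, which a GameInstance event later destroys by tag.
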(event Custom|SpawnFirstWave
  ;[1 1 1] First Wave
  (CallFunction|SpawnbyIndex 0 true)
  (Utilities|FlowControl|Delay 0.5)
  (CallFunction|SpawnbyIndex 1 false)
  (CallFunction|SpawnbyIndex 2 false)
  (CallFunction|ShowingLifeBar))

(event Custom|KilledEnemy
  (bind _result (Math|Float|IncrementFloat (Variables|Vars|GetKilledEnemies))
    (:%20%20
      (bind _output_get (Variables|States|SetIsFinished? (== (/ _result (Variables|Vars|GetTotalEnemies)) 1.0)))
      (Default|CallUpdateHordeCompletion (Variables|References|GetGameInstance) (/ _result (Variables|Vars|GetTotalEnemies)) _output_get)
      (if (not (Variables|States|GetIsFinished?))
        (bind _result_2 (Math|Integer|DecrementInt (Variables|States|GetSpawnedUnitsCount))
          (:%20%20
            (if (and (<= _result_2 2) (!= (Variables|-->Config|GetWavesLeft) 0))
              (if (not (Variables|Default|GetSecondSpawnMethod?))
                ;[1 1 1] Group method
                (for _array_element (Variables|References|GetSpawnPoints)
                  (Math|Float|CompareFloat (Math|Vector|Distance2D(Vector) (Transformation|GetActorLocation _array_element) (Transformation|GetActorLocation (Game|GetPlayerCharacter 0))) (Variables|Vars|GetFarestPointDistance)
                    (:>
                      _)
                    (:==
                      _))
                  (Variables|Vars|SetFarestPointDistance (Math|Vector|Distance2D(Vector) (Transformation|GetActorLocation _array_element) (Transformation|GetActorLocation (Game|GetPlayerCharacter 0))))
                  (Variables|Vars|SetFarestSpawnPoint _array_element))
                (Variables|Vars|SetFarestPointDistance 0.0)
                (for _index (range 1 (Variables|-->Config|GetPerWaveEnemis))
                  (bind _returnvalue (Actor|GetActorOfClass "/Game/Project/Blueprints/AI/Behavior/BP_PatrolPath.BP_PatrolPath_C"))
                  (Game|SpawnActorfromClass "/Game/Project/Blueprints/AI/Characters/BP_EnemiBase_Horde.BP_EnemiBase_Horde_C" (Math|Transform|MakeTransform (.RandomLocation (Class|NavigationSystemV1|GetRandomPointinNavigableRadius (Transformation|GetActorLocation (Variables|Vars|GetFarestSpawnPoint)) 3e+02 0 0)) (Math|Rotator|FindLookatRotation (.RandomLocation (Class|NavigationSystemV1|GetRandomPointinNavigableRadius (Transformation|GetActorLocation (Variables|Vars|GetFarestSpawnPoint)) 3e+02 0 0)) (Transformation|GetActorLocation (Game|GetPlayerCharacter 0))) "1,1,1") "AlwaysSpawn" 0 false "NewEnumerator5" _returnvalue 1e+02 false false 0)
                  (Math|Integer|IncrementInt (Variables|States|GetSpawnedUnitsCount)))
                (Math|Integer|DecrementInt (Variables|-->Config|GetWavesLeft))
                (else
                  ;[1 1 1] Different spawn points spawn
                  (for _index_2 (range 0 (- (Variables|-->Config|GetPerWaveEnemis) 1))
                    (bind _returnvalue_2 (Actor|GetActorOfClass "/Game/Project/Blueprints/AI/Behavior/BP_PatrolPath.BP_PatrolPath_C"))
                    (Game|SpawnActorfromClass "/Game/Project/Blueprints/AI/Characters/BP_EnemiBase_Horde.BP_EnemiBase_Horde_C" (Math|Transform|MakeTransform (.RandomLocation (Class|NavigationSystemV1|GetRandomPointinNavigableRadius (Transformation|GetActorLocation (Utilities|Array|Get(acopy) (Variables|References|GetSpawnPoints) _index_2)) 3e+02 0 0)) (Math|Rotator|FindLookatRotation (.RandomLocation (Class|NavigationSystemV1|GetRandomPointinNavigableRadius (Transformation|GetActorLocation (Utilities|Array|Get(acopy) (Variables|References|GetSpawnPoints) _index_2)) 3e+02 0 0)) (Transformation|GetActorLocation (Game|GetPlayerCharacter 0))) "1,1,1") "AlwaysSpawn" 0 false "NewEnumerator5" _returnvalue_2 1e+02 false false 0)
                    (Math|Integer|IncrementInt (Variables|States|GetSpawnedUnitsCount)))
                  (Math|Integer|DecrementInt (Variables|-->Config|GetWavesLeft)))))))))))

(event Custom|Example%20Update%20horde
  (params (Percentage%280%20to%201%29 :type Float%20%28single-precision%29) (IsFinished? :type Boolean))
  (CallFunction|DevPrintwithAppend "NewEnumerator1" 0 "Percentage : " (Utilities|String|ToString(Float) Percentage%280%20to%201%29) true true "(R=0.000000,G=0.658824,B=1.000000,A=1.000000)" 5.0)
  (if IsFinished?
    ;[1 1 1] Spawn cine enemy
    (for (_array_element _array_index) (Variables|Default|GetCinematicSpawner)
      (Game|SpawnActorfromClass "/Game/Project/Blueprints/AI/Characters/BP_EnemiCine.BP_EnemiCine_C" (Transformation|GetActorTransform _array_element) "Undefined" 0 _array_index "NewEnumerator3" 0 1e+02 false false 0))
    (bind _asbp_last_hope_game_instance (Utilities|Casting|CastToBP_LastHopeGameInstance (Game|GetGameInstance)))
    (EventDispatchers|BindEventtoDestroyCineEnemy _asbp_last_hope_game_instance (delegate Custom|DestroyCineEnemy))))

(event Custom|DestroyCineEnemy
  (params (Index :type Integer))
  (CallFunction|DestroyCEnemy Index))

(event EventBeginPlay
  (Utilities|FlowControl|Sequence
    (:then_0
      (Variables|Vars|SetTotalEnemies (Math|Conversions|ToFloat(Integer) (+ (Utilities|Array|Length (Variables|-->Config|GetFirstSpawnPoints)) (* (Variables|-->Config|GetWavesNumber) (Variables|-->Config|GetPerWaveEnemis)))))
      (Variables|-->Config|SetWavesLeft (Variables|-->Config|GetWavesNumber)))
    (:then_1
      (bind _outactors (Actor|GetAllActorsOfClasswithTag "/Game/Project/Blueprints/AI/BP_SpawnPoint.BP_SpawnPoint_C" (Variables|-->Config|GetSpawnerTag)))
      (Variables|References|SetSpawnPoints _outactors))
    (:then_2
      (bind _asbp_last_hope_game_instance (Utilities|Casting|CastToBP_LastHopeGameInstance (Game|GetGameInstance)))
      (bind _output_get (Variables|References|SetGameInstance _asbp_last_hope_game_instance))
      (EventDispatchers|BindEventtoUpdateHordeCompletion _output_get (delegate Custom|Example%20Update%20horde)))))

(event Collision|EventActorBeginOverlap
  (params (OtherActor :type Actor%20Object%20Reference))
  (bind _sandstormfx (Variables|Default|GetSandStormFx))
  (Utilities|FlowControl|Sequence
    (:then_0
      (if (and (== (Utilities|GetClass OtherActor) "/Game/Project/Blueprints/BP_PlayerCharacter.BP_PlayerCharacter_C") (not (Variables|States|GetHasTriggered?)))
        (Variables|States|SetHasTriggered? true)
        (bind _returnvalue (Actor|GetActorOfClass "/Game/Project/Audio/BP_MusicPlayer.BP_MusicPlayer_C"))
        (Default|PlayMusicFade _returnvalue "NewEnumerator3" 3.0 3.0 0.0)
        (CallFunction|SpawnFirstWave)
        (EventDispatchers|BindEventtoEnemyWaveKilled (Variables|References|GetGameInstance) (delegate Custom|KilledEnemy))))
    (:then_1
      (Utilities|IsValid _sandstormfx
        (:Is%20Valid
          (if (not (Variables|/Game/Project/Blueprints/FX/BP_SandStorm.BP_SandStorm_C|Getfinished? _sandstormfx))
            (Default|Start _sandstormfx)))))))

(event EventTick
  (params (DeltaSeconds :type Float%20%28single-precision%29)))

(fn ConstructionScript
  (for (_array_element _array_index) (Variables|Default|GetCinematicSpawner)
    (bind _output_get (Variables|/Game/Project/Blueprints/AI/BP_AICinematicSpawner.BP_AICinematicSpawner_C|SetIndex _array_element _array_index))
    (Rendering|Components|TextRender|SetText (Variables|/Game/Project/Blueprints/AI/BP_AICinematicSpawner.BP_AICinematicSpawner_C|GetTextRender _array_element) (Utilities|Text|ToText(Integer) _output_get))))

(fn SpawnbyIndex
  (params (Index :type Integer) (IsLeader? :type Boolean))
  (bind _returnvalue (Transformation|GetActorTransform))
  (bind _firstspawnpoints (Variables|-->Config|GetFirstSpawnPoints))
  (bind _output (Utilities|Array|Get(acopy) _firstspawnpoints Index))
  (bind _returnvalue_2 (Math|Transform|TransformLocation _returnvalue _output))
  (bind _returnvalue_3 (Game|SpawnActorfromClass "/Game/Project/Blueprints/AI/Characters/BP_EnemiBase_Horde.BP_EnemiBase_Horde_C" (Math|Transform|MakeTransform _returnvalue_2 (Math|Rotator|FindLookatRotation _returnvalue_2 (Transformation|GetActorLocation (Game|GetPlayerCharacter 0))) "1,1,1") "AlwaysSpawn" 0 IsLeader? "NewEnumerator5" 0 1e+02 false false 0))
  (Math|Integer|IncrementInt (Variables|States|GetSpawnedUnitsCount)))

(fn RemoveLifeBar
  (Utilities|Time|SetTimerbyFunctionName (CallFunction|GetHudPlayer) "HideLifeBar" 3.0))

(fn DestroyCEnemy
  (params (Index :type Integer))
  (bind _returnvalue (Utilities|String|ToString(Integer) Index))
  (bind _outactors (Actor|GetAllActorsOfClasswithTag "/Game/Project/Blueprints/AI/Characters/BP_EnemiCine.BP_EnemiCine_C" (Utilities|String|StringToName (Utilities|String|Append "E" (Utilities|String|ToString(Integer) Index)))))
  (Utilities|IsValid (Utilities|Array|Get(acopy) _outactors)
    (:Is%20Valid
      (Default|StartDestroy (Utilities|Array|Get(acopy) _outactors))
      (CallFunction|DevPrintwithAppend "NewEnumerator1" 0 "Start destroy actor with index  : " _returnvalue true true "(R=0.000000,G=0.658824,B=1.000000,A=1.000000)" 2.0))
    (:Is%20Not%20Valid
      (CallFunction|DevPrintwithAppend "NewEnumerator1" 0 "Error destroy actor with index  : " _returnvalue true true "(R=0.000000,G=0.658824,B=1.000000,A=1.000000)" 2.0))))