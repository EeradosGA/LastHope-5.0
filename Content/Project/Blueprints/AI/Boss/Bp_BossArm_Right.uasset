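; Right arm of the boss, a child Blueprint that overrides the parent arm's attack patterns, laser and enemy summoning.
; StartPattern picks the attack state, activating the summon trail for pattern 0, and SpawnEnemies creates two static horde leaders.
; Laser either spawns a beam effect aimed at the player or rotates toward them.
; Tick blocks laser launch during Wander and Cooldown, stops the trail on Death, and fades then destroys flagged lasers.
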(event EventBeginPlay
  (|CallParentFunction)
  (Rendering|Material|SetVectorParameterValueonMaterials (Variables|Character|GetMesh) "Color" (Variables|Default|GetArmColor)))

(event Collision|EventActorBeginOverlap
  (params (OtherActor :type Actor%20Object%20Reference)))

(event EventTick
  (params (DeltaSeconds :type Float%20%28single-precision%29))
  (bind _laserref (Variables|Default|GetLaserRef))
  (|CallParentFunction 0.0)
  (Utilities|FlowControl|Sequence
    (:then_0
      (switch Utilities|FlowControl|Switch|SwitchonEnum_BossState (Variables|Default|GetCurrentState)
        (:NewEnumerator0
          (Variables|Default|SetCanLaunchLaserEffect false :!label _label))
        (:NewEnumerator2
          (goto _label))
        (:NewEnumerator3
          (Components|Activation|Deactivate (Variables|Default|GetFX_BossSummonTrail)))))
    (:then_1
      (if (Variables|Default|GetcanDestroyLaser)
        (Utilities|FlowControl|DoOnce true :!label _label_2
          (:Completed
            (Audio|Components|Audio|FadeOut (Variables|/Game/Project/Blueprints/FX/BP_BeetleLaser_FX.BP_BeetleLaser_FX_C|GetAudio _laserref) 2.0 0.0 "Linear" :!class /Script/Engine.AudioComponent)
            (Components|Activation|Deactivate (Variables|/Game/Project/Blueprints/FX/BP_BeetleLaser_FX.BP_BeetleLaser_FX_C|GetFX_BeetleLaser _laserref))
            (Utilities|FlowControl|Delay 5.0)
            (Actor|DestroyActor _laserref)
            (Variables|Default|SetcanDestroyLaser false)))
        (else
          (goto _label_2 Reset))))))

(fn ConstructionScript
  (|CallParentFunction))

(fn StartPattern
  (params (Pattern%20Number%20 :type Integer))
  (|CallParentFunction Pattern%20Number%20)
  (switch int Pattern%20Number%20
    (:0
      (Variables|Default|SetCurrentStateAttack "NewEnumerator2")
      (CallFunction|DevPrintwithAppend "NewEnumerator4" 0 "Override Pattern number 0 of --> " (Utilities|GetDisplayName self) true true "(R=0.000000,G=0.658824,B=1.000000,A=1.000000)" 2.0)
      (Components|Activation|Activate (Variables|Default|GetFX_BossSummonTrail) false))
    (:1
      (Variables|Default|SetCurrentStateAttack "NewEnumerator0")
      (CallFunction|DevPrintwithAppend "NewEnumerator4" 0 "Pattern number 1 of --> " (Utilities|GetDisplayName self) true true "(R=0.000000,G=0.658824,B=1.000000,A=1.000000)" 2.0))))

(fn Laser
  (Utilities|FlowControl|Sequence
    (:then_0
      (if (Variables|Default|GetCanLaunchLaserEffect)
        (CallFunction|LaunchLaserEffect)
        (elif (Variables|Default|GetUpdateLaserRotation)
          (CallFunction|RotateTowardPlayer (Transformation|GetActorLocation (Game|GetPlayerCharacter 0))))))))

(fn Invocation)

(fn SpawnEnemies
  (bind _spawnlocation1 (Variables|Default|GetSpawnLocation1))
  (bind _spawnlocation2 (Variables|Default|GetSpawnLocation2))
  (bind _returnvalue (Transformation|GetWorldTransform _spawnlocation1))
  (bind _returnvalue_2 (Transformation|GetWorldTransform _spawnlocation2))
  (Game|SpawnActorfromClass "/Game/Project/Blueprints/AI/Characters/BP_EnemiBase_Horde.BP_EnemiBase_Horde_C" (Math|Transform|MakeTransform (.location _returnvalue) (.rotation _returnvalue) "1,1,1") "AdjustIfPossibleButAlwaysSpawn" 0 true "NewEnumerator5" 0 75.0 true false 0)
  (Game|SpawnActorfromClass "/Game/Project/Blueprints/AI/Characters/BP_EnemiBase_Horde.BP_EnemiBase_Horde_C" (Math|Transform|MakeTransform (.location _returnvalue_2) (.rotation _returnvalue_2) "1,1,1") "AdjustIfPossibleButAlwaysSpawn" 0 true "NewEnumerator5" 0 75.0 true false 0))

(fn LaunchLaserEffect
  (bind _returnvalue (Game|GetPlayerController 0))
  (bind _spawnlocation (Variables|Default|GetSpawnLocation))
  (bind _returnvalue_2 (Pawn|GetControlledPawn _returnvalue))
  (bind _returnvalue_3 (Transformation|GetWorldLocation _spawnlocation))
  (bind _returnvalue_4 (Transformation|GetActorLocation _returnvalue_2))
  (bind _returnvalue_5 (Game|SpawnActorfromClass "/Game/Project/Blueprints/FX/BP_BeetleLaser_FX.BP_BeetleLaser_FX_C" (Math|Transform|MakeTransform _returnvalue_3 (Math|Rotator|MakeRotfromX (Math|Vector|Normalize (- _returnvalue_4 _returnvalue_3))) "1,1,1") "AlwaysSpawn" 0 0))
  (Transformation|SetWorldRotation (Variables|/Game/Project/Blueprints/FX/BP_BeetleLaser_FX.BP_BeetleLaser_FX_C|GetDefaultSceneRoot _returnvalue_5) (Math|Rotator|FindLookatRotation _returnvalue_3 _returnvalue_4) false false)
  (Variables|Default|SetLaserRef _returnvalue_5)
  (Variables|Default|SetCanLaunchLaserEffect false)
  (Variables|Default|SetUpdateLaserRotation false))

(fn ActiveEndAnimation)

(fn DestroyLaser
  (Variables|Default|SetcanDestroyLaser true))