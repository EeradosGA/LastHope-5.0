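; Boss actor that spawns left and right arm actors and runs the boss fight until both arms are dead.
; Once started, a timeline alternates attacks between arms, cycling two patterns each, falling back to the survivor and switching to a one-arm timer.
; Meanwhile it turns toward the player and cycles through destinations by shrinking, teleporting and growing back.
; When both arms die, it plays a camera sequence after a delay.
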(event EventBeginPlay
  ;[1 1 1] Spawn des Bras
  (bind _returnvalue (Game|SpawnActorfromClass (Variables|Right|GetRight_Arm) (Math|Transform|MakeTransform (.location (Transformation|GetWorldTransform (Variables|Right|GetSpawnRightArm))) "0, 0, 0" "-0.500000,0.500000,0.500000") "Undefined" 0 2e+02 0))
  (bind _output_get (Variables|Right|SetRightArmRef _returnvalue))
  (Variables|/Game/Project/Blueprints/AI/Boss/Bp_BossArm_Template.Bp_BossArm_Template_C|SetRefBoss _output_get self)
  (Variables|/Game/Project/Blueprints/AI/Boss/Bp_BossArm_Template.Bp_BossArm_Template_C|SetRefArmOrigin _output_get (Variables|Right|GetSpawnRightArm))
  (bind _returnvalue_2 (Game|SpawnActorfromClass (Variables|Left|GetLeft_Arm) (Math|Transform|MakeTransform (.location (Transformation|GetWorldTransform (Variables|Left|GetSpawnLeftArm))) "0,180.000000, 0" "0.500000,0.500000,0.500000") "Undefined" 0 2e+02 0))
  (bind _output_get_2 (Variables|Left|SetLeft%20Arm%20Ref _returnvalue_2))
  (Variables|/Game/Project/Blueprints/AI/Boss/Bp_BossArm_Template.Bp_BossArm_Template_C|SetRefBoss _output_get_2 self)
  (Variables|/Game/Project/Blueprints/AI/Boss/Bp_BossArm_Template.Bp_BossArm_Template_C|SetRefArmOrigin _output_get_2 (Variables|Left|GetSpawnLeftArm))
  (Components|Timeline|SetTimelineLength (Variables|Default|GetTimelineBeetwenPattern) (Variables|Default|GetTimerBetweenPattern))
  (Variables|Default|SetCanStartUpdateStats true)
  (Variables|Default|SetMaxID (Utilities|Array|Length (Variables|Default|GetTabDestination))))

(event Collision|EventActorBeginOverlap
  (params (OtherActor :type Actor%20Object%20Reference)))

(event EventTick
  (params (DeltaSeconds :type Float%20%28single-precision%29))
  (bind _returnvalue (Transformation|GetActorLocation))
  (bind _returnvalue_2 (Game|GetPlayerCharacter 0))
  (bind _returnvalue_3 (Transformation|GetActorLocation _returnvalue_2))
  (bind _returnvalue_4 (Math|Rotator|FindLookatRotation _returnvalue _returnvalue_3))
  (if (Variables|Default|GetCanStartUpdateStats)
    (if (CallFunction|CheckifArmsAreAlive) ; CheckIfArmAreStillAlive
      (Utilities|FlowControl|Sequence
        (:then_0
          ;[1 1 1] Gestion des pattern des bras du boss
          (if (Variables|Default|GetCanStartPattern)
            (Utilities|FlowControl|Sequence
              (:then_0
                (Utilities|FlowControl|DoOnce false :!label _label
                  (:Completed
                    (Timeline|TimelineBeetwenPattern PlayFromStart
                      (:Update
                        (CallFunction|DevPrint "NewEnumerator4" 0 "Waiting For New Pattern" true true "(R=1.000000,G=0.761645,B=0.000000,A=1.000000)" 0.0))
                      (:Finished
                        (CallFunction|DevPrint "NewEnumerator4" 0 "LaunchPattern" true true "(R=1.000000,G=0.761645,B=0.000000,A=1.000000)" 2.0)
                        (if (Variables|Default|GetLeft)
                          (bind _left_arm_ref (Variables|Left|GetLeft%20Arm%20Ref :!label _label_2)
                            (:then
                              (Default|StartPattern _left_arm_ref (Variables|Left|GetCurrentLeftPattern))
                              (if (< (Variables|Left|GetCurrentLeftPattern) 1)
                                (Math|Integer|IncrementInt (Variables|Left|GetCurrentLeftPattern)
                                  (:%20%20
                                    _))
                                (else
                                  (Variables|Left|SetCurrentLeftPattern 0)))
                              (Variables|Default|SetLeft false)
                              (goto _label Reset))
                            (:else
                              (if (CallFunction|CheckifArmsAreAlive) ; CheckIfArmAreStillAlive
                                (bind _rightarmref (Variables|Right|GetRightArmRef :!label _label_3)
                                  (:then
                                    (Default|StartPattern _rightarmref (Variables|Right|GetCurrentRightPattern))
                                    (if (< (Variables|Right|GetCurrentRightPattern) 1)
                                      (Math|Integer|IncrementInt (Variables|Right|GetCurrentRightPattern)
                                        (:%20%20
                                          _))
                                      (else
                                        (Variables|Right|SetCurrentRightPattern 0)))
                                    (Variables|Default|SetLeft true)
                                    (goto _label Reset))
                                  (:else
                                    (if (CallFunction|CheckifArmsAreAlive) ; CheckIfArmAreStillAlive
                                      (goto _label_2)))))))
                          (else
                            (goto _label_3))))))))
              (:then_1
                (Utilities|FlowControl|DoOnce false :!label _label_4
                  (:Completed
                    (bind _alpha (Timeline|LerpScale PlayFromStart)
                      (:Update
                        (Transformation|SetActorScale3D self (Math|Vector|Lerp(Vector) "1.000000,1.000000,1.000000" "0, 0, 0" _alpha)))
                      (:Finished
                        (Transformation|SetActorLocation (Transformation|GetActorLocation (Utilities|Array|Get(acopy) (Variables|Default|GetTabDestination) (Variables|Default|GetcurrentID))) true true)
                        (if (< (Variables|Default|GetcurrentID) (- (Variables|Default|GetMaxID) 1))
                          (Variables|Default|SetcurrentID (+ (Variables|Default|GetcurrentID) 1))
                          (bind _alpha_2 (Timeline|Lerp2 PlayFromStart)
                            (:Update
                              (Transformation|SetActorScale3D self (Math|Vector|Lerp(Vector) "0, 0, 0" "1.000000,1.000000,1.000000" _alpha_2)))
                            (:Finished
                              (Utilities|FlowControl|Delay 1e+01)
                              (goto _label_4 Reset)))
                          (else
                            (Variables|Default|SetcurrentID 0)
                            (Timeline|Lerp2 PlayFromStart))))))))
              (:then_2
                (Utilities|IsValid _returnvalue_2
                  (:Is%20Valid
                    (Transformation|SetActorRotation (Math|Rotator|MakeRotator (.roll _returnvalue_4) 0.0 (.yaw _returnvalue_4))))))))))
      (else
        (Utilities|FlowControl|DoOnce false
          (:Completed
            ;[1 1 1] ETAT DE MORT
            (CallFunction|DevPrint "NewEnumerator4" 0 "All My arm are dead" true true "(R=1.000000,G=0.099778,B=0.000000,A=1.000000)" 2.0)
            (Utilities|FlowControl|Delay 5.0)
            (CallFunction|CameraPlaySequence "NewEnumerator8")))))))

(fn ConstructionScript)

(fn CheckifLeftArmIsAlive
  (bind _left_arm_ref (Variables|Left|GetLeft%20Arm%20Ref)
    (:then
      (if (Utilities|Enum|NotEqual(Enum) (Variables|/Game/Project/Blueprints/AI/Boss/Bp_BossArm_Template.Bp_BossArm_Template_C|GetCurrentState _left_arm_ref) "NewEnumerator3")
        (return true)
        (else
          _)))
    (:else
      _))
  (CallFunction|ChangeTimertoOneArm)
  (return false))

(fn CheckifRightArmIsAlive
  (bind _rightarmref (Variables|Right|GetRightArmRef)
    (:then
      (if (Utilities|Enum|NotEqual(Enum) (Variables|/Game/Project/Blueprints/AI/Boss/Bp_BossArm_Template.Bp_BossArm_Template_C|GetCurrentState _rightarmref) "NewEnumerator3")
        (return true)
        (else
          _)))
    (:else
      _))
  (CallFunction|ChangeTimertoOneArm)
  (return false))

(fn CheckifArmsAreAlive
  (return (or (CallFunction|CheckifLeftArmIsAlive) (CallFunction|CheckifRightArmIsAlive))))

(fn ChangeTimertoOneArm
  (Components|Timeline|SetTimelineLength (Variables|Default|GetTimelineBeetwenPattern) (Variables|Default|GetTimerBetweenPatternWhenOneArm)))

(fn StartPattern
  (Variables|Default|SetCanStartPattern true))