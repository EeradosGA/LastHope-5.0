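; Left arm actor of the boss, overriding parent attack patterns for a rocket punch (Fulguro Point) and a ground slam.
; Nested state enums drive both attacks, with Tick resetting them outside Attack.
; The punch thrusts horizontally, damaging the player until hitting a "Wall" actor, then a timeline returns it to the boss's spawn point.
; The slam hovers over the buffered player position, drops via line trace and spawns an impact zone.
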(event OnComponentBeginOverlap(DetectionCollision)
  (params (OverlappedComponent :type Primitive%20Component%20Object%20Reference) (OtherActor :type Actor%20Object%20Reference) (OtherComp :type Primitive%20Component%20Object%20Reference) (OtherBodyIndex :type Integer) (bFromSweep :type Boolean) (SweepResult :type Hit%20Result%20Structure%20%28by%20ref%29))
  (switch Utilities|FlowControl|Switch|SwitchonEnum_BossAttack (Variables|Default|GetCurrentStateAttack)
    (:NewEnumerator1
      (bind _asbp_player_character (Utilities|Casting|CastToBP_PlayerCharacter OtherActor))
      (Default|TakeDamage _asbp_player_character (Variables|Default|GetDamageFulguro) "NewEnumerator0"))))

(event OnComponentBeginOverlap(BoxLockWall)
  (params (OverlappedComponent :type Primitive%20Component%20Object%20Reference) (OtherActor :type Actor%20Object%20Reference) (OtherComp :type Primitive%20Component%20Object%20Reference) (OtherBodyIndex :type Integer) (bFromSweep :type Boolean) (SweepResult :type Hit%20Result%20Structure%20%28by%20ref%29))
  (if (Actor|ActorHasTag OtherActor "Wall")
    (Variables|Default|SetFulguroState "NewEnumerator2")
    (Components|Activation|Activate (Variables|Default|GetNiagara) false)))

(event Custom|CustomEvent_0
  (Actor|DestroyActor))

(event EventBeginPlay
  (|CallParentFunction)
  (Rendering|Material|SetVectorParameterValueonMaterials (Variables|Character|GetMesh) "Color" (Variables|Default|GetArmColor)))

(event Collision|EventActorBeginOverlap
  (params (OtherActor :type Actor%20Object%20Reference)))

(event EventTick
  (params (DeltaSeconds :type Float%20%28single-precision%29))
  (|CallParentFunction 0.0)
  (switch Utilities|FlowControl|Switch|SwitchonEnum_BossState (Variables|Default|GetCurrentState)
    (:NewEnumerator0
      (Variables|Default|SetFulguroState "NewEnumerator0" :!label _label)
      (Variables|Default|SetImpactState "NewEnumerator0")
      (Variables|Default|SetOnceStartImpact false))
    (:NewEnumerator1
      (switch Utilities|FlowControl|Switch|SwitchonEnum_BossAttack (Variables|Default|GetCurrentStateAttack)
        (:NewEnumerator1
          (switch Utilities|FlowControl|Switch|SwitchonEnum_FulguPointState (Variables|Default|GetFulguroState)
            (:NewEnumerator1
              (goto _label_2 Reset))
            (:NewEnumerator3
              (Utilities|FlowControl|DoOnce false :!label _label_2
                (:Completed
                  (bind _alpha (Timeline|TimelineReturn PlayFromStart)
                    (:Update
                      (Transformation|SetActorLocation (Math|Vector|Lerp(Vector) (Transformation|GetActorLocation) (Transformation|GetWorldLocation (Variables|/Game/Project/Blueprints/AI/Boss/Bp_Boss.Bp_Boss_C|GetSpawnLeftArm (Variables|Default|GetRefBoss))) _alpha) false false))
                    (:Finished
                      (Variables|Default|SetEndLooping false)
                      (Variables|Default|SetCurrentState "NewEnumerator2"))))))))))
    (:NewEnumerator2
      (goto _label))
    (:NewEnumerator3
      (goto _label))))

(fn ConstructionScript
  (|CallParentFunction))

(fn StartPattern
  (params (Pattern%20Number%20 :type Integer))
  (|CallParentFunction Pattern%20Number%20)
  (switch int Pattern%20Number%20
    (:0
      (Variables|Default|SetCurrentStateAttack "NewEnumerator1")
      (CallFunction|DevPrintwithAppend "NewEnumerator4" 0 "Override Pattern number 0 of --> " (Utilities|GetDisplayName self) true true "(R=0.000000,G=0.658824,B=1.000000,A=1.000000)" 2.0))
    (:1
      (Variables|Default|SetCurrentStateAttack "NewEnumerator3")
      (CallFunction|DevPrintwithAppend "NewEnumerator4" 0 "Pattern number 1 of --> " (Utilities|GetDisplayName self) true true "(R=0.000000,G=0.658824,B=1.000000,A=1.000000)" 2.0))))

(fn ImpactGround
  (bind _returnvalue (Transformation|GetActorLocation))
  (Utilities|FlowControl|Sequence
    (:then_0
      (switch Utilities|FlowControl|Switch|SwitchonEnum_BossState (Variables|Default|GetCurrentState)
        (:NewEnumerator1
          (switch Utilities|FlowControl|Switch|SwitchonEnum_ImpactState (Variables|Default|GetImpactState)
            (:NewEnumerator0
              (Utilities|FlowControl|Sequence
                (:then_0
                  (if (not (Variables|Default|GetOnceStartImpact))
                    (Variables|Default|SetOnceStartImpact true)
                    (Variables|Default|SetImpactStartReturnPosition (Transformation|GetActorLocation))
                    (Variables|Default|SetOnceImpactSound false)
                    (Audio|PlaySoundatLocation "/Game/Project/Audio/SFX/Entity/Enemy/Boss/LeftArm/AbovePlayer/SC_Boss_AbovePlayer.SC_Boss_AbovePlayer" (Transformation|GetWorldLocation (Variables|Default|GetSocket_Whrist)) "0, 0, 0" 1.0 1.0 0.0 0 0 0)))
                (:then_1
                  (Transformation|SetActorLocation (Math|Interpolation|VInterpTo (Transformation|GetActorLocation) (+ (Variables|Default|GetPlayerPositionBuffer) (Variables|Default|GetOffsetImpactPosition)) (Utilities|Time|GetWorldDeltaSeconds) 6.0) false false))))
            (:NewEnumerator2
              (bind _outhit (Collision|LineTraceByChannel _returnvalue (+ _returnvalue (* (Transformation|GetActorUpVector (Game|GetPlayerCharacter 0)) -5e+02)) "TraceTypeQuery1" false 0 "ForDuration"))
              (Transformation|SetActorLocation (Math|Interpolation|VInterpTo (Transformation|GetActorLocation) (- (.location _outhit) "0, 0, 0") (Utilities|Time|GetWorldDeltaSeconds) 12.0) false false)
              (Variables|Default|SetOnceStartImpact false)
              (if (Math|Float|NearlyEqual(Float) (Math|Vector|VectorLength (- (.location _outhit) (Transformation|GetActorLocation))) 0.0 4.0)
                (if (not (Variables|Default|GetOnceImpactSound))
                  (Audio|PlaySoundatLocation "/Game/Project/Audio/SFX/Entity/Enemy/Boss/LeftArm/ImpactGround/SC_ImpactGround.SC_ImpactGround" (Transformation|GetWorldLocation (Variables|Default|GetSocket_Whrist)) "0, 0, 0" 1.0 1.0 0.0 0 0 0)
                  (Variables|Default|SetOnceImpactSound true)
                  (Game|SpawnActorfromClass "/Game/Project/Blueprints/AI/Boss/BP_ImpactZoneBoss.BP_ImpactZoneBoss_C" (Transformation|GetWorldTransform (Variables|Default|GetSocket_Whrist)) "Undefined" 0 0))))
            (:NewEnumerator3
              (CallFunction|ReturntoPositionImpact))))))))

(fn FulguroPoint
  (Utilities|FlowControl|Sequence
    (:then_0
      (switch Utilities|FlowControl|Switch|SwitchonEnum_FulguPointState (Variables|Default|GetFulguroState)
        (:NewEnumerator0
          (if (Variables|Default|GetOnceStartFulguPoint)
            (CallFunction|RotateTowardPlayer (Variables|Default|GetPlayerPositionBuffer))
            (Variables|Default|SetFulguStartPosition (Transformation|GetActorLocation))
            (Variables|Default|SetOnceStartFulguPoint false)))
        (:NewEnumerator1
          (CallFunction|FulguMovement)
          (CallFunction|ActiveDamage true)
          (Variables|Default|SetOnceStartFulguPoint true)
          (Components|Activation|SetActive (Variables|Default|GetFX_BossArmTrail) true false)
          (Variables|Default|SetOnceFulguSound false))
        (:NewEnumerator2
          (CallFunction|ActiveDamage false)
          (Components|Activation|SetActive (Variables|Default|GetFX_BossArmTrail) false false)
          (if (not (Variables|Default|GetOnceFulguSound))
            (Audio|PlaySoundatLocation "/Game/Project/Audio/SFX/Entity/Enemy/Boss/LeftArm/ImpactWall/SC_Boss_ImpactWall.SC_Boss_ImpactWall" (Transformation|GetActorLocation) "0, 0, 0" 1.0 1.0 0.0 "/Game/Project/Audio/SoundAttenuation/SA_Enemy.SA_Enemy" 0 0)
            (Variables|Default|SetOnceFulguSound true)))
        (:NewEnumerator3
          (CallFunction|ActiveDamage false))))))

(fn FulguMovement
  (bind _returnvalue (Transformation|GetActorLocation))
  (bind _speed (Variables|Default|GetSpeed))
  (bind _armdirection (Variables|Default|GetArmDirection))
  (bind _returnvalue_2 (* _armdirection _speed))
  (bind _returnvalue_3 (+ _returnvalue_2 _returnvalue))
  (Transformation|SetActorLocation (Math|Vector|MakeVector (.x _returnvalue_3) (.y _returnvalue_3) (.Z (Math|Vector|BreakVector (Transformation|GetActorLocation)))) false false))

(fn DetectFulguWall)

(fn ActiveDamage
  (params (NewParam :type Boolean))
  (if NewParam
    (Collision|SetCollisionResponsetoAllChannels (Variables|Default|GetDetectionCollision) "ECR_Overlap")
    (else
      (Collision|SetCollisionResponsetoAllChannels (Variables|Default|GetDetectionCollision) "ECR_Ignore"))))

(fn ReturntoPositionImpact
  (Transformation|SetActorLocation (Math|Vector|Lerp(Vector) (Transformation|GetActorLocation) (Transformation|GetWorldLocation (Variables|/Game/Project/Blueprints/AI/Boss/Bp_Boss.Bp_Boss_C|GetSpawnLeftArm (Variables|Default|GetRefBoss))) (Utilities|Time|GetWorldDeltaSeconds)) false false))

(fn ActiveEndAnimation
  (switch Utilities|FlowControl|Switch|SwitchonEnum_BossAttack (Variables|Default|GetCurrentStateAttack)
    (:NewEnumerator1
      (Variables|Default|SetFulguroState "NewEnumerator3")
      (Variables|Default|SetFulguStartReturnPosition (Transformation|GetActorLocation)))))