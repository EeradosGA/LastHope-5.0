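; BP_ImpactZoneBoss is a short-lived boss attack impact zone that damages the player on overlap.
; When ImpactOverlap touches a BP_PlayerCharacter, it calls TakeDamage with DamageImpact, and the DoOnceDamage flag limits this to a single hit.
; Delays driven from Tick, rather than BeginPlay, set that flag after about a second to close the damage window, then destroy the actor about ten seconds later.
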(event OnComponentBeginOverlap(ImpactOverlap)
  (params (OverlappedComponent :type Primitive%20Component%20Object%20Reference) (OtherActor :type Actor%20Object%20Reference) (OtherComp :type Primitive%20Component%20Object%20Reference) (OtherBodyIndex :type Integer) (bFromSweep :type Boolean) (SweepResult :type Hit%20Result%20Structure%20%28by%20ref%29))
  (if (not (Variables|Default|GetDoOnceDamage))
    (bind _asbp_player_character (Utilities|Casting|CastToBP_PlayerCharacter OtherActor))
    (Default|TakeDamage _asbp_player_character (Variables|Default|GetDamageImpact) "NewEnumerator0")
    (Variables|Default|SetDoOnceDamage true)))

(event EventBeginPlay)

(event Collision|EventActorBeginOverlap
  (params (OtherActor :type Actor%20Object%20Reference)))

(event EventTick
  (params (DeltaSeconds :type Float%20%28single-precision%29))
  (Utilities|FlowControl|Delay 1.0)
  (Variables|Default|SetDoOnceDamage true)
  (Utilities|FlowControl|Delay 1e+01)
  (Actor|DestroyActor))

(fn ConstructionScript)