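; Template actor for a boss arm that runs BT_BossArm, with empty attack and end-animation functions, presumably for child arms to override.
; Tick drives a state machine: Wander returns to its origin facing the player, Attack times its loop, Cooldown waits out overheat before wandering again.
; LaunchPatternAttack buffers the player's position and dispatches the current attack.
; Damage raises a material frequency; zero HP stops effects and makes the chain disappear.
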(event EventBeginPlay
  (bind _maxemmissivstrenght (Variables|Emmissiv|GetMaxEmmissivStrenght))
  (Variables|HpValue|SetCurrentHp (Variables|HpValue|GetMaxHp))
  (Components|Timeline|SetTimelineLength (Variables|Default|GetResetOverHeat) (Variables|Default|GetTimerOverHeat))
  (AI|RunBehaviorTree (AI|GetAIController self) "/Game/Project/Blueprints/AI/Boss/BT_BossArm.BT_BossArm")
  (Variables|Default|SetInitialRotation (Transformation|GetActorLocation))
  ;[1 1 1] Set emmissiv strenght at start
  (Rendering|Material|SetScalarParameterValueonMaterials (Variables|Default|GetMesh) "EmmissivStrenght" _maxemmissivstrenght)
  (Variables|Emmissiv|SetCurrentEmmissivStrenght _maxemmissivstrenght))

(event Collision|EventActorBeginOverlap
  (params (OtherActor :type Actor%20Object%20Reference)))

(event EventTick
  (params (DeltaSeconds :type Float%20%28single-precision%29))
  (bind _returnvalue (Game|GetPlayerCharacter 0))
  (bind _returnvalue_2 (Transformation|GetActorLocation))
  (bind _returnvalue_3 (Utilities|Time|GetWorldDeltaSeconds))
  (bind _refarmorigin (Variables|Default|GetRefArmOrigin))
  (bind _returnvalue_4 (Transformation|GetWorldLocation _refarmorigin))
  (bind _returnvalue_5 (* 1e+03 _returnvalue_3))
  (Variables|Default|SetDeltaTime DeltaSeconds)
  (Utilities|IsValid _returnvalue
    (:Is%20Valid
      (Variables|Player|SetPlayerPosition (Transformation|GetWorldLocation (Variables|/Script/Engine.Character|GetMesh _returnvalue))))
    (:Is%20Not%20Valid
      (Variables|Player|SetPlayerPosition "-6620.000000,20910.000000,-1420.000000")))
  (Utilities|FlowControl|Sequence
    (:then_0
      (if (<= (Variables|HpValue|GetCurrentHp) 0.0)
        ;[1 1 1] Destroy the arm 'cause 0hp
        (Variables|Default|SetCurrentState "NewEnumerator3")
        (Components|Activation|Deactivate (Variables|Default|GetFX_ArmJoint))
        (Utilities|FlowControl|DoOnce false
          (:Completed
            (Default|Disappear (.AsBP%20Chain (Utilities|Casting|CastToBP_Chain (Variables|/Script/Engine.ChildActorComponent|GetChildActor (Variables|Default|GetBP_Chain)))))))))
    (:then_1
      (switch Utilities|FlowControl|Switch|SwitchonEnum_BossState (Variables|Default|GetCurrentState)
        (:NewEnumerator0
          (CallFunction|ResetValuesAttack)
          (CallFunction|RotateTowardPlayer (Variables|Player|GetPlayerPosition))
          (if (<= (Math|Vector|Distance(Vector) _returnvalue_4 _returnvalue_2) _returnvalue_5)
            (Transformation|SetActorLocation _returnvalue_4 false false))
          (Transformation|AddActorWorldOffset (* (Math|Vector|Normalize (- _returnvalue_4 _returnvalue_2)) _returnvalue_5)))
        (:NewEnumerator1
          (if (Variables|Default|GetStartLooping)
            (Utilities|FlowControl|DoOnce false :!label _label
              (:Completed
                (if (Utilities|Enum|Equal(Enum) (Variables|Default|GetCurrentStateAttack) "NewEnumerator2")
                  (Variables|Default|SetStartLooping false :!label _label_2)
                  (Variables|Default|SetEndLooping true)
                  (Variables|Default|SetEndCooldown false)
                  (CallFunction|ActiveEndAnimation)
                  (else
                    (Timeline|TimerLooping PlayFromStart
                      (:Update
                        (CallFunction|DevPrintwithAppend "NewEnumerator4" 0 "Looping arm : " (Utilities|GetDisplayName self) true true "(R=0.000000,G=0.658824,B=1.000000,A=1.000000)" 0.0))
                      (:Finished
                        (goto _label_2)))))))))
        (:NewEnumerator2
          (CallFunction|ResetValuesAttack)
          (Utilities|FlowControl|Sequence
            (:then_0
              (Utilities|FlowControl|DoOnce false :!label _label_3
                (:Completed
                  (Timeline|ResetOverHeat PlayFromStart
                    (:Update
                      (CallFunction|DevPrintwithAppend "NewEnumerator4" 0 "Cooling arm : " "" true true "(R=0.000000,G=0.658824,B=1.000000,A=1.000000)" 0.0))
                    (:Finished
                      (Variables|Default|SetEndCooldown true)
                      (Variables|Default|SetCurrentState "NewEnumerator0")
                      (goto _label_3 Reset))))))
            (:then_1
              (goto _label Reset))))
        (:NewEnumerator3
          (Components|Activation|SetActive (Variables|Default|GetFX_BossArmTrail) false false))))
    (:then_2
      (CallFunction|UpdateEmmissivStrenght))))

(fn ConstructionScript)

(fn StartPattern
  (params (Pattern%20Number%20 :type Integer))
  (Variables|Default|SetCurrentState "NewEnumerator1"))

(fn DestroyArm
  (Actor|DestroyActor))

(fn StartingLooping
  (Variables|Default|SetStartLooping true))

(fn WanderBehavior
  (params (PlayerPosition :type BP%20Player%20Character%20Object%20Reference)))

(fn RotateTowardPlayer
  (params (PlayerPosition :type Vector))
  (Variables|Player|SetPlayerPosition PlayerPosition)
  (Transformation|SetActorRotation (Math|Rotator|MakeRotfromZY (Transformation|GetActorUpVector) (- PlayerPosition (Transformation|GetWorldLocation (Variables|Default|GetSocket_Whrist)))))
  (CallFunction|UpdateDirectionArm))

(fn RotateAroundPlayer
  (params (ActorToRotate :type Actor%20Object%20Reference) (ActorTarget :type Actor%20Object%20Reference) (TargetLocation :type Vector) (Radius :type Float%20%28single-precision%29) (Angle :type Float%20%28single-precision%29) (RotationRate :type Float%20%28single-precision%29))
  (LocalVariables|SetLocation TargetLocation)
  (if (Utilities|IsValid ActorTarget)
    (bind _output_get (LocalVariables|SetLocation (Transformation|GetActorLocation ActorTarget))))
  (Transformation|SetActorLocation ActorToRotate (+ _output_get (Math|Vector|RotateVectorAroundAxis (Math|Vector|MakeVector Radius 0.0 0.0) (+ Angle RotationRate) "0,0.000000,1.000000")) false false))

(fn UpdateEmmissivStrenght
  (Rendering|Material|SetScalarParameterValueonMaterials (Variables|Default|GetMesh) "Frequency" (+ (- 1.0 (/ (Variables|HpValue|GetCurrentHp) (Variables|HpValue|GetMaxHp))) 0.3)))

(fn LaunchPatternAttack
  (Utilities|FlowControl|Sequence
    (:then_0
      (if (not (Variables|Default|GetHasSetPlayerPosition))
        (Variables|Player|SetPlayerPositionBuffer (Variables|Player|GetPlayerPosition)) ; Set Position Player at Launch Pattern
        (Variables|Default|SetHasSetPlayerPosition true)))
    (:then_1
      (switch Utilities|FlowControl|Switch|SwitchonEnum_BossAttack (Variables|Default|GetCurrentStateAttack)
        (:NewEnumerator0
          (Pattern|Laser))
        (:NewEnumerator1
          (Pattern|FulguroPoint))
        (:NewEnumerator2
          (Pattern|Invocation))
        (:NewEnumerator3
          (Pattern|ImpactGround))))))

(fn Laser)

(fn Invocation)

(fn FulguroPoint)

(fn ImpactGround)

(fn ResetValuesAttack
  (Variables|Default|SetHasSetPlayerPosition false))

(fn UpdateDirectionArm
  (bind _asbp_player_character (Utilities|Casting|CastToBP_PlayerCharacter (Game|GetPlayerCharacter 0)))
  (Variables|Default|SetArmDirection (Math|Vector|Normalize (- (Transformation|GetWorldLocation (Variables|/Game/Project/Blueprints/BP_PlayerCharacter.BP_PlayerCharacter_C|GetSpringArm _asbp_player_character)) (Transformation|GetActorLocation)))))

(fn ActiveEndAnimation)

(fn TakeDamageArm
  (params (damage :type Float%20%28single-precision%29))
  (Variables|HpValue|SetCurrentHp (- (Variables|HpValue|GetCurrentHp) damage))
  (CallFunction|DevPrint "NewEnumerator4" 0 "J'ai mal au bras, surement le vaccin covid" true true "(R=0.000000,G=0.658824,B=1.000000,A=1.000000)" 2.0))