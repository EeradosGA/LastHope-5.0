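; Combat zone actor that arms enemy spawning while the player character is inside its box.
; Box overlaps update the ACSpawner component's player flag and bind or unbind SpawnEnemies to the game instance's weapon pickup trigger.
; When triggered, ACSpawner spawns actors using the zone's spawn point tag.
; Helper functions remove enemies from a list and schedule a delayed HUD life bar hide once it is empty.
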(event OnComponentBeginOverlap(Box)
  (params (OverlappedComponent :type Primitive%20Component%20Object%20Reference) (OtherActor :type Actor%20Object%20Reference) (OtherComp :type Primitive%20Component%20Object%20Reference) (OtherBodyIndex :type Integer) (bFromSweep :type Boolean) (SweepResult :type Hit%20Result%20Structure%20%28by%20ref%29))
  (bind _isinzone_ (Default|GetIsPlayerinZone? (Variables|Default|GetAC_Spawner)))
  (if (not _isinzone_)
    (if (== (Utilities|GetClass OtherActor) "/Game/Project/Blueprints/BP_PlayerCharacter.BP_PlayerCharacter_C")
      (Utilities|Casting|CastToBP_PlayerCharacter OtherActor)
      (Default|SetPlayerinZone (Variables|Default|GetAC_Spawner) true)
      (bind _asbp_last_hope_game_instance (Utilities|Casting|CastToBP_LastHopeGameInstance (Game|GetGameInstance)))
      (EventDispatchers|BindEventtoTriggerWeaponPickup _asbp_last_hope_game_instance (delegate Custom|SpawnEnemies)))))

(event OnComponentEndOverlap(Box)
  (params (OverlappedComponent :type Primitive%20Component%20Object%20Reference) (OtherActor :type Actor%20Object%20Reference) (OtherComp :type Primitive%20Component%20Object%20Reference) (OtherBodyIndex :type Integer))
  (bind _isinzone_ (Default|GetIsPlayerinZone? (Variables|Default|GetAC_Spawner)))
  (if _isinzone_
    (if (== (Utilities|GetClass OtherActor) "/Game/Project/Blueprints/BP_PlayerCharacter.BP_PlayerCharacter_C")
      (Default|SetPlayerinZone (Variables|Default|GetAC_Spawner) false)
      (bind _asbp_last_hope_game_instance (Utilities|Casting|CastToBP_LastHopeGameInstance (Game|GetGameInstance)))
      (EventDispatchers|UnbindEventfromTriggerWeaponPickup _asbp_last_hope_game_instance (delegate Custom|SpawnEnemies)))))

(event Custom|SpawnEnemies
  (Default|SpawnActors (Variables|Default|GetAC_Spawner) (Variables|Default|GetSpawnPointsTag)))

(event Input|KeyboardEvents|NumPadFive
  (params (Key :type Key%20Structure)))

(fn ConstructionScript)

(fn CheckEnemyinZone
  (if (<= (Utilities|Array|Length (Variables|Default|GetlistEnemiesInZone)) 0)
    (if (not (Variables|Default|GetneedHideHUD))
      (Utilities|Time|SetTimerbyFunctionName (CallFunction|GetHudPlayer) "HideLifeBar" 3.0)
      (Variables|Default|SetneedHideHUD true))))

(fn RemoveEnemyfromList
  (params (ItemToFind :type BP%20Enemi%20Base%20Object%20Reference%20%28by%20ref%29))
  (bind _listenemiesinzone (Variables|Default|GetlistEnemiesInZone))
  (Utilities|Array|RemoveIndex _listenemiesinzone (Utilities|Array|FindItem _listenemiesinzone ItemToFind))
  (CallFunction|CheckEnemyinZone))

(fn RemoveHud
  (Utilities|Time|SetTimerbyFunctionName (CallFunction|GetHudPlayer) "HideLifeBar" 3.0))