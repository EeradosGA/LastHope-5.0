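; Blueprint function library for cinematic camera control, starting, playing and stopping level sequences through BP_SequenceManager and BP_PlayerCharacter.
; PlaySequence maps an enum to story sequences, while Begin toggles input possession, third-person drawing and cinematic HUD.
; Stop places a blend camera at the sequence camera's transform, then returns to first person, blending via SetViewTargetWithBlend only when called by the sequencer.
; Small helpers cover possession, TPS drawing, player look-at and a tutorial HUD prompt.
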(fn CameraManageBlendtoFirstPerson
  (params (TimeBlendEndSequence :type Float%20%28single-precision%29) (CallBySequencer? :type Boolean))
  (LocalVariables|SetL_TimeBlendEndSequence TimeBlendEndSequence)
  ;[1 0 0.9609] Get SequenceManager
  (bind _returnvalue (Actor|GetActorOfClass 0 "/Game/Project/Blueprints/Camera/BP_SequenceManager.BP_SequenceManager_C"))
  (Utilities|IsValid _returnvalue
    (:Is%20Valid
      (LocalVariables|SetL_SequenceManager _returnvalue)
      ;[0 0 1] Get PlayerCharacter
      (bind _returnvalue_2 (Actor|GetActorOfClass 0 "/Game/Project/Blueprints/BP_PlayerCharacter.BP_PlayerCharacter_C"))
      (Utilities|IsValid _returnvalue_2
        (:Is%20Valid
          (bind _output_get (LocalVariables|SetL_PlayerCharacter _returnvalue_2))
          (Utilities|FlowControl|Sequence
            (:then_0
              ;[0 1 1] Get Player Controller
              (Utilities|IsValid (Variables|/Game/Project/Blueprints/BP_PlayerCharacter.BP_PlayerCharacter_C|GetCurrentPlayerController _output_get)
                (:Is%20Valid
                  (LocalVariables|SetL_PlayerController (Variables|/Game/Project/Blueprints/BP_PlayerCharacter.BP_PlayerCharacter_C|GetCurrentPlayerController _output_get)))
                (:Is%20Not%20Valid
                  (Development|PrintString 0 "ERROR !!!! --> CFL : Player Controller is not valid" true true "(R=1.000000,G=0.007670,B=0.000000,A=1.000000)" 5.0))))
            (:then_1
              (if CallBySequencer?
                ;[1 1 1] Si valeur > 0 je peux faire un blend
                (if (> (LocalVariables|GetL_TimeBlendEndSequence) 0.0)
                  (Default|CPSetCamera (LocalVariables|GetL_PlayerCharacter) true)
                  ;[0 1 0.2] SetViewTarget qui fonctionne Blend To Player
                  (CallFunction|DevPrint "NewEnumerator6" 0 (Utilities|String|Append "CFL / CameraBlendToFirstPerson / First SetViewTargetWith --> LPlayerController  : " (Utilities|GetDisplayName (LocalVariables|GetL_PlayerController)) " / LSequenceManager : " (Utilities|GetDisplayName (LocalVariables|GetL_SequenceManager))) true true "(R=0.000000,G=1.000000,B=0.200000,A=1.000000)" 4.0)
                  (Game|Player|SetViewTargetwithBlend (LocalVariables|GetL_PlayerController) (LocalVariables|GetL_SequenceManager) 0.0 "VTBlend_Linear" 0.0 true)
                  (CallFunction|DevPrint "NewEnumerator6" 0 (Utilities|String|Append "CFL / CameraBlendToFirstPerson / Second SetViewTargetWith --> LPlayerController  : " (Utilities|GetDisplayName (LocalVariables|GetL_PlayerController)) " / LPlayerCharacter : " (Utilities|GetDisplayName (LocalVariables|GetL_PlayerCharacter))) true true "(R=0.000000,G=1.000000,B=0.200000,A=1.000000)" 4.0)
                  (Game|Player|SetViewTargetwithBlend (LocalVariables|GetL_PlayerController) (LocalVariables|GetL_PlayerCharacter) (LocalVariables|GetL_TimeBlendEndSequence) "VTBlend_Linear" 2.0 false)
                  ;[0.1647 0 1] Event Change Camera (Cette fonction d'occupe aussi de reset les inputs aprés la transition)
                  (Default|EventChangeCamera (LocalVariables|GetL_PlayerCharacter) false (LocalVariables|GetL_TimeBlendEndSequence))
                  ;[1 1 1] Undrw TPS
                  (Default|CPUndrawTPS (LocalVariables|GetL_PlayerCharacter))
                  (else
                    (Default|CPSetCamera (LocalVariables|GetL_PlayerCharacter) false :!label _label)
                    ;[0 1 0.2] SetViewTarget qui fonctionne pas de blend
                    (CallFunction|DevPrint "NewEnumerator6" 0 (Utilities|String|Append "CFL / CameraBlendToFirstPerson / Second SetViewTargetWith --> LPlayerController  : " (Utilities|GetDisplayName (LocalVariables|GetL_PlayerController)) " / LPlayerCharacter : " (Utilities|GetDisplayName (LocalVariables|GetL_PlayerCharacter))) true true "(R=0.000000,G=1.000000,B=0.200000,A=1.000000)" 1e+01)
                    (Game|Player|SetViewTargetwithBlend (LocalVariables|GetL_PlayerController) (LocalVariables|GetL_PlayerCharacter) (LocalVariables|GetL_TimeBlendEndSequence) "VTBlend_Linear" 2.0 false)
                    ;[0.1647 0 1] Possess & activate Input
                    (Default|CPDoPossess (LocalVariables|GetL_PlayerCharacter))
                    ;[1 1 1] Undrw TPS
                    (Default|CPUndrawTPS (LocalVariables|GetL_PlayerCharacter))))
                (else
                  (goto _label))))))
        (:Is%20Not%20Valid
          (Development|PrintString 0 "ERROR !!! / CFL / Blend To First Person --> Get actor \"BP_PlayerCharacter\" failed" true true "(R=1.000000,G=0.000000,B=0.000000,A=1.000000)" 5.0))))
    (:Is%20Not%20Valid
      (Development|PrintString 0 "ERROR !!! / CFL / Camera_Blend_To_First_Person --> Get actor \"BP_SequenceManager\" failed" true true "(R=1.000000,G=0.000000,B=0.000000,A=1.000000)" 5.0))))

(fn CameraStoptheSequence
  (params (CallBySequencer? :type Boolean) (TimeBlendEndSequence :type Float%20%28single-precision%29))
  (LocalVariables|SetL_CallBySequencer? CallBySequencer?)
  (Development|PrintString 0 "STOP THE SEQUENCE" true true "(R=0.906382,G=1.000000,B=0.852686,A=1.000000)")
  ;[0 0 1] Get PlayerCharacter
  (bind _returnvalue (Actor|GetActorOfClass 0 "/Game/Project/Blueprints/BP_PlayerCharacter.BP_PlayerCharacter_C"))
  (Utilities|IsValid _returnvalue
    (:Is%20Valid
      (LocalVariables|SetL_PlayerCharacter _returnvalue)
      ;[1 0 0.9609] Get SequenceManager
      (bind _returnvalue_2 (Actor|GetActorOfClass 0 "/Game/Project/Blueprints/Camera/BP_SequenceManager.BP_SequenceManager_C"))
      (Utilities|IsValid _returnvalue_2
        (:Is%20Valid
          (LocalVariables|SetL_SequenceManager _returnvalue_2)
          (Utilities|FlowControl|Sequence
            (:then_0
              ;[0.702 0.2314 0] Get ActiveCameraComponent of the sequence & set transform of camera blend
              (Utilities|IsValid (Variables|/Game/Project/Blueprints/Camera/BP_SequenceManager.BP_SequenceManager_C|GetCurrentLevelSequencePlayer (LocalVariables|GetL_SequenceManager))
                (:Is%20Valid
                  (CallFunction|DevPrint "NewEnumerator6" 0 (Utilities|String|Append "CFL / CameraStopAllTheSequence --> Get ActiveCameraComponent  :   " (Utilities|GetDisplayName (Class|LevelSequencePlayer|GetActiveCameraComponent (Variables|/Game/Project/Blueprints/Camera/BP_SequenceManager.BP_SequenceManager_C|GetCurrentLevelSequencePlayer (LocalVariables|GetL_SequenceManager)))) " / With Transform : " (Utilities|String|ToString(Transform) (Variables|/Game/Project/Blueprints/Camera/BP_SequenceManager.BP_SequenceManager_C|GetCurrentLSCameraTransform (LocalVariables|GetL_SequenceManager)))) true true "(R=0.701961,G=0.231373,B=0.000000,A=1.000000)" 5.0)
                  (Transformation|SetWorldTransform (Variables|/Game/Project/Blueprints/Camera/BP_SequenceManager.BP_SequenceManager_C|GetCameraForBlend (LocalVariables|GetL_SequenceManager)) (Variables|/Game/Project/Blueprints/Camera/BP_SequenceManager.BP_SequenceManager_C|GetCurrentLSCameraTransform (LocalVariables|GetL_SequenceManager)) false false))
                (:Is%20Not%20Valid
                  (Development|PrintString 0 "ERROR !!! : CFL : CameraBlendToFirstPerson CurrentLevelSequencePlayer is not valid" true true "(R=1.000000,G=0.000000,B=0.000000,A=1.000000)" 5.0))))
            (:then_1
              ;[0.5 0 0] Stop Current Lvl Sequence
              (Default|StopLvLSequence (LocalVariables|GetL_SequenceManager) (LocalVariables|GetL_CallBySequencer?))
              ;[1 0.6885 0] CameraBlend (Si appeler autrement que ar le sequencer le blend ne peut pas se faire)
              (CallFunction|CameraManageBlendtoFirstPerson TimeBlendEndSequence (LocalVariables|GetL_CallBySequencer?))
              ;[1 0 0.9087] HUD --> UI Hide Cross Hair
              (CallFunction|UIStop12Cinematic)
              ;[1 0.199 0.4734] Set Value Player
              (Variables|/Game/Project/Blueprints/BP_PlayerCharacter.BP_PlayerCharacter_C|SetIsInCinematic (LocalVariables|GetL_PlayerCharacter) false))))
        (:Is%20Not%20Valid
          (Development|PrintString 0 "ERROR !!! / CFL / Stop All the Sequence --> Get actor \"BP_SequenceManager\" failed" true true "(R=1.000000,G=0.000000,B=0.000000,A=1.000000)" 5.0))))
    (:Is%20Not%20Valid
      (Development|PrintString 0 "ERROR !!! / CFL / Stop the sequence --> Get actor \"BP_PlayerCharacter\" failed" true true "(R=1.000000,G=0.000000,B=0.000000,A=1.000000)" 5.0))))

(fn CameraBegintheSequence
  (params (EnableInput&Posess? :type Boolean) (DrawTPS? :type Boolean) (ToTPS? :type Boolean))
  (Development|PrintString 0 "BEGIN THE SEQUENCE" true true "(R=0.906382,G=1.000000,B=0.852686,A=1.000000)")
  (LocalVariables|SetL_EnableInput%20&%20Possess? EnableInput&Posess?)
  (LocalVariables|SetL_DrawTPS? DrawTPS?)
  ;[1 0 0.9609] Get SequenceManager
  (bind _returnvalue (Actor|GetActorOfClass 0 "/Game/Project/Blueprints/Camera/BP_SequenceManager.BP_SequenceManager_C"))
  (Utilities|IsValid _returnvalue
    (:Is%20Valid
      (LocalVariables|SetL_SequenceManager _returnvalue)
      ;[0 0 1] Get PlayerCharacter & setInput + drawTPS
      (bind _returnvalue_2 (Actor|GetActorOfClass 0 "/Game/Project/Blueprints/BP_PlayerCharacter.BP_PlayerCharacter_C"))
      (Utilities|IsValid _returnvalue_2
        (:Is%20Valid
          (LocalVariables|SetL_PlayerCharacter _returnvalue_2)
          (CallFunction|CameraEnableInput&Possess (LocalVariables|GetL_EnableInput%20&%20Possess?))
          (CallFunction|CameraDrawTPS (LocalVariables|GetL_DrawTPS?))
          ;[1 0.199 0.4734] Set Value Player
          (Variables|/Game/Project/Blueprints/BP_PlayerCharacter.BP_PlayerCharacter_C|SetIsInCinematic (LocalVariables|GetL_PlayerCharacter) true)
          ;[1 0 0.9087] HUD --> UI Hide Cross Hair
          (CallFunction|UIStart12Cinematic))
        (:Is%20Not%20Valid
          (Development|PrintString 0 "ERROR !!! / CFL / Begin the sequence --> Get actor \"BP_PlayerCharacter\" failed" true true "(R=1.000000,G=0.000000,B=0.000000,A=1.000000)" 5.0))))
    (:Is%20Not%20Valid
      (Development|PrintString 0 "ERROR !!! / CFL / Begin the sequence --> Get actor \"BP_SequenceManager\" failed" true true "(R=1.000000,G=0.000000,B=0.000000,A=1.000000)" 5.0))))

(fn CameraHUDActivateTutoActionInformation
  ;[1 0 0.1004] A METTRE A LA FIN DE LA SEQUENCE DE REVEIL
  (Default|ActivateTutoActionInformation (CallFunction|GetHudPlayer) "NewEnumerator0"))

(fn CameraPlaySequence
  (params (Sequence :type Enum_Sequence%20Enum :default "NewEnumerator0"))
  ;[1 0 0.9609] Get SequenceManager
  (bind _returnvalue (Actor|GetActorOfClass 0 "/Game/Project/Blueprints/Camera/BP_SequenceManager.BP_SequenceManager_C"))
  (Utilities|IsValid _returnvalue
    (:Is%20Valid
      (LocalVariables|SetL_SequenceManager _returnvalue)
      ;[0 0 1] Get PlayerCharacter
      (bind _returnvalue_2 (Actor|GetActorOfClass 0 "/Game/Project/Blueprints/BP_PlayerCharacter.BP_PlayerCharacter_C"))
      (Utilities|IsValid _returnvalue_2
        (:Is%20Valid
          (LocalVariables|SetL_PlayerCharacter _returnvalue_2)
          (switch Utilities|FlowControl|Switch|SwitchonEnum_Sequence Sequence
            (:NewEnumerator0
              (Development|PrintString 0 "Camera_FunctionsLibrary / None / Il faut sélectionner une séquence" true true "(R=1.000000,G=0.307249,B=0.000000,A=1.000000)"))
            (:NewEnumerator1
              ;[1 0.3209 0.788] IsInCinematic
              (Variables|/Game/Project/Blueprints/BP_PlayerCharacter.BP_PlayerCharacter_C|SetIsInCinematic (LocalVariables|GetL_PlayerCharacter) true)
              ;[1 1 1] Play Sequence Reveil
              (Default|PlayLevelSequence (LocalVariables|GetL_SequenceManager) "/Game/Project/CameraSequence/SequencerMM_Reveil.SequencerMM_Reveil" false (Utilities|Struct|MakeMovieSceneSequencePlaybackSettings false "(Value=0)" 1.0 0.0 false false true true false true false false))
              ;[0 1 0.9552] Musique --> Change la musique
              (bind _returnvalue_3 (Actor|GetActorOfClass 0 "/Game/Project/Audio/BP_MusicPlayer.BP_MusicPlayer_C"))
              (Default|PlayMusicFade _returnvalue_3 "NewEnumerator1" 3.0 3.0 0.0))
            (:NewEnumerator2
              ;[1 0.3209 0.788] IsInCinematic
              (Variables|/Game/Project/Blueprints/BP_PlayerCharacter.BP_PlayerCharacter_C|SetIsInCinematic (LocalVariables|GetL_PlayerCharacter) true)
              ;[1 1 1] Play Sequence Pre Reveil
              (Default|PlayLevelSequence (LocalVariables|GetL_SequenceManager) "/Game/Project/CameraSequence/SequencerMM_PreReveil.SequencerMM_PreReveil" true (Utilities|Struct|MakeMovieSceneSequencePlaybackSettings false "(Value=0)" 2.0 0.0 false false true true true true false false)))
            (:NewEnumerator3
              ;[1 0.3209 0.788] IsInCinematic
              (Variables|/Game/Project/Blueprints/BP_PlayerCharacter.BP_PlayerCharacter_C|SetIsInCinematic (LocalVariables|GetL_PlayerCharacter) true)
              ;[1 1 1] Play Sequence Waouh
              (Default|PlayLevelSequence (LocalVariables|GetL_SequenceManager) "/Game/Project/CameraSequence/SequencerMM_Waouh1.SequencerMM_Waouh1" false (Utilities|Struct|MakeMovieSceneSequencePlaybackSettings false "(Value=0)" 1.0 0.0 false false true true false true false false)))
            (:NewEnumerator5
              ;[1 0.3209 0.788] IsInCinematic
              (Variables|/Game/Project/Blueprints/BP_PlayerCharacter.BP_PlayerCharacter_C|SetIsInCinematic (LocalVariables|GetL_PlayerCharacter) true)
              ;[1 1 1] End Battle
              (Default|PlayLevelSequence (LocalVariables|GetL_SequenceManager) "/Game/Project/CameraSequence/SequencerMM_EndBattle_V2.SequencerMM_EndBattle_V2" false (Utilities|Struct|MakeMovieSceneSequencePlaybackSettings false "(Value=0)" 1.0 0.0 false false true true false true false false)))
            (:NewEnumerator9
              ;[1 0.3209 0.788] IsInCinematic
              (Variables|/Game/Project/Blueprints/BP_PlayerCharacter.BP_PlayerCharacter_C|SetIsInCinematic (LocalVariables|GetL_PlayerCharacter) true)
              ;[1 1 1] Showcase Enemy arme
              (Default|PlayLevelSequence (LocalVariables|GetL_SequenceManager) "/Game/Project/CameraSequence/SequencerMM_EnemyArme_V2.SequencerMM_EnemyArme_V2" false (Utilities|Struct|MakeMovieSceneSequencePlaybackSettings false "(Value=0)" 1.0 0.0 false false true true false true false false)))
            (:NewEnumerator6
              ;[1 0.3209 0.788] IsInCinematic
              (Variables|/Game/Project/Blueprints/BP_PlayerCharacter.BP_PlayerCharacter_C|SetIsInCinematic (LocalVariables|GetL_PlayerCharacter) true)
              ;[1 1 1] Begin Boss Battle
              (Default|PlayLevelSequence (LocalVariables|GetL_SequenceManager) "/Game/Project/CameraSequence/SequencerMM_BeginBossBattle.SequencerMM_BeginBossBattle" false (Utilities|Struct|MakeMovieSceneSequencePlaybackSettings false "(Value=0)" 1.0 0.0 false false true true false true false false)))
            (:NewEnumerator8
              ;[1 0.3209 0.788] IsInCinematic
              (Variables|/Game/Project/Blueprints/BP_PlayerCharacter.BP_PlayerCharacter_C|SetIsInCinematic (LocalVariables|GetL_PlayerCharacter) true)
              ;[1 1 1] End Boss Battle
              (Default|PlayLevelSequence (LocalVariables|GetL_SequenceManager) "/Game/Project/CameraSequence/SequencerMM_EndBossBattle.SequencerMM_EndBossBattle" false (Utilities|Struct|MakeMovieSceneSequencePlaybackSettings false "(Value=0)" 1.0 0.0 false false true true false true false false)))))
        (:Is%20Not%20Valid
          (Development|PrintString 0 "ERROR !!! / CFL / CameraPlaySequence --> Get actor \"BP_PlayerCharacter\" failed" true true "(R=1.000000,G=0.000000,B=0.000000,A=1.000000)" 5.0))))
    (:Is%20Not%20Valid
      (Development|PrintString 0 "ERROR !!! / CFL / PlaySequence --> Get actor \"BP_SequenceManager\" failed" true true "(R=1.000000,G=0.000000,B=0.000000,A=1.000000)" 5.0))))

(fn CameraEnableInput&Possess
  (params (EnableInput&Possess? :type Boolean))
  (LocalVariables|SetL_EnableInnput&Possess? EnableInput&Possess?)
  ;[0 0 1] Get PlayerCharacter
  (bind _returnvalue (Actor|GetActorOfClass 0 "/Game/Project/Blueprints/BP_PlayerCharacter.BP_PlayerCharacter_C"))
  (Utilities|IsValid _returnvalue
    (:Is%20Valid
      (LocalVariables|SetL_PlayerCharacter _returnvalue)
      (if (LocalVariables|GetL_EnableInnput&Possess?)
        ;[0.1647 0 1] Possess & EnableInput
        (Default|CPDoPossess (LocalVariables|GetL_PlayerCharacter))
        (else
          ;[1 0 0.1161] Unpossess & disableInput
          (Default|CPDoUnPossess (LocalVariables|GetL_PlayerCharacter)))))
    (:Is%20Not%20Valid
      (Development|PrintString 0 "ERROR !!! / CFL / Enable Input & Possess --> Get actor \"BP_PlayerCharacter\" failed" true true "(R=1.000000,G=0.000000,B=0.000000,A=1.000000)" 5.0))))

(fn CameraDrawTPS
  (params (DrawTPS? :type Boolean))
  (LocalVariables|SetL_DrawTPS? DrawTPS?)
  ;[0 0 1] Get PlayerCharacter
  (bind _returnvalue (Actor|GetActorOfClass 0 "/Game/Project/Blueprints/BP_PlayerCharacter.BP_PlayerCharacter_C"))
  (Utilities|IsValid _returnvalue
    (:Is%20Valid
      (LocalVariables|SetL_PlayerCharacter _returnvalue)
      (if (LocalVariables|GetL_DrawTPS?)
        (Default|CPDrawTPS (LocalVariables|GetL_PlayerCharacter))
        (else
          (Default|CPUndrawTPS (LocalVariables|GetL_PlayerCharacter)))))
    (:Is%20Not%20Valid
      (Development|PrintString 0 "ERROR !!! / CFL / Camera_Draw_TPS --> Get actor \"BP_PlayerCharacter\" failed" true true "(R=1.000000,G=0.000000,B=0.000000,A=1.000000)" 5.0))))

(fn CameraPlayerLookat
  (params (TargetActor :type Actor%20Object%20Reference) (SpeedLookAt :type Float%20%28single-precision%29))
  (LocalVariables|SetL_TargetActor TargetActor)
  (LocalVariables|SetL_SpeedLookAt SpeedLookAt)
  ;[0 0 1] Get PlayerCharacter & setInput + drawTPS
  (bind _returnvalue (Actor|GetActorOfClass 0 "/Game/Project/Blueprints/BP_PlayerCharacter.BP_PlayerCharacter_C"))
  (Utilities|IsValid _returnvalue
    (:Is%20Valid
      (LocalVariables|SetL_PlayerCharacter _returnvalue)
      (Default|PlayerLookat (LocalVariables|GetL_PlayerCharacter) (LocalVariables|GetL_TargetActor) (LocalVariables|GetL_SpeedLookAt)))
    (:Is%20Not%20Valid
      (Development|PrintString 0 "ERROR !!! / CFL / CameraPlayerLookAt --> Get actor \"BP_PlayerCharacter\" failed" true true "(R=1.000000,G=0.000000,B=0.000000,A=1.000000)" 5.0))))