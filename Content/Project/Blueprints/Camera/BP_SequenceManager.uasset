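; Level sequence manager actor that plays and stops the game's cinematics and registers itself on BP_LastHopeGameMode at BeginPlay.
; PlayLevelSequence replaces the current player with a new looping or one-shot one, while StopLvLSequence either stops it or jumps to its end.
; Tick caches the active sequence camera's world transform.
; Named events trigger the Reveil and Effet Waouh sequences, and DestroyCineEnemy forwards an enemy index to the GameInstance.
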(event Custom|Play_PreReveil
  ;[1 1 1] Test Play Sequence
  (CallFunction|DevPrint "NewEnumerator6" 0 "BP_SequenceManager --> Play Level Sequencer Pre Reveil" true true "(R=1.000000,G=0.011765,B=0.960784,A=1.000000)" 2.0)
  (bind _returnvalue (Sequencer|Player|CreateLevelSequencePlayer 0))
  (Class|MovieSceneSequencePlayer|PlayLooping _returnvalue -1))

(event Custom|Play_Reveil
  ;[1 1 1] Test Play Sequence
  (CallFunction|DevPrint "NewEnumerator6" 0 "BP_SequenceManager --> Play Level Sequencer Reveil" true true "(R=1.000000,G=0.011765,B=0.960784,A=1.000000)" 2.0)
  (Utilities|FlowControl|Sequence
    (:then_0
      (if (Utilities|IsValid (stale Custom|Play_PreReveil _returnvalue))
        (Sequencer|Player|Stop (stale Custom|Play_PreReveil _returnvalue) :!class /Script/MovieScene.MovieSceneSequencePlayer)))
    (:then_1
      (bind _returnvalue (Sequencer|Player|CreateLevelSequencePlayer 0))
      (Sequencer|Player|Play _returnvalue :!class /Script/MovieScene.MovieSceneSequencePlayer))))

(event Custom|PlayEffetWaouh1
  ;[1 1 1] Test Play Sequence
  (CallFunction|DevPrint "NewEnumerator6" 0 "BP_SequenceManager --> Play Level Sequencer \"Effet Waouh 1\"" true true "(R=1.000000,G=0.011765,B=0.960784,A=1.000000)" 2.0)
  (CallFunction|PlayLevelSequence 0 false))

(event Custom|PlayEffetWaouh1MM
  (CallFunction|DevPrint "NewEnumerator6" 0 "BP_SequenceManager --> Play Level Sequencer \"Effet Waouh 1MM\"" true true "(R=1.000000,G=0.011765,B=0.960784,A=1.000000)" 2.0)
  (CallFunction|PlayLevelSequence "/Game/Project/CameraSequence/SequencerMM_Waouh1.SequencerMM_Waouh1" false (Utilities|Struct|MakeMovieSceneSequencePlaybackSettings false "(Value=0)" 1.0 0.0 false false true true false false false false)))

(event EventBeginPlay
  (bind _returnvalue (Game|GetGameMode))
  (Utilities|FlowControl|Sequence
    (:then_0
      ;[0 0.8303 1] Set SequenceManager into the GameMode
      (Utilities|IsValid _returnvalue
        (:Is%20Valid
          (bind _asbp_last_hope_game_mode (Utilities|Casting|CastToBP_LastHopeGameMode _returnvalue))
          (Variables|/Game/Project/Blueprints/BP_LastHopeGameMode.BP_LastHopeGameMode_C|SetSequenceManager _asbp_last_hope_game_mode self))))
    (:then_1
      ;[0 0.2242 1] Verif CharacterRef
      (Utilities|IsValid (Variables|Default|GetCharacterRef)
        (:Is%20Not%20Valid
          (Development|PrintString "ERROR !!!! BP_SequenceManager --> CharacterRef is not valid : il faut mettre le BP du PlayerCharacter en paramètre" true true "(R=1.000000,G=0.000000,B=0.046384,A=1.000000)" 5.0))))))

(event Collision|EventActorBeginOverlap
  (params (OtherActor :type Actor%20Object%20Reference)))

(event EventTick
  (params (DeltaSeconds :type Float%20%28single-precision%29))
  (Utilities|FlowControl|Sequence
    (:then_0
      ;[1 0.8 0] Set CurrentLS Camera Transform
      (bind _currentlevelsequenceplayer (Variables|Default|GetCurrentLevelSequencePlayer)
        (:then
          (Utilities|IsValid (Class|LevelSequencePlayer|GetActiveCameraComponent _currentlevelsequenceplayer)
            (:Is%20Valid
              (CallFunction|DevPrint "NewEnumerator6" 0 (Utilities|String|Append "BP_SequenceManager / Tick --> Camera Component : " (Utilities|GetDisplayName (Class|LevelSequencePlayer|GetActiveCameraComponent _currentlevelsequenceplayer)) " / WorldTransform : " (Utilities|String|ToString(Transform) (Transformation|GetWorldTransform (Class|LevelSequencePlayer|GetActiveCameraComponent _currentlevelsequenceplayer)))) true true "(R=1.000000,G=0.800000,B=0.000000,A=1.000000)" 0.0)
              (Variables|Default|SetCurrentLSCameraTransform (Transformation|GetWorldTransform (Class|LevelSequencePlayer|GetActiveCameraComponent _currentlevelsequenceplayer))))))
        (:else)))))

(fn ConstructionScript)

(fn PlayLevelSequence
  (params (LevelSequence :type Level%20Sequence%20Object%20Reference) (Loop? :type Boolean) (setting :type Movie%20Scene%20Sequence%20Playback%20Settings%20Structure))
  (Utilities|FlowControl|Sequence
    (:then_0
      ;[0.8 0.498 1] Stop LevelSequencePlayer
      (Utilities|IsValid (Variables|Default|GetCurrentLevelSequencePlayer)
        (:Is%20Valid
          (Sequencer|Player|Stop (Variables|Default|GetCurrentLevelSequencePlayer) :!class /Script/MovieScene.MovieSceneSequencePlayer)
          (CallFunction|DevPrint "NewEnumerator6" 0 (Utilities|String|Append "BP_SequenceManager --> Stop Sequence & delete old Level SequencePlayer :" (Utilities|GetDisplayName (Variables|Default|GetCurrentLevelSequencePlayer))) true true "(R=0.800000,G=0.498039,B=1.000000,A=1.000000)" 2.0)
          ;[0.5358 0 1] Reset
          (Variables|Default|SetCurrentLevelSequence 0)
          (Variables|Default|SetCurrentLevelSequencePlayer 0)
          (Variables|Default|SetCurrentSequenceCameraActor 0)
          (Variables|Default|SetCurrentLSCameraTransform ""))
        (:Is%20Not%20Valid
          (Development|PrintString "BP_SequenceManager --> Play Level Sequence : (Stop Level SequencePlayer) : CurrentLevelSequencePlayer is not valid" true true "(R=1.000000,G=0.457516,B=0.000000,A=1.000000)"))))
    (:then_1
      ;[0 0.9059 1] Init & Play Sequence / Sequence Player
      (Utilities|IsValid LevelSequence
        (:Is%20Valid
          (bind _output_get (Variables|Default|SetCurrentLevelSequence LevelSequence))
          (bind _returnvalue (Sequencer|Player|CreateLevelSequencePlayer _output_get setting))
          (bind _output_get_2 (Variables|Default|SetCurrentLevelSequencePlayer _returnvalue))
          (Utilities|IsValid _output_get_2
            (:Is%20Valid
              (CallFunction|DevPrint "NewEnumerator6" 0 "BP_SequenceManager --> Play Level Sequence Player is valid" true true "(R=0.000000,G=0.905882,B=1.000000,A=1.000000)" 2.0)
              (if Loop?
                ;;[1 1 1] Play Loop
                (Class|MovieSceneSequencePlayer|PlayLooping _output_get_2 -1)
                (CallFunction|DevPrint "NewEnumerator6" 0 (Utilities|String|Append "BP_SequenceManager / Play Sequence Loop --> " (Utilities|GetDisplayName (Variables|Default|GetCurrentLevelSequence))) true true "(R=0.000000,G=0.905882,B=1.000000,A=1.000000)" 2.0)
                (else
                  ;;[1 1 1] Play Simple
                  (Sequencer|Player|Play _output_get_2 :!class /Script/MovieScene.MovieSceneSequencePlayer)
                  (CallFunction|DevPrint "NewEnumerator6" 0 (Utilities|String|Append "BP_Sequence / Play Sequence --> " (Utilities|GetDisplayName (Variables|Default|GetCurrentLevelSequence))) true true "(R=0.000000,G=0.905882,B=1.000000,A=1.000000)" 2.0))))
            (:Is%20Not%20Valid
              (Development|PrintString "Error : BP_SequenceManager --> Play Level Sequence Player is not valid " true true "(R=1.000000,G=0.000000,B=0.000000,A=1.000000)" 5.0))))
        (:Is%20Not%20Valid
          (Development|PrintString "ERROR --> BP_SequenceManager /PlayLevelSequence --> Level Sequence is not valid" true true "(R=1.000000,G=0.000000,B=0.000000,A=1.000000)" 5.0))))))

(fn StopLvLSequence
  (params (CallBySequencer? :type Boolean))
  ;[0 0 0] Stop SequencePlayer
  (CallFunction|DevPrint "NewEnumerator6" 0 "BP_SequenceManager --> StopSequence" true true "(R=0.000000,G=0.000000,B=0.000000,A=1.000000)" 2.0)
  (bind _currentlevelsequenceplayer (Variables|Default|GetCurrentLevelSequencePlayer)
    (:then
      (if CallBySequencer?
        ;;[1 1 1] Quand c'est déclencher par le sequencer
        (Sequencer|Player|Stop _currentlevelsequenceplayer :!class /Script/MovieScene.MovieSceneSequencePlayer)
        (else
          ;;[1 1 1] Quand c'est déclencher autrement que par le séquencer
          (Class|MovieSceneSequencePlayer|GotoEndandStop _currentlevelsequenceplayer))))
    (:else
      (Development|PrintString "ERRORRR 2 !!! BP_SequenceManager --> Event StopCurrentSequence : CurrentLevelSequencePlayer is not valid" true true "(R=1.000000,G=0.000000,B=0.000000,A=1.000000)" 5.0))))

(fn DestroyCineEnemy
  (params (indexEnemy :type Integer))
  (CallFunction|DevPrintwithAppend "NewEnumerator6" 0 "SequenceManager -->> destroy cine enemy : " (Utilities|String|ToString(Integer) indexEnemy) true true "(R=1.000000,G=0.920669,B=0.951342,A=1.000000)" 2.0)
  (bind _asbp_last_hope_game_instance (Utilities|Casting|CastToBP_LastHopeGameInstance (Game|GetGameInstance)))
  (Default|CallDestroyCineEnemy _asbp_last_hope_game_instance indexEnemy))