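; BP_TriggerSequencer is a trigger volume that starts a camera sequence when the player enters it.
; On box overlap it casts to BP_PlayerCharacter and proceeds only if the player is outside a cinematic with movement enabled.
; A DoOnce then prints a debug message and calls CameraPlaySequence with the SequenceName enum, so it fires once and blocked overlaps do not consume it.
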(event OnComponentBeginOverlap(BoxTrigger)
  (params (OverlappedComponent :type Primitive%20Component%20Object%20Reference) (OtherActor :type Actor%20Object%20Reference) (OtherComp :type Primitive%20Component%20Object%20Reference) (OtherBodyIndex :type Integer) (bFromSweep :type Boolean) (SweepResult :type Hit%20Result%20Structure%20%28by%20ref%29))
  (bind _asbp_player_character (Utilities|Casting|CastToBP_PlayerCharacter OtherActor))
  (if (and (not (Variables|/Game/Project/Blueprints/BP_PlayerCharacter.BP_PlayerCharacter_C|GetIsInCinematic _asbp_player_character)) (Variables|/Game/Project/Blueprints/BP_PlayerController.BP_PlayerController_C|GetMovement%20Enabled (Variables|/Game/Project/Blueprints/BP_PlayerCharacter.BP_PlayerCharacter_C|GetCurrentPlayerController _asbp_player_character)))
    (Utilities|FlowControl|DoOnce false
      (:Completed
        (Development|PrintString (Utilities|String|Append "BP_TriggerSequencer --> CameraPlaySequence : " (Utilities|String|EnumtoString (Variables|Default|GetSequenceName))))
        (CallFunction|CameraPlaySequence (Variables|Default|GetSequenceName))))))

(event EventBeginPlay)

(event Collision|EventActorBeginOverlap
  (params (OtherActor :type Actor%20Object%20Reference)))

(event EventTick
  (params (DeltaSeconds :type Float%20%28single-precision%29)))

(fn ConstructionScript)