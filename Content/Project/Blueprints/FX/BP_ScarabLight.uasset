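; Scarab light FX actor with two counter-rotating scarab meshes, point lights and a particle effect that can appear and disappear.
; Appear and Disappear toggle light visibility and set flags that Tick uses to ramp mesh opacity and main light intensity.
; Particles activate once appearing completes and stop immediately on Disappear, which the construction script calls.
; UpdateEmissive maps an input float to mesh emissive, particle emissive and the secondary light's intensity.
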(event EventBeginPlay)

(event Collision|EventActorBeginOverlap
  (params (OtherActor :type Actor%20Object%20Reference)))

(event EventTick
  (params (DeltaSeconds :type Float%20%28single-precision%29))
  (bind _returnvalue (* "0,180.000000, 0" DeltaSeconds))
  (bind _opacityminmax (Variables|Default|GetOpacityMinMax))
  (bind _opacityminmax_2 (Variables|Default|GetOpacityMinMax))
  (Utilities|FlowControl|Sequence
    (:then_0
      (Transformation|AddRelativeRotation (Variables|Default|GetScarabeFX_low1) _returnvalue false false)
      (Transformation|AddRelativeRotation (Variables|Default|GetScarabeFX_low) (Class|KismetMathLibrary|NegateRotator _returnvalue) false false))
    (:then_1
      (if (Variables|Default|GetAppearing)
        (bind _output_get (Variables|Default|SetCurrentTime (/ (+ (Variables|Default|GetCurrentTime) DeltaSeconds) (Variables|Default|GetAppearDuration))))
        (Rendering|Material|SetScalarParameterValueonMaterials (Variables|Default|GetScarabeFX_low1) "Opacity" (Math|Float|Clamp(Float) (Math|Float|Lerp (.x _opacityminmax) (.y _opacityminmax) _output_get)))
        (Rendering|Components|Light|SetIntensity (Variables|Default|GetPointLight) (Math|Float|Lerp 0.0 (Variables|Default|GetMaxIntensity) _output_get))
        (if (>= (Variables|Default|GetCurrentTime) 1.0)
          (Variables|Default|SetCurrentTime 0.0)
          (Variables|Default|SetAppearing false)
          (Components|Activation|Activate (Variables|Default|GetFX_ScarabLight) false))))
    (:then_2
      (if (Variables|Default|GetDisappearing)
        (bind _output_get_2 (Variables|Default|SetCurrentTime (/ (+ (Variables|Default|GetCurrentTime) 1.0) (Variables|Default|GetDisappearDuration))))
        (Rendering|Material|SetScalarParameterValueonMaterials (Variables|Default|GetScarabeFX_low1) "Opacity" (Math|Float|Clamp(Float) (Math|Float|Lerp (.x _opacityminmax_2) (.y _opacityminmax_2) (- 1.0 _output_get_2))))
        (Rendering|Components|Light|SetIntensity (Variables|Default|GetPointLight) (Math|Float|Lerp 0.0 (Variables|Default|GetMaxIntensity) (- 1.0 _output_get_2)))
        (if (>= (Variables|Default|GetCurrentTime) 1.0)
          (Variables|Default|SetCurrentTime 0.0)
          (Variables|Default|SetDisappearing false))))))

(fn ConstructionScript
  (CallFunction|Disappear))

(fn Appear
  (Variables|Default|SetAppearing true)
  (Rendering|SetVisibility (Variables|Default|GetPointLight) true false))

(fn Disappear
  (Variables|Default|SetDisappearing true)
  (Components|Activation|Deactivate (Variables|Default|GetFX_ScarabLight))
  (Rendering|SetVisibility (Variables|Default|GetPointLight) false false))

(fn UpdateEmissive
  (params (FloatValue :type Float%20%28single-precision%29))
  (bind _returnvalue (* 50 FloatValue))
  (bind _emissiveminmax (Variables|Default|GetEmissiveMinMax))
  (Rendering|Material|SetScalarParameterValueonMaterials (Variables|Default|GetScarabeFX_low1) "Emissive" (Math|Float|Lerp (.x _emissiveminmax) (.y _emissiveminmax) FloatValue))
  (Niagara|SetNiagaraVariable(Float) (Variables|Default|GetFX_ScarabLight) "User_Emissive" FloatValue)
  (if (> _returnvalue (Variables|Default|GetMinLightMini))
    (Rendering|Components|Light|SetIntensity (Variables|Default|GetPointLight1) _returnvalue)))