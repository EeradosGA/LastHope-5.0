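; BP_AutoPlay_FX is an actor that replays its Niagara effect automatically on a loop.
; Tick accumulates scaled delta time into CurrentTime, reaching its threshold roughly every three seconds.
; It then reactivates the Niagara component with reset and zeroes the counter.
; BeginPlay and the construction script are empty.
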(event EventBeginPlay)

(event Collision|EventActorBeginOverlap
  (params (OtherActor :type Actor%20Object%20Reference)))

(event EventTick
  (params (DeltaSeconds :type Float%20%28single-precision%29))
  (bind _output_get (Variables|Default|SetcurrentTime (+ (Variables|Default|GetcurrentTime) (/ DeltaSeconds 3.0))))
  (if (> (Variables|Default|GetcurrentTime) 1.0)
    (Components|Activation|Activate (Variables|Default|GetNiagara) true)
    (Variables|Default|SetcurrentTime 0.0)))

(fn ConstructionScript)