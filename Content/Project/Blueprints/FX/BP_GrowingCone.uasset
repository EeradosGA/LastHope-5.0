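; BP_GrowingCone is a cone actor that acts as a light volume for swarm Niagara effects.
; Every tick it finds all BP_SwarmFX actors and writes light start, end and axis user parameters into their Niagara components.
; The start is the actor's location, the end lies a fixed distance down the Cone's negative up vector, and the axis is that up vector's absolute value.
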(event EventBeginPlay)

(event Collision|EventActorBeginOverlap
  (params (OtherActor :type Actor%20Object%20Reference)))

(event EventTick
  (params (DeltaSeconds :type Float%20%28single-precision%29))
  (bind _cone (Variables|Default|GetCone))
  (bind _returnvalue (Math|Vector|GetUpVector _cone))
  (bind _outactors (Actor|GetAllActorsOfClass "/Game/Project/Blueprints/FX/BP_SwarmFX.BP_SwarmFX_C"))
  (for _array_element _outactors
    (Class|NiagaraComponent|SetNiagaraVariableVec3 (Variables|/Game/Project/Blueprints/FX/BP_SwarmFX.BP_SwarmFX_C|GetNiagara _array_element) "User_LightStartPos" (Transformation|GetActorLocation))
    (Niagara|SetNiagaraVariable(Vector3) (Variables|/Game/Project/Blueprints/FX/BP_SwarmFX.BP_SwarmFX_C|GetNiagara _array_element) "User_LightEndPos" (+ (Transformation|GetActorLocation) (* _returnvalue -3e+02)))
    (Niagara|SetNiagaraVariable(Vector3) (Variables|/Game/Project/Blueprints/FX/BP_SwarmFX.BP_SwarmFX_C|GetNiagara _array_element) "User_LightAxis" (Math|Vector|VectorGetAbs _returnvalue))))

(fn ConstructionScript)