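; Sandstorm actor that, once started, activates a Niagara effect and keeps the player inside its area.
; Each tick it ramps a density parameter on the hidden sphere's dynamic material up to a cap.
; When no player overlaps Sphere1, it adds movement input pulling the player toward the actor's center.
; A finished wave event calls Stop, which deactivates Niagara, disables cube collision and permanently ends the storm.
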(event Custom|WaveEndEvent
  (params (Percentage%280%20to%201%29 :type Float%20%28single-precision%29) (IsFinished? :type Boolean))
  (if IsFinished?
    (CallFunction|Stop)))

(event EventBeginPlay
  (bind _sphere (Variables|Default|GetSphere))
  (bind _returnvalue (Rendering|Material|CreateDynamicMaterialInstance _sphere 0 "/Game/Project/FX/Materials/FallingSand_Inst4.FallingSand_Inst4" "None" :!class /Script/Engine.PrimitiveComponent))
  (Rendering|Material|SetMaterial _sphere 0 _returnvalue)
  (Variables|Default|SetmatInst _returnvalue)
  (Collision|SetCollisionEnabled (Variables|Default|GetSphere) "NoCollision")
  (Rendering|SetVisibility (Variables|Default|GetSphere) false false))

(event EventTick
  (params (DeltaSeconds :type Float%20%28single-precision%29))
  (if (not (Variables|Default|Getfinished?))
    (if (Variables|Default|GetHas%20started)
      (Utilities|FlowControl|Sequence
        (:then_0
          (if (< (Variables|Default|GetSandIntensity) 1.5)
            (Rendering|Material|SetScalarParameterValue (Variables|Default|GetmatInst) "Density Variation Divider" (+ (Variables|Default|GetSandIntensity) (/ (Utilities|Time|GetWorldDeltaSeconds) 3.0)) :!class /Script/Engine.MaterialInstanceDynamic)
            (Variables|Default|SetSandIntensity (+ (Variables|Default|GetSandIntensity) (/ (Utilities|Time|GetWorldDeltaSeconds) 3.0)))))
        (:then_1
          (if (== (Utilities|Array|Length (Collision|GetOverlappingActors (Variables|Default|GetSphere1) "/Game/Project/Blueprints/BP_PlayerCharacter.BP_PlayerCharacter_C" :!class /Script/Engine.PrimitiveComponent)) 0)
            (bind _asbp_player_character (Utilities|Casting|CastToBP_PlayerCharacter (Game|GetPlayerCharacter 0)))
            (Class|PawnMovementComponent|AddInputVector (Variables|/Script/Engine.Character|GetCharacterMovement _asbp_player_character) (* (Math|Vector|GetUnitDirection(Vector) (Transformation|GetActorLocation _asbp_player_character) (Transformation|GetActorLocation)) 1.5) false)))))))

(fn ConstructionScript)

(fn Start
  (Components|Activation|Activate (Variables|Default|GetNiagara) true)
  (Variables|Default|SetHas%20started true))

(fn Stop
  (if (Variables|Default|GetHas%20started)
    (Collision|SetCollisionEnabled (Variables|Default|GetCube8) "NoCollision")
    (Components|Activation|Deactivate (Variables|Default|GetNiagara))
    (Variables|Default|SetHas%20started false)
    (Variables|Default|Setfinished? true)
    (Development|PrintString "STOP SANDTROMS")))