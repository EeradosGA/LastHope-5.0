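; BP_BeetleLaser_FX is a beetle laser hazard that damages the player and reacts to their light ring.
; Each tick, an active ring feeds its position and the controller's forward axis into the Niagara effect as a light segment with avoidance intensity.
; Box overlap events flag the player's presence; while flagged, Tick waits a cooldown Delay, then deals damage unless the ring is active.
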(event OnComponentBeginOverlap(Box)
  (params (OverlappedComponent :type Primitive%20Component%20Object%20Reference) (OtherActor :type Actor%20Object%20Reference) (OtherComp :type Primitive%20Component%20Object%20Reference) (OtherBodyIndex :type Integer) (bFromSweep :type Boolean) (SweepResult :type Hit%20Result%20Structure%20%28by%20ref%29))
  (Utilities|Casting|CastToBP_PlayerCharacter OtherActor)
  (Variables|Default|SetisOverlappingPlayer true))

(event OnComponentEndOverlap(Box)
  (params (OverlappedComponent :type Primitive%20Component%20Object%20Reference) (OtherActor :type Actor%20Object%20Reference) (OtherComp :type Primitive%20Component%20Object%20Reference) (OtherBodyIndex :type Integer))
  (Utilities|Casting|CastToBP_PlayerCharacter OtherActor)
  (Variables|Default|SetisOverlappingPlayer false))

(event EventBeginPlay)

(event Collision|EventActorBeginOverlap
  (params (OtherActor :type Actor%20Object%20Reference)))

(event EventTick
  (params (DeltaSeconds :type Float%20%28single-precision%29))
  (bind _returnvalue (Game|GetPlayerController 0))
  (bind _fx_beetlelaser (Variables|Default|GetFX_BeetleLaser))
  (bind _returnvalue_2 (Transformation|GetActorForwardVector _returnvalue))
  (Utilities|FlowControl|Sequence
    (:then_0
      (bind _asbp_player_character (Utilities|Casting|CastToBP_PlayerCharacter (Pawn|GetControlledPawn _returnvalue)))
      (if (Utilities|IsValid (.AsBP%20Ring (Utilities|Casting|CastToBP_Ring (Variables|/Game/Project/Blueprints/Items/ACP_Weapon.ACP_Weapon_C|GetCurrentRing (Variables|/Game/Project/Blueprints/BP_PlayerCharacter.BP_PlayerCharacter_C|GetACP_Weapon _asbp_player_character)))))
        (if (Variables|/Game/Project/Blueprints/Items/ItemEquip/BP_Ring.BP_Ring_C|GetisActivate (.AsBP%20Ring (Utilities|Casting|CastToBP_Ring (Variables|/Game/Project/Blueprints/Items/ACP_Weapon.ACP_Weapon_C|GetCurrentRing (Variables|/Game/Project/Blueprints/BP_PlayerCharacter.BP_PlayerCharacter_C|GetACP_Weapon _asbp_player_character)))))
          (Niagara|SetNiagaraVariable(Float) _fx_beetlelaser "User_AvoidIntensity" 2e+02)
          (Class|NiagaraComponent|SetNiagaraVariableVec3 _fx_beetlelaser "User_LightStartPos" (Transformation|GetActorLocation (Variables|/Game/Project/Blueprints/Items/ACP_Weapon.ACP_Weapon_C|GetCurrentRing (Variables|/Game/Project/Blueprints/BP_PlayerCharacter.BP_PlayerCharacter_C|GetACP_Weapon _asbp_player_character))))
          (Niagara|SetNiagaraVariable(Vector3) _fx_beetlelaser "User_LightEndPos" (+ (Transformation|GetActorLocation (Variables|/Game/Project/Blueprints/Items/ACP_Weapon.ACP_Weapon_C|GetCurrentRing (Variables|/Game/Project/Blueprints/BP_PlayerCharacter.BP_PlayerCharacter_C|GetACP_Weapon _asbp_player_character))) (* _returnvalue_2 1e+03)))
          (Class|NiagaraComponent|SetNiagaraVariableVec3 _fx_beetlelaser "User_LightAxis" (Math|Vector|VectorGetAbs _returnvalue_2))
          (else
            (Niagara|SetNiagaraVariable(Float) _fx_beetlelaser "User_AvoidIntensity" 0.0)))))
    (:then_2
      (if (Variables|Default|GetisOverlappingPlayer)
        (CallFunction|DevPrint "NewEnumerator4" 0 "Overlapping Player" true true "(R=1.000000,G=0.808808,B=0.000000,A=1.000000)" 0.0)
        (Utilities|FlowControl|Delay (Variables|Default|GetCooldownDamage))
        ;[1 1 1] Savoir si on utilise l'anneau
        (bind _asbp_player_character_2 (Utilities|Casting|CastToBP_PlayerCharacter (Pawn|GetControlledPawn (Game|GetPlayerController 0))))
        (Utilities|IsValid (.AsBP%20Ring (Utilities|Casting|CastToBP_Ring (Variables|/Game/Project/Blueprints/Items/ACP_Weapon.ACP_Weapon_C|GetCurrentRing (Variables|/Game/Project/Blueprints/BP_PlayerCharacter.BP_PlayerCharacter_C|GetACP_Weapon _asbp_player_character_2))))
          (:Is%20Valid
            (if (not (Variables|/Game/Project/Blueprints/Items/ItemEquip/BP_Ring.BP_Ring_C|GetisActivate (.AsBP%20Ring (Utilities|Casting|CastToBP_Ring (Variables|/Game/Project/Blueprints/Items/ACP_Weapon.ACP_Weapon_C|GetCurrentRing (Variables|/Game/Project/Blueprints/BP_PlayerCharacter.BP_PlayerCharacter_C|GetACP_Weapon _asbp_player_character_2))))))
              (CallFunction|DevPrint "NewEnumerator4" 0 "Aïe" true true "(R=0.000000,G=0.658824,B=1.000000,A=1.000000)" 2.0 :!label _label)
              (Default|TakeDamage _asbp_player_character_2 (Variables|Default|GetDamage) "NewEnumerator0")))
          (:Is%20Not%20Valid
            (goto _label)))))))

(fn ConstructionScript)