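; BP_TriggerFX is a trigger actor that plays an environmental rock or sand Niagara effect when its box is overlapped.
; The construction script maps two FX type enums to stonefall, sandfall or sand gust systems on two Niagara components.
; On overlap it restarts only the first component, optionally just once, adding a falling-rocks sound for the Rock type.
; The restart logic for the second component is unconnected and never runs.
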(event OnComponentBeginOverlap(Box)
  (params (OverlappedComponent :type Primitive%20Component%20Object%20Reference) (OtherActor :type Actor%20Object%20Reference) (OtherComp :type Primitive%20Component%20Object%20Reference) (OtherBodyIndex :type Integer) (bFromSweep :type Boolean) (SweepResult :type Hit%20Result%20Structure%20%28by%20ref%29))
  (bind _niagara1 (Variables|Default|GetNiagara1))
  (if (Variables|Default|GetOnceUse?)
    (if (not (Variables|Default|GetIsUse?))
      (Variables|Default|SetIsUse? true)
      (Niagara|ResetSystem _niagara1 :!label _label)
      (Components|Activation|SetAutoActivate _niagara1 true)
      (switch Utilities|FlowControl|Switch|SwitchonEnum_TypeFx (Variables|Default|GetTypeFX_1)
        (:NewEnumerator0
          (Audio|PlaySoundatLocation "/Game/Project/Audio/SFX/Environment/Rocks/SC_RocksFalling_01.SC_RocksFalling_01" (Transformation|GetWorldLocation (Variables|Default|GetNiagara1)) "0, 0, 0" 1.0 1.0 0.0 0 0 0))))
    (else
      (goto _label))))

(event EventBeginPlay)

(event Collision|EventActorBeginOverlap
  (params (OtherActor :type Actor%20Object%20Reference)))

(event EventTick
  (params (DeltaSeconds :type Float%20%28single-precision%29)))

(fn ConstructionScript
  (switch Utilities|FlowControl|Switch|SwitchonEnum_TypeFx (Variables|Default|GetTypeFX_1)
    (:NewEnumerator0
      (Variables|Default|SetNiagaraSystem_1 "/Game/Project/FX/Systems/Validé/FX_Stonefall.FX_Stonefall"))
    (:NewEnumerator1
      (Variables|Default|SetNiagaraSystem_1 "/Game/Project/FX/Systems/Validé/FX_Sandfall.FX_Sandfall"))
    (:NewEnumerator2
      (Variables|Default|SetNiagaraSystem_1 "/Game/Project/FX/Systems/Validé/FX_SandGust.FX_SandGust")))
  (Class|NiagaraComponent|SetAsset (Variables|Default|GetNiagara1) (Variables|Default|GetNiagaraSystem_1))
  (switch Utilities|FlowControl|Switch|SwitchonEnum_TypeFx (Variables|Default|GetTypeFX_2)
    (:NewEnumerator0
      (Variables|Default|SetNiagaraSystem_2 "/Game/Project/FX/Systems/Validé/FX_Stonefall.FX_Stonefall"))
    (:NewEnumerator1
      (Variables|Default|SetNiagaraSystem_2 "/Game/Project/FX/Systems/Validé/FX_Sandfall.FX_Sandfall"))
    (:NewEnumerator2
      (Variables|Default|SetNiagaraSystem_2 "/Game/Project/FX/Systems/Validé/FX_SandGust.FX_SandGust")))
  (Class|NiagaraComponent|SetAsset (Variables|Default|GetNiagara2) (Variables|Default|GetNiagaraSystem_2)))