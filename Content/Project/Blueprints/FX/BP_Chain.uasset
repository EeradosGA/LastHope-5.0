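; BP_Chain is a physics chain that points toward a named BP_Pivot, with links fading out along its length.
; BeginPlay repeats two template links, pinning locked indices and joining neighbors with spawned constraint actors that copy the template's swing limits.
; Tick places the last link toward the pivot, scaling reach by pivot distance up to the chain's length.
; Appear and Disappear trigger timed opacity fades through material parameters.
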(event EventBeginPlay
  (bind _link_2 (Variables|Default|GetLink_2))
  (bind _link_1 (Variables|Default|GetLink_1))
  (bind _links (Variables|Default|GetLinks))
  (bind _link_1_2 (Variables|Default|GetLink_1))
  (bind _physicsconstraint (Variables|Default|GetPhysicsConstraint))
  (bind _link_1_3 (Variables|Default|GetLink_1))
  (bind _returnvalue (Transformation|GetWorldLocation _link_2))
  (bind _returnvalue_2 (Transformation|GetWorldLocation _link_1_2))
  (bind _returnvalue_3 (Class|PhysicsConstraintComponent|GetCurrentSwing2 _physicsconstraint))
  (bind _returnvalue_4 (Transformation|GetWorldLocation _link_1))
  (bind _returnvalue_5 (- _returnvalue _returnvalue_2))
  (Utilities|FlowControl|Sequence
    (:then_0
      (Variables|Default|Setscale (Transformation|GetWorldScale (Variables|Default|GetLink_1)))
      (Utilities|Array|Add _links (Variables|Default|GetLink_1))
      (Utilities|Array|Add _links (Variables|Default|GetLink_2))
      (bind _output_get (Variables|Default|Setid 2))
      (while (< _output_get (Variables|Default|GetLinkNumber))
        (bind _returnvalue_6 (AddComponent|AddStaticMeshComponent true (Transformation|GetRelativeTransform (Variables|Default|GetDefaultSceneRoot))))
        (Collision|SetCollisionProfileName _returnvalue_6 "Custom..." true :!class /Script/Engine.PrimitiveComponent)
        (Collision|SetCollisionResponsetoAllChannels _returnvalue_6 "ECR_Ignore")
        (Collision|SetCollisionResponsetoChannel _returnvalue_6 "ECC_WorldDynamic" "ECR_Block")
        (Collision|SetCollisionResponsetoChannel _returnvalue_6 "ECC_WorldStatic" "ECR_Block")
        (Collision|SetCollisionObjectType _returnvalue_6 "ECC_GameTraceChannel2")
        (Transformation|SetWorldLocation _returnvalue_6 (+ (Transformation|GetWorldLocation _link_1_2) (* _returnvalue_5 (Variables|Default|Getid))) false true)
        (Transformation|SetWorldScale3D _returnvalue_6 (Variables|Default|Getscale))
        (if (Utilities|Array|ContainsItem (Variables|Default|GetLockedLinks) (Variables|Default|Getid))
          (Physics|SetSimulatePhysics _returnvalue_6 false)
          (else
            (Physics|SetSimulatePhysics _returnvalue_6 true)))
        (bind _link (CallFunction|GetNextLink))
        (Components|StaticMesh|SetStaticMesh _returnvalue_6 (Variables|/Script/Engine.StaticMeshComponent|GetStaticMesh _link))
        (Transformation|SetWorldRotation _returnvalue_6 (Transformation|GetWorldRotation _link) false false)
        (Transformation|SetMobility _returnvalue_6 "Movable")
        (Utilities|Array|Add (Variables|Default|GetLinks) _returnvalue_6)
        (bind _returnvalue_7 (Game|SpawnActorfromClass "/Script/Engine.PhysicsConstraintActor" (Transformation|GetRelativeTransform (Variables|Default|GetDefaultSceneRoot)) "AlwaysSpawn" self 0))
        (Transformation|SetWorldLocation (Variables|/Script/Engine.Actor|GetRootComponent _returnvalue_7) (+ (Transformation|GetWorldLocation _link_1_3) (- (Transformation|GetWorldLocation (Variables|Default|GetPhysicsConstraint)) (Transformation|GetWorldLocation _link_1_3)) (* _returnvalue_5 (- (Variables|Default|Getid) 1))) false true)
        (Class|PhysicsConstraintComponent|SetConstrainedComponents (Variables|/Script/Engine.PhysicsConstraintActor|GetConstraintComp _returnvalue_7) (Utilities|Array|Get(acopy) (Variables|Default|GetLinks) (- (Variables|Default|Getid) 1)) "None" (Utilities|Array|Get(acopy) (Variables|Default|GetLinks) (Variables|Default|Getid)) "None")
        (Class|PhysicsConstraintComponent|SetDisableCollision (Variables|/Script/Engine.PhysicsConstraintActor|GetConstraintComp _returnvalue_7) true)
        (Class|PhysicsConstraintComponent|SetAngularSwing1Limit (Variables|/Script/Engine.PhysicsConstraintActor|GetConstraintComp _returnvalue_7) "ACM_Limited" (Class|PhysicsConstraintComponent|GetCurrentSwing1 _physicsconstraint))
        (Class|PhysicsConstraintComponent|SetAngularSwing2Limit (Variables|/Script/Engine.PhysicsConstraintActor|GetConstraintComp _returnvalue_7) "ACM_Limited" _returnvalue_3)
        (Class|PhysicsConstraintComponent|SetAngularTwistLimit (Variables|/Script/Engine.PhysicsConstraintActor|GetConstraintComp _returnvalue_7) "ACM_Limited" _returnvalue_3)
        (Class|PhysicsConstraintComponent|SetLinearXLimit (Variables|/Script/Engine.PhysicsConstraintActor|GetConstraintComp _returnvalue_7) "LCM_Locked" 0.0)
        (Class|PhysicsConstraintComponent|SetLinearYLimit (Variables|/Script/Engine.PhysicsConstraintActor|GetConstraintComp _returnvalue_7) "LCM_Locked" 0.0)
        (Class|PhysicsConstraintComponent|SetLinearZLimit (Variables|/Script/Engine.PhysicsConstraintActor|GetConstraintComp _returnvalue_7) "LCM_Locked" 0.0)
        (Math|Integer|IncrementInt (Variables|Default|Getid))))
    (:then_1
      (CallFunction|AttachtoPivot))
    (:then_2
      (Variables|Default|SetMaxChainLength (* (Math|Vector|Distance(Vector) _returnvalue_4 (Transformation|GetWorldLocation (Utilities|GetLastLink))) 1.0))
      (Variables|Default|SetMinChainLength (Math|Vector|Distance(Vector) _returnvalue_4 (Transformation|GetWorldLocation (Utilities|Array|Get(acopy) (Variables|Default|GetLinks) (- (Variables|Default|GetNumberOfVisibleLinks) 1))))))
    (:then_3
      (for (_array_element _array_index) (Variables|Default|GetLinks)
        (Rendering|Material|SetScalarParameterValueonMaterials _array_element "Opacity" (* 1.0 (- 1.0 (Math|Float|Clamp(Float) (/ (Math|Conversions|ToFloat(Integer) _array_index) (Math|Conversions|ToFloat(Integer) (Variables|Default|GetNumberOfVisibleLinks)))))))
        (Rendering|Material|SetScalarParameterValueonMaterials _array_element "Emissive" (* (* 1.0 (- 1.0 (Math|Float|Clamp(Float) (/ (Math|Conversions|ToFloat(Integer) _array_index) (Math|Conversions|ToFloat(Integer) (Variables|Default|GetNumberOfVisibleLinks)))))) 5.0))
        (if (== _array_index (- (Variables|Default|GetNumberOfVisibleLinks) 1))
          (Rendering|Material|SetScalarParameterValueonMaterials _array_element "Dissolve Amount" -0.6))))))

(event Collision|EventActorBeginOverlap
  (params (OtherActor :type Actor%20Object%20Reference)))

(event EventTick
  (params (DeltaSeconds :type Float%20%28single-precision%29))
  (bind _returnvalue (Transformation|GetActorLocation))
  (bind _pivot (Variables|Default|GetPivot))
  (bind _maxchainlength (Variables|Default|GetMaxChainLength))
  (bind _maxdistancetopivot (Variables|Default|GetMaxDistanceToPivot))
  (bind _returnvalue_2 (Transformation|GetActorLocation _pivot))
  (bind _returnvalue_3 (- _returnvalue_2 _returnvalue))
  (bind _returnvalue_4 (Math|Vector|Normalize _returnvalue_3))
  (bind _returnvalue_5 (Math|Vector|VectorLength _returnvalue_3))
  (bind _returnvalue_6 (/ _returnvalue_5 _maxdistancetopivot))
  (bind _returnvalue_7 (Math|Float|Clamp(Float) _returnvalue_6))
  (bind _returnvalue_8 (* _maxchainlength _returnvalue_7))
  (bind _returnvalue_9 (* _returnvalue_4 _returnvalue_8))
  (Utilities|FlowControl|Sequence
    (:then_0
      (Transformation|SetWorldLocation (Utilities|GetLastLink) (+ (Transformation|GetWorldLocation (Variables|Default|GetLink_1)) _returnvalue_9) false false)
      (Transformation|SetWorldRotation (Utilities|GetLastLink) (Math|Rotator|MakeRotfromX (Math|Vector|NegateVector _returnvalue_9)) false false))
    (:then_2
      (if (Variables|Default|GetAppearing)
        (bind _output_get (Variables|Default|SetCurrentTime (+ (Variables|Default|GetCurrentTime) (/ (Utilities|Time|GetWorldDeltaSeconds) (Variables|Default|GetAppearTime)))))
        (for (_array_element _array_index) (Variables|Default|GetLinks)
          (Rendering|Material|SetScalarParameterValueonMaterials _array_element "Opacity" (Math|Float|Lerp 0.0 (Math|Float|Clamp(Float) (* 1.0 (- 1.0 (Math|Float|Clamp(Float) (/ (Math|Conversions|ToFloat(Integer) _array_index) (Math|Conversions|ToFloat(Integer) (Variables|Default|GetNumberOfVisibleLinks))))))) _output_get)))
        (if (>= (Variables|Default|GetCurrentTime) 1.0)
          (Variables|Default|SetAppearing false)
          (Variables|Default|SetCurrentTime 0.0))))
    (:then_3
      (if (Variables|Default|GetDisappearing)
        (bind _output_get_2 (Variables|Default|SetCurrentTime (+ (Variables|Default|GetCurrentTime) (/ (Utilities|Time|GetWorldDeltaSeconds) (Variables|Default|GetDisappearTime)))))
        (for (_array_element_2 _array_index_2) (Variables|Default|GetLinks)
          (Rendering|Material|SetScalarParameterValueonMaterials _array_element_2 "Opacity" (Math|Float|Lerp 0.0 (Math|Float|Clamp(Float) (* 1.0 (- 1.0 (Math|Float|Clamp(Float) (/ (Math|Conversions|ToFloat(Integer) _array_index_2) (Math|Conversions|ToFloat(Integer) (Variables|Default|GetNumberOfVisibleLinks))))))) (- 1.0 _output_get_2))))
        (if (>= (Variables|Default|GetCurrentTime) 1.0)
          (Variables|Default|SetDisappearing false)
          (Variables|Default|SetCurrentTime 0.0))))))

(fn ConstructionScript)

(fn GetNextLink
  (if (== (Math|Integer|%(Integer) (Variables|Default|Getid) 2) 0)
    (LocalVariables|SetTempLink (Variables|Default|GetLink_1))
    (else
      (LocalVariables|SetTempLink (Variables|Default|GetLink_2))))
  (return (LocalVariables|GetTempLink)))

(fn AttachtoPivot
  (bind _outactors (Actor|GetAllActorsOfClass "/Game/Project/Blueprints/FX/BP_Pivot.BP_Pivot_C"))
  (bind _array_element (Utilities|Array|ForEachLoopwithBreak _outactors :!label _label)
    (:LoopBody
      (if (Utilities|Name|Equal(Name) (Variables|/Game/Project/Blueprints/FX/BP_Pivot.BP_Pivot_C|GetPivotName _array_element) (Variables|Default|GetPivotNameToAttach))
        (Variables|Default|SetPivot _array_element)
        (goto _label Break)))))

(fn Appear
  (Variables|Default|SetAppearing true))

(fn Disappear
  (Variables|Default|SetDisappearing true))