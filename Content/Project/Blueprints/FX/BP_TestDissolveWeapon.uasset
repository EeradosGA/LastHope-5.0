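; BP_TestDissolveWeapon is a test actor that repeatedly plays a dissolve effect on its Cylinder component.
; Tick accumulates time and restarts a timeline roughly every three seconds.
; The timeline drives the "Dissolve Amount" scalar parameter on the cylinder's materials, then resets it to -1 when finished.
; A disconnected branch holds an alternative that animates the same parameter by manual time accumulation.
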(event EventBeginPlay)

(event Collision|EventActorBeginOverlap
  (params (OtherActor :type Actor%20Object%20Reference)))

(event EventTick
  (params (DeltaSeconds :type Float%20%28single-precision%29))
  (bind _cylinder (Variables|Default|GetCylinder))
  (bind _output_get (Variables|Default|Setdelay (+ (Variables|Default|Getdelay) DeltaSeconds)))
  (if (> _output_get 3.0)
    (Variables|Default|Setdelay 0.0)
    (bind _amount (Timeline|Timeline_0 PlayFromStart)
      (:Update
        (Rendering|Material|SetScalarParameterValueonMaterials _cylinder "Dissolve Amount" _amount))
      (:Finished
        (Rendering|Material|SetScalarParameterValueonMaterials _cylinder "Dissolve Amount" -1.0)))))

(fn ConstructionScript)