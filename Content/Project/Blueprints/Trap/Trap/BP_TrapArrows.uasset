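; Arrow trap actor that launches a fixed set of five BP_Arrow projectiles when triggered.
; The construction script calls its parent, gathers five child actor components into a list and sets each one's class to BP_Arrow.
; ActiveTrap loops over that list and activates each arrow's projectile movement.
; A disconnected construction branch would instead spawn a variable number of arrow components from NbArrows, but it never runs.
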(event EventBeginPlay)

(event Collision|EventActorBeginOverlap
  (params (OtherActor :type Actor%20Object%20Reference)))

(event EventTick
  (params (DeltaSeconds :type Float%20%28single-precision%29)))

(event EventActiveTrap
  (for _array_element (Variables|Default|GetListChildArrows)
    (bind _asbp_arrow (Utilities|Casting|CastToBP_Arrow (Variables|/Script/Engine.ChildActorComponent|GetChildActor _array_element)))
    (Components|Activation|Activate (Variables|/Game/Project/Blueprints/Trap/Trap/BP_Arrow.BP_Arrow_C|GetProjectileMovement _asbp_arrow) true)))

(fn ConstructionScript
  (|CallParentFunction)
  (bind _output_get (Variables|Default|SetListChildArrows (Utilities|Array|MakeArray (Variables|Default|GetChildActor) (Variables|Default|GetChildActor1) (Variables|Default|GetChildActor2) (Variables|Default|GetChildActor3) (Variables|Default|GetChildActor4))))
  (for _array_element _output_get
    (ChildActorComponent|SetChildActorClass _array_element "/Game/Project/Blueprints/Trap/Trap/BP_Arrow.BP_Arrow_C")))