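; BP_TrapDalle is a pressure plate slab that sinks when something overlaps its box and activates a linked trap.
; Begin overlap sets a target height below the start position and calls ActiveTrapMessage on TrapLink; end overlap restores the start height.
; Tick eases the mesh's Z toward that target with FInterpTo once movement starts.
; The Moving flag is never cleared, and both Down branches perform the same move.
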(event OnComponentBeginOverlap(Box)
  (params (OverlappedComponent :type Primitive%20Component%20Object%20Reference) (OtherActor :type Actor%20Object%20Reference) (OtherComp :type Primitive%20Component%20Object%20Reference) (OtherBodyIndex :type Integer) (bFromSweep :type Boolean) (SweepResult :type Hit%20Result%20Structure%20%28by%20ref%29))
  (Variables|Default|SetValueStop (- (.z (Variables|Default|GetLocationStart)) (Variables|Default|GetValuePush)))
  (Variables|Default|SetMoving? true)
  (Variables|Default|SetDown? true)
  (Class|InterfaceActivateTrap|ActiveTrap(Message) (Variables|Default|GetTrapLink)))

(event OnComponentEndOverlap(Box)
  (params (OverlappedComponent :type Primitive%20Component%20Object%20Reference) (OtherActor :type Actor%20Object%20Reference) (OtherComp :type Primitive%20Component%20Object%20Reference) (OtherBodyIndex :type Integer))
  (Variables|Default|SetValueStop (.z (Variables|Default|GetLocationStart)))
  (Variables|Default|SetMoving? true)
  (Variables|Default|SetDown? false))

(event EventBeginPlay
  (Variables|Default|SetLocationStart (Transformation|GetWorldLocation (Variables|Default|GetMeshDalle))))

(event EventTick
  (params (DeltaSeconds :type Float%20%28single-precision%29))
  (if (Variables|Default|GetMoving?)
    (Variables|Default|SetLocationDalle (Transformation|GetWorldLocation (Variables|Default|GetMeshDalle)))
    (if (Variables|Default|GetDown?)
      (Transformation|SetWorldLocation (Variables|Default|GetMeshDalle) (Math|Vector|MakeVector (.x (Variables|Default|GetLocationDalle)) (.y (Variables|Default|GetLocationDalle)) (Math|Interpolation|FInterpTo (.z (Variables|Default|GetLocationDalle)) (Variables|Default|GetValueStop) (Utilities|Time|GetWorldDeltaSeconds) 1.0)) false false)
      (else
        (Transformation|SetWorldLocation (Variables|Default|GetMeshDalle) (Math|Vector|MakeVector (.x (Variables|Default|GetLocationDalle)) (.y (Variables|Default|GetLocationDalle)) (Math|Interpolation|FInterpTo (.z (Variables|Default|GetLocationDalle)) (Variables|Default|GetValueStop) (Utilities|Time|GetWorldDeltaSeconds) 1.0)) false false)))))

(fn ConstructionScript)