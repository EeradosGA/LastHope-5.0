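; Player controller that turns input into BP_PlayerCharacter actions: movement, camera, jump, dodge, interaction, attacks and ring/bracelet use.
; Movement axes ramp acceleration and resolve an eight-way direction that steers dodges and limits sprinting to forward directions.
; Tick times held attacks to choose light or heavy, and line-traces from the camera to target items, toggling pop-ups and crosshair size.
; Debug inputs teleport, damage the player and grant equipment.
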(event EventBeginPlay
  ;[0.2138 1 0.2401] Sprint and begin play
  (Variables|References|SetRefPlayer (.AsBP%20Player%20Character (Utilities|Casting|CastToBP_PlayerCharacter (Game|GetPlayerCharacter 0))))
  (Utilities|Map|Add (Variables|/Game/Project/Blueprints/BP_PlayerCharacter.BP_PlayerCharacter_C|GetDirection (Variables|References|GetRefPlayer)) "Back-Right" "0,0,315.000000")
  (Utilities|Map|Add (Variables|/Game/Project/Blueprints/BP_PlayerCharacter.BP_PlayerCharacter_C|GetDirection (Variables|References|GetRefPlayer)) "Right" "0,0,270.000000")
  (Utilities|Map|Add (Variables|/Game/Project/Blueprints/BP_PlayerCharacter.BP_PlayerCharacter_C|GetDirection (Variables|References|GetRefPlayer)) "Front-Right" "0,0,225.000000")
  (Utilities|Map|Add :TargetMap (Variables|/Game/Project/Blueprints/BP_PlayerCharacter.BP_PlayerCharacter_C|GetDirection (Variables|References|GetRefPlayer)) :Key "Back")
  (Utilities|Map|Add (Variables|/Game/Project/Blueprints/BP_PlayerCharacter.BP_PlayerCharacter_C|GetDirection (Variables|References|GetRefPlayer)) "Front" "0,0,180.000000")
  (Utilities|Map|Add (Variables|/Game/Project/Blueprints/BP_PlayerCharacter.BP_PlayerCharacter_C|GetDirection (Variables|References|GetRefPlayer)) "Back-Left" "0,0,45.000000")
  (Utilities|Map|Add (Variables|/Game/Project/Blueprints/BP_PlayerCharacter.BP_PlayerCharacter_C|GetDirection (Variables|References|GetRefPlayer)) "Left" "0,0,90.000000")
  (Utilities|Map|Add (Variables|/Game/Project/Blueprints/BP_PlayerCharacter.BP_PlayerCharacter_C|GetDirection (Variables|References|GetRefPlayer)) "Front-Left" "0,0,135.000000"))

(event Collision|EventActorBeginOverlap
  (params (OtherActor :type Actor%20Object%20Reference))
  ;[1 1 1] On Collectibles
  (bind _asbp_player_character (Utilities|Casting|CastToBP_PlayerCharacter OtherActor))
  (if (not (Math|Rotator|Equal(Rotator) (Math|Rotator|FindLookatRotation (Transformation|GetWorldLocation (Variables|Default|GetSphere)) (Transformation|GetWorldLocation (Variables|/Game/Project/Blueprints/BP_PlayerCharacter.BP_PlayerCharacter_C|GetCamera _asbp_player_character))) (Transformation|GetWorldRotation (Variables|/Game/Project/Blueprints/BP_PlayerCharacter.BP_PlayerCharacter_C|GetCamera _asbp_player_character)) 1.8e+02))
    (Development|PrintString "Not Looking at object")))

(event EventTick
  (params (DeltaSeconds :type Float%20%28single-precision%29))
  (bind _refplayer (Variables|References|GetRefPlayer))
  (bind _refplayer_2 (Variables|References|GetRefPlayer))
  (bind _directionstring (Variables|DashRelated|GetDirectionString))
  (bind _refplayer_3 (Variables|References|GetRefPlayer))
  (bind _refplayer_4 (Variables|References|GetRefPlayer))
  (bind _refplayer_5 (Variables|References|GetRefPlayer))
  (bind _refplayer_6 (Variables|References|GetRefPlayer))
  (bind _direction (Variables|/Game/Project/Blueprints/BP_PlayerCharacter.BP_PlayerCharacter_C|GetDirection _refplayer))
  (bind _camera (Variables|/Game/Project/Blueprints/BP_PlayerCharacter.BP_PlayerCharacter_C|GetCamera _refplayer_3))
  (bind _value (Utilities|Map|Find _direction _directionstring))
  (bind _returnvalue (Transformation|GetWorldLocation _camera))
  (bind _returnvalue_2 (> (.z _value) 95.0))
  (bind _returnvalue_3 (< (.z _value) 265.0))
  (bind _returnvalue_4 (and _returnvalue_3 _returnvalue_2))
  (Utilities|FlowControl|Sequence
    (:then_0
      ;[1 1 1] Count CD For Attack Heavy
      (if (Variables|Attack|GetAttackPress?)
        (Variables|Attack|CDHeavy|SetCurrentTimeCDAttack (+ (Variables|Attack|CDHeavy|GetCurrentTimeCDAttack) (Utilities|Time|GetWorldDeltaSeconds)))))
    (:then_1
      (Utilities|FlowControl|Sequence
        (:then_0
          (if (Variables|SprintRelated|GetSprinting?)
            (if (not _returnvalue_4)
              (Variables|SprintRelated|SetSprinting? false)
              (Variables|DashRelated|SetCurrentAcceleration 1.0))
            (elif _returnvalue_4
              (if (Variables|SprintRelated|GetSprintPressed)
                (Variables|SprintRelated|SetSprinting? true)))))
        (:then_1
          (if (Variables|SprintRelated|GetSprinting?)
            (if (Math|Vector|VectorIsNearlyZero (Transformation|GetVelocity (Variables|References|GetRefPlayer)) 1.0)
              (Variables|SprintRelated|SetSprinting? false)
              (Variables|SprintRelated|SetSprintPressed false)
              (Development|PrintString "Hello"))))))
    (:then_2
      (bind _outhit (Collision|LineTraceByChannel _returnvalue (+ _returnvalue (* (Math|Vector|GetForwardVector _camera) 225.0)) "TraceTypeQuery1" false 0 "None"))
      (bind _asbp_item_equip (Utilities|Casting|CastToBP_ItemEquip (.hitactor _outhit))
        (:then
          (bind _output_get (Variables|/Game/Project/Blueprints/BP_PlayerCharacter.BP_PlayerCharacter_C|SetItemOverlaped _refplayer_4 _asbp_item_equip))
          (if (not (Variables|/Game/Project/Blueprints/BP_PlayerCharacter.BP_PlayerCharacter_C|GetCollided _refplayer_4))
            (Variables|/Game/Project/Blueprints/BP_PlayerCharacter.BP_PlayerCharacter_C|SetCollided _refplayer_4 true)
            (bind _asw_pop_up_tuto (Utilities|Casting|CastToW_PopUpTuto (UserInterface|GetUserWidgetObject (Variables|/Game/Project/Blueprints/Items/BP_Item.BP_Item_C|GetWidget _output_get))))
            (Default|DrawPopUp _asw_pop_up_tuto)
            (Default|UpdateCrosshairSelectionSize (CallFunction|GetHudPlayer) true :!label _label)
            (Variables|Default|SetcrosshairIsOnItem? true)))
        (:CastFailed
          (bind _asbp_item (Utilities|Casting|CastToBP_Item (.hitactor _outhit))
            (:then
              (bind _output_get_2 (Variables|/Game/Project/Blueprints/BP_PlayerCharacter.BP_PlayerCharacter_C|SetItemOverlaped _refplayer_2 _asbp_item))
              (if (not (Variables|/Game/Project/Blueprints/BP_PlayerCharacter.BP_PlayerCharacter_C|GetCollided _refplayer_2))
                (Variables|/Game/Project/Blueprints/BP_PlayerCharacter.BP_PlayerCharacter_C|SetCollided _refplayer_2 true)
                (bind _asw_pop_up_tuto_2 (Utilities|Casting|CastToW_PopUpTuto (UserInterface|GetUserWidgetObject (Variables|/Game/Project/Blueprints/Items/BP_Item.BP_Item_C|GetWidget _output_get_2))))
                (Default|DrawPopUp _asw_pop_up_tuto_2)
                (goto _label)))
            (:CastFailed
              (Utilities|IsValid (Variables|/Game/Project/Blueprints/BP_PlayerCharacter.BP_PlayerCharacter_C|GetItemOverlaped (Variables|References|GetRefPlayer))
                (:Is%20Valid
                  (bind _asw_pop_up_tuto_3 (Utilities|Casting|CastToW_PopUpTuto (UserInterface|GetUserWidgetObject (Variables|/Game/Project/Blueprints/Items/BP_Item.BP_Item_C|GetWidget (Variables|/Game/Project/Blueprints/BP_PlayerCharacter.BP_PlayerCharacter_C|GetItemOverlaped (Variables|References|GetRefPlayer))))))
                  (Default|HidePopUp _asw_pop_up_tuto_3)
                  (Variables|/Game/Project/Blueprints/BP_PlayerCharacter.BP_PlayerCharacter_C|SetItemOverlaped _refplayer_6 0)
                  (Variables|/Game/Project/Blueprints/BP_PlayerCharacter.BP_PlayerCharacter_C|SetCollided _refplayer_6 false)
                  (Default|UpdateCrosshairSelectionSize (CallFunction|GetHudPlayer) false))
                (:Is%20Not%20Valid
                  (if (Variables|Default|GetcrosshairIsOnItem?)
                    (Variables|/Game/Project/Blueprints/BP_PlayerCharacter.BP_PlayerCharacter_C|SetItemOverlaped _refplayer_5 0)
                    (Variables|/Game/Project/Blueprints/BP_PlayerCharacter.BP_PlayerCharacter_C|SetCollided _refplayer_5 false)
                    (Default|UpdateCrosshairSelectionSize (CallFunction|GetHudPlayer) false)
                    (Variables|Default|SetcrosshairIsOnItem? false)))))))))))

(event Input|ActionEvents|InputActionInteract
  (params (Key :type Key%20Structure :default "None"))
  (bind _refplayer (Variables|References|GetRefPlayer))
  (bind _objectoverlaped (Variables|/Game/Project/Blueprints/BP_PlayerCharacter.BP_PlayerCharacter_C|GetObjectOverlaped _refplayer))
  (bind _itemoverlaped (Variables|/Game/Project/Blueprints/BP_PlayerCharacter.BP_PlayerCharacter_C|GetItemOverlaped _refplayer))
  ;[1 1 1] INTERACT
  (:Pressed
    (Utilities|IsValid _itemoverlaped
      (:Is%20Valid
        ;;[1 1 1] Collect Item
        (if (or (Utilities|Enum|Equal(Enum) (.typeitem (Variables|/Game/Project/Blueprints/Items/BP_Item.BP_Item_C|GetStruct%20InfoItem _itemoverlaped)) "NewEnumerator3") (Variables|/Game/Project/Blueprints/Items/ACP_Inventory.ACP_Inventory_C|GethaveBackpack? (Variables|/Game/Project/Blueprints/BP_PlayerCharacter.BP_PlayerCharacter_C|GetACP_Inventory _refplayer)))
          (Default|AddItem (Variables|/Game/Project/Blueprints/BP_PlayerCharacter.BP_PlayerCharacter_C|GetACP_Inventory _refplayer) _itemoverlaped (Utilities|GetClass _itemoverlaped))
          (Actor|DestroyActor _itemoverlaped)
          (Development|PrintString "Collecting")
          (else
            ;;[1 1 1] Use Object
            (Utilities|IsValid _objectoverlaped :!label _label
              (:Is%20Valid
                (Development|PrintString "Activating")
                (Default|UseObject _objectoverlaped))
              (:Is%20Not%20Valid
                (Development|PrintString "Can't Interact"))))))
      (:Is%20Not%20Valid
        (goto _label)))))

(event Input|ActionEvents|InputActionUse
  (params (Key :type Key%20Structure :default "None"))
  (bind _refplayer (Variables|References|GetRefPlayer))
  (bind _acp_weapon (Variables|/Game/Project/Blueprints/BP_PlayerCharacter.BP_PlayerCharacter_C|GetACP_Weapon _refplayer))
  ;[1 1 1] Attack Weapon
  (:Pressed
    (if (Variables|/Game/Project/Blueprints/Items/ACP_Weapon.ACP_Weapon_C|GetWeaponEquip? (Variables|/Game/Project/Blueprints/BP_PlayerCharacter.BP_PlayerCharacter_C|GetACP_Weapon _refplayer))
      (bind _canuse_ (CallFunction|ConditionforAttack))
      (if (not _canuse_)
        (Variables|Attack|SetAttackPress? true))))
  (:Released
    (Variables|Attack|SetAttackPress? false)
    (if (Variables|/Game/Project/Blueprints/Items/ACP_Weapon.ACP_Weapon_C|GetWeaponEquip? _acp_weapon)
      (bind _canuse__2 (CallFunction|ConditionforAttack))
      (if (not _canuse__2)
        (if (< (Variables|Attack|CDHeavy|GetCurrentTimeCDAttack) (Variables|Attack|CDHeavy|GetTimeToCDAttack))
          (Default|AttackSlight _acp_weapon)
          (else
            (Default|AttackHeavy _acp_weapon)))
        (Variables|Attack|CDHeavy|SetCurrentTimeCDAttack 0.0)))))

(event Input|ActionEvents|InputActionGetBracelet
  (params (Key :type Key%20Structure :default "None"))
  ;[1 1 1] Debug equipment and tp
  (:Pressed
    (bind _returnvalue (Game|SpawnActorfromClass "/Game/Project/Blueprints/Items/ItemEquip/BP_Ring.BP_Ring_C" (Math|Transform|MakeTransform "0, 0, 0" "0, 0, 0" "1,1,1") "Undefined" 0 0))
    (Default|AddItem (Variables|/Game/Project/Blueprints/BP_PlayerCharacter.BP_PlayerCharacter_C|GetACP_Inventory (Variables|References|GetRefPlayer)) _returnvalue (Utilities|GetClass _returnvalue))
    (Actor|DestroyActor _returnvalue)))

(event Input|ActionEvents|InputActionGetBackpack
  (params (Key :type Key%20Structure :default "None"))
  ;[1 1 1] Debug equipment and tp
  (:Pressed
    (bind _returnvalue (Game|SpawnActorfromClass "/Game/Project/Blueprints/Items/BP_Backpack.BP_Backpack_C" (Math|Transform|MakeTransform "0, 0, 0" "0, 0, 0" "1,1,1") "Undefined" 0 0))
    (Default|AddItem (Variables|/Game/Project/Blueprints/BP_PlayerCharacter.BP_PlayerCharacter_C|GetACP_Inventory (Variables|References|GetRefPlayer)) _returnvalue (Utilities|GetClass _returnvalue))
    (Actor|DestroyActor _returnvalue)))

(event Input|ActionEvents|InputActionGoToWahou1
  (params (Key :type Key%20Structure :default "None"))
  ;[1 1 1] Debug equipment and tp
  (:Pressed
    (Transformation|SetActorLocation (Pawn|GetControlledPawn) "-2532.000000,-950.000000,-692.000000" false true)))

(event Input|ActionEvents|InputActionJump
  (params (Key :type Key%20Structure :default "None"))
  (bind _refplayer (Variables|References|GetRefPlayer))
  (:Pressed
    (Character|Jump _refplayer)
    (Variables|Default|SetJumping? true))
  (:Released
    (Character|StopJumping _refplayer)))

(event Input|ActionEvents|InputActionDodge
  (params (Key :type Key%20Structure :default "None"))
  (bind _refplayer (Variables|References|GetRefPlayer))
  ;[1 1 1] Esquive
  (:Pressed
    (if (Variables|Default|GetMovement%20Enabled)
      (if (Variables|/Game/Project/Blueprints/BP_PlayerCharacter.BP_PlayerCharacter_C|GetDashIsOnCD? _refplayer)
        (Development|PrintString "Can't Dodge for now")
        (elif (not (AI|Components|NavMovement|IsFalling (Variables|/Script/Engine.Character|GetCharacterMovement _refplayer)))
          (Default|StartDashing (Variables|References|GetRefPlayer) (Variables|Default|GetYMoving) (Variables|Default|GetXMoving) (Variables|DashRelated|GetDirectionString))
          (Audio|PlaySound2D "/Game/Project/Audio/SFX/Entity/Player/Dodge/SoundCue/SC_PlayerDodge.SC_PlayerDodge" 1.0 1.0 0.0 0 0))))))

(event Input|ActionEvents|InputActionSprint
  (params (Key :type Key%20Structure :default "None"))
  (bind _refplayer (Variables|References|GetRefPlayer))
  (bind _directionstring (Variables|DashRelated|GetDirectionString))
  (bind _direction (Variables|/Game/Project/Blueprints/BP_PlayerCharacter.BP_PlayerCharacter_C|GetDirection _refplayer))
  (bind _value (Utilities|Map|Find _direction _directionstring))
  (:Pressed
    (if (Variables|SprintRelated|GetSprinting?)
      (Variables|DashRelated|SetCurrentAcceleration 1.0)
      (Variables|SprintRelated|SetSprinting? false)
      (Variables|SprintRelated|SetSprintPressed false)
      (elif (Variables|Default|GetMovement%20Enabled)
        (if (and (< (.z _value) 265.0) (> (.z _value) 95.0))
          (Variables|SprintRelated|SetSprinting? true)
          (Variables|DashRelated|SetCurrentAcceleration (/ (Variables|DashRelated|GetCurrentAcceleration) 2.0))
          (Variables|SprintRelated|SetSprintPressed true))))))

(event Input|ActionEvents|InputActionGoToWahou2
  (params (Key :type Key%20Structure :default "None"))
  ;[1 1 1] Debug equipment and tp
  (:Pressed
    (Transformation|SetActorLocation (Pawn|GetControlledPawn) "-340.000000,4640.000000,-100.000000" false true)))

(event Input|ActionEvents|InputActionGetWeapon
  (params (Key :type Key%20Structure :default "None"))
  ;[1 1 1] Debug equipment and tp
  (:Pressed
    (Development|PrintString "sword debug")
    (bind _returnvalue (Game|SpawnActorfromClass "/Game/Project/Blueprints/Items/Weapon/BP_Sword.BP_Sword_C" (Math|Transform|MakeTransform "0, 0, 0" "0, 0, 0" "1,1,1") "Undefined" 0 0))
    (Default|AddItem (Variables|/Game/Project/Blueprints/BP_PlayerCharacter.BP_PlayerCharacter_C|GetACP_Inventory (Variables|References|GetRefPlayer)) _returnvalue (Utilities|GetClass _returnvalue))
    (Actor|DestroyActor _returnvalue)))

(event Input|ActionEvents|InputActionUseRing
  (params (Key :type Key%20Structure :default "None"))
  (bind _refplayer (Variables|References|GetRefPlayer))
  (bind _acp_weapon (Variables|/Game/Project/Blueprints/BP_PlayerCharacter.BP_PlayerCharacter_C|GetACP_Weapon _refplayer))
  (bind _currentring (Variables|/Game/Project/Blueprints/Items/ACP_Weapon.ACP_Weapon_C|GetCurrentRing _acp_weapon))
  ;[1 1 1] Use Ring
  (:Pressed
    (if (Variables|Default|GetMovement%20Enabled)
      (Utilities|IsValid _currentring
        (:Is%20Valid
          (bind _canuse_ (CallFunction|ConditionforUseItem))
          (if (not _canuse_)
            (Default|UseItemEquip _acp_weapon "NewEnumerator0"))))))
  (:Released
    (Variables|/Game/Project/Blueprints/Items/ACP_Weapon.ACP_Weapon_C|SetUseRing? _acp_weapon false)
    (Class|InterfaceUseItem|StopUseItemEquip(Message) _currentring)))

(event Input|ActionEvents|InputActionUseBracelet
  (params (Key :type Key%20Structure :default "None"))
  (bind _refplayer (Variables|References|GetRefPlayer))
  (bind _acp_weapon (Variables|/Game/Project/Blueprints/BP_PlayerCharacter.BP_PlayerCharacter_C|GetACP_Weapon _refplayer))
  (bind _currentbracelet (Variables|/Game/Project/Blueprints/Items/ACP_Weapon.ACP_Weapon_C|GetCurrentBracelet _acp_weapon))
  ;[1 1 1] Use Bracelet
  (:Pressed
    (if (Variables|Default|GetMovement%20Enabled)
      (Utilities|IsValid _currentbracelet
        (:Is%20Valid
          (bind _canuse_ (CallFunction|ConditionforUseItem))
          (if (not _canuse_)
            (Default|UseItemEquip _acp_weapon "NewEnumerator1"))))))
  (:Released
    (Variables|/Game/Project/Blueprints/Items/ACP_Weapon.ACP_Weapon_C|SetUseBracelet? _acp_weapon false)
    (Class|InterfaceUseItem|StopUseItemEquip(Message) _currentbracelet)))

(event Input|ActionEvents|InputActionGetRing
  (params (Key :type Key%20Structure :default "None"))
  ;[1 1 1] Debug equipment and tp
  (:Pressed
    (bind _returnvalue (Game|SpawnActorfromClass "/Game/Project/Blueprints/Items/ItemEquip/BP_Bracelet.BP_Bracelet_C" (Math|Transform|MakeTransform "0, 0, 0" "0, 0, 0" "1,1,1") "Undefined" 0 0))
    (Default|AddItem (Variables|/Game/Project/Blueprints/BP_PlayerCharacter.BP_PlayerCharacter_C|GetACP_Inventory (Variables|References|GetRefPlayer)) _returnvalue (Utilities|GetClass _returnvalue))
    (Actor|DestroyActor _returnvalue)))

(event Input|AxisEvents|InputAxisMoveForward
  (params (AxisValue :type Float%20%28single-precision%29))
  (bind _returnvalue (Utilities|Time|GetWorldDeltaSeconds))
  (bind _refplayer (Variables|References|GetRefPlayer))
  (bind _refplayer_2 (Variables|References|GetRefPlayer))
  (bind _returnvalue_2 (Pawn|GetControlRotation _refplayer_2 :!class /Script/Engine.Pawn))
  (bind _yaw (Math|Rotator|BreakRotator _returnvalue_2))
  (bind _returnvalue_3 (Math|Rotator|MakeRotator 0.0 0.0 _yaw))
  (bind _returnvalue_4 (Math|Vector|GetForwardVector _returnvalue_3))
  ;[0.2138 1 0.2401] Base Movements
  ;;[1 1 1] Player Movement
  (if (Variables|Default|GetMovement%20Enabled)
    (if (Variables|SprintRelated|GetSprinting?)
      (Pawn|Input|AddMovementInput _refplayer _returnvalue_4 (* AxisValue (Variables|DashRelated|GetCurrentAcceleration)) false)
      (else
        (Pawn|Input|AddMovementInput _refplayer _returnvalue_4 (/ (* AxisValue (Variables|DashRelated|GetCurrentAcceleration)) (Variables|SprintRelated|GetSprintSpeed)) false)))
    (Utilities|FlowControl|Sequence
      (:then_0
        (bind _output_get (Variables|Default|SetMoving? (Math|Boolean|Equal(Boolean) (and (== (Input|AxisValues|GetMoveForward) 0.0) (== (Input|AxisValues|GetMoveRight) 0.0)) false)))
        (if _output_get
          (CallFunction|CheckDirection)
          (if (<= (+ (Variables|DashRelated|GetCurrentAcceleration) _returnvalue) 1.0)
            (if (Variables|SprintRelated|GetSprinting?)
              (Variables|DashRelated|SetCurrentAcceleration (+ (Variables|DashRelated|GetCurrentAcceleration) (/ _returnvalue 3.0)))
              (else
                (Variables|DashRelated|SetCurrentAcceleration (+ (Variables|DashRelated|GetCurrentAcceleration) _returnvalue)))))
          (else
            (Variables|DashRelated|SetCurrentAcceleration 0.5))))
      (:then_1
        ;[1 1 1] MoveMoveValue
        (bind _refplayer_3 (Variables|References|GetRefPlayer)
          (:then
            (Variables|/Game/Project/Blueprints/BP_PlayerCharacter.BP_PlayerCharacter_C|SetMoveForwardValue _refplayer_3 AxisValue)
            (Variables|/Game/Project/Blueprints/BP_PlayerCharacter.BP_PlayerCharacter_C|SetMoveRightValue _refplayer_3 (stale Input|AxisEvents|InputAxisMoveRight AxisValue)))
          (:else
            (Development|PrintString "BP_PlayerController --> RefPlayer is not valid")))))))

(event Input|AxisEvents|InputAxisMoveRight
  (params (AxisValue :type Float%20%28single-precision%29))
  (bind _returnvalue (Utilities|Time|GetWorldDeltaSeconds))
  (bind _refplayer (Variables|References|GetRefPlayer))
  (bind _refplayer_2 (Variables|References|GetRefPlayer))
  (bind _returnvalue_2 (Pawn|GetControlRotation _refplayer_2 :!class /Script/Engine.Pawn))
  (bind _yaw (Math|Rotator|BreakRotator _returnvalue_2))
  (bind _returnvalue_3 (Math|Rotator|MakeRotator 0.0 0.0 _yaw))
  (bind _returnvalue_4 (Math|Vector|GetRightVector _returnvalue_3))
  ;[0.2138 1 0.2401] Base Movements
  ;;[1 1 1] Player Movement
  (if (Variables|Default|GetMovement%20Enabled)
    (if (Variables|SprintRelated|GetSprinting?)
      (Pawn|Input|AddMovementInput _refplayer _returnvalue_4 (* AxisValue (Variables|DashRelated|GetCurrentAcceleration)) false)
      (else
        (Pawn|Input|AddMovementInput _refplayer _returnvalue_4 (/ (* AxisValue (Variables|DashRelated|GetCurrentAcceleration)) (Variables|SprintRelated|GetSprintSpeed)) false)))
    (Utilities|FlowControl|Sequence
      (:then_0
        (bind _output_get (Variables|Default|SetMoving? (Math|Boolean|Equal(Boolean) (and (== (Input|AxisValues|GetMoveForward) 0.0) (== (Input|AxisValues|GetMoveRight) 0.0)) false)))
        (if _output_get
          (CallFunction|CheckDirection)
          (if (<= (+ (Variables|DashRelated|GetCurrentAcceleration) _returnvalue) 1.0)
            (if (Variables|SprintRelated|GetSprinting?)
              (Variables|DashRelated|SetCurrentAcceleration (+ (Variables|DashRelated|GetCurrentAcceleration) (/ _returnvalue 3.0)))
              (else
                (Variables|DashRelated|SetCurrentAcceleration (+ (Variables|DashRelated|GetCurrentAcceleration) _returnvalue)))))
          (else
            (Variables|DashRelated|SetCurrentAcceleration 0.5))))
      (:then_1
        ;[1 1 1] MoveMoveValue
        (bind _refplayer_3 (Variables|References|GetRefPlayer)
          (:then
            (Variables|/Game/Project/Blueprints/BP_PlayerCharacter.BP_PlayerCharacter_C|SetMoveForwardValue _refplayer_3 (stale Input|AxisEvents|InputAxisMoveForward AxisValue))
            (Variables|/Game/Project/Blueprints/BP_PlayerCharacter.BP_PlayerCharacter_C|SetMoveRightValue _refplayer_3 AxisValue))
          (:else
            (Development|PrintString "BP_PlayerController --> RefPlayer is not valid")))))))

(event Input|AxisEvents|InputAxisCameraUp
  (params (AxisValue :type Float%20%28single-precision%29))
  ;[0.2138 1 0.2401] Base Movements
  ;;[1 1 1] Camera Movement
  (Pawn|Input|AddControllerPitchInput (Variables|References|GetRefPlayer) AxisValue))

(event Input|AxisEvents|InputAxisCameraRight
  (params (AxisValue :type Float%20%28single-precision%29))
  ;[0.2138 1 0.2401] Base Movements
  ;;[1 1 1] Camera Movement
  (Pawn|Input|AddControllerYawInput (Variables|References|GetRefPlayer) AxisValue))

(event Input|KeyboardEvents|Subtract
  (params (Key :type Key%20Structure :default "None"))
  (:Pressed
    (Default|TakeDamage (Variables|References|GetRefPlayer) 25.0 "NewEnumerator0")))

(event Input|KeyboardEvents|AnyKey
  (params (Key :type Key%20Structure :default "None")))

(event Input|KeyboardEvents|AnyKey
  (params (Key :type Key%20Structure :default "None"))
  (:Released
    (CallFunction|IfGamepadIsUsed Key)))

(fn ConstructionScript)

(fn CheckDirection
  (bind _returnvalue (Input|AxisValues|GetMoveForward))
  (bind _returnvalue_2 (Input|AxisValues|GetMoveRight))
  (if (< _returnvalue 0.0)
    (Variables|Default|SetXMoving -1)
    (elif (== _returnvalue 0.0)
      (Variables|Default|SetXMoving 0)
      (elif (> _returnvalue 0.0)
        (Variables|Default|SetXMoving 1))))
  (if (< _returnvalue_2 0.0)
    (Variables|Default|SetYMoving -1)
    (switch int (Variables|Default|GetXMoving)
      (:-1
        (Variables|DashRelated|SetDirectionString "Back-Left"))
      (:0
        (Variables|DashRelated|SetDirectionString "Left"))
      (:1
        (Variables|DashRelated|SetDirectionString "Front-Left")))
    (elif (== _returnvalue_2 0.0)
      (Variables|Default|SetYMoving 0)
      (switch int (Variables|Default|GetXMoving)
        (:-1
          (Variables|DashRelated|SetDirectionString "Back"))
        (:0
          (Variables|Default|SetXMoving 1)
          (Variables|DashRelated|SetDirectionString "Front" :!label _label))
        (:1
          (goto _label)))
      (elif (> _returnvalue_2 0.0)
        (Variables|Default|SetYMoving 1)
        (switch int (Variables|Default|GetXMoving)
          (:-1
            (Variables|DashRelated|SetDirectionString "Back-Right"))
          (:0
            (Variables|DashRelated|SetDirectionString "Right"))
          (:1
            (Variables|DashRelated|SetDirectionString "Front-Right")))
        (else
          (Development|PrintString "Error"))))))

(fn SetAttackPress
  (params (AttackPress? :type Boolean))
  (Variables|Attack|SetAttackPress? AttackPress?))

(fn ConditionforUseItem
  (bind _refplayer (Variables|References|GetRefPlayer))
  (bind _acp_weapon (Variables|/Game/Project/Blueprints/BP_PlayerCharacter.BP_PlayerCharacter_C|GetACP_Weapon _refplayer))
  (return (and (Variables|/Game/Project/Blueprints/Items/ItemEquip/BP_Ring.BP_Ring_C|GetAnimOk? (.AsBP%20Ring (Utilities|Casting|CastToBP_Ring (Variables|/Game/Project/Blueprints/Items/ACP_Weapon.ACP_Weapon_C|GetCurrentRing _acp_weapon)))) (Math|Boolean|ORBoolean (Variables|/Game/Project/Blueprints/Items/ACP_Weapon.ACP_Weapon_C|GetUseBracelet? _acp_weapon) (Variables|/Game/Project/Blueprints/Items/ACP_Weapon.ACP_Weapon_C|GetUseRing? _acp_weapon) (Variables|/Game/Project/Blueprints/Items/ACP_Weapon.ACP_Weapon_C|GetUseSlightAttack? _acp_weapon) (Variables|/Game/Project/Blueprints/Items/ACP_Weapon.ACP_Weapon_C|GetUseHeavyAttack? _acp_weapon) (Variables|Attack|GetAttackPress?)))))

(fn ConditionforAttack
  (bind _refplayer (Variables|References|GetRefPlayer))
  (bind _acp_weapon (Variables|/Game/Project/Blueprints/BP_PlayerCharacter.BP_PlayerCharacter_C|GetACP_Weapon _refplayer))
  (return (or (Variables|/Game/Project/Blueprints/Items/ACP_Weapon.ACP_Weapon_C|GetUseBracelet? _acp_weapon) (Variables|/Game/Project/Blueprints/Items/ACP_Weapon.ACP_Weapon_C|GetUseRing? _acp_weapon))))